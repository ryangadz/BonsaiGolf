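; Actor that fills a spline-outlined pot with randomly chosen succulents, sized to pack inside the outline.
; PotComplete builds a point grid inside SplineWithMesh, then a looping timer spawns and grows one plant at a time.
; CalculateLocations greedily places circles using distances to the spline and earlier circles, clearing covered points; radius sets plant scale, spawn order sets age.
; The construction script only randomizes Size; its mesh and debug experiments are disconnected.
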(event `self.ReceiveBeginPlay`
  (`parent.ReceiveBeginPlay`))

(event `self.ReceiveActorBeginOverlap`
  (params (OtherActor :type "Actor Object Reference"))
  (`parent.ReceiveActorBeginOverlap` null))

(event `self.ReceiveTick`
  (params (DeltaSeconds :type "Float (single-precision)"))
  (`parent.ReceiveTick` 0.0))

(event `self.PotComplete`
  (bind (_insideindices _gridx _verts) (`/Game/Blueprints/Libraries/BFL_MeshBuilding.MakePointGrid` (`self.SplineWithMesh`) 3.0))
  (set `self.Verts` _verts)
  (set `self.Triangles` _insideindices)
  (`KismetSystemLibrary.K2_SetTimerDelegate` (delegate `SpawnNewPlant`) 0.15 true))

(event `SpawnNewPlant`
  (`self.CalculateLocations` (`self.CurrentPlantNum`))
  (bind _returnvalue (`|SpawnActorFromClass` (`|GetArrayItem` (`self.SucculentClasses`) (`KismetMathLibrary.RandomIntegerInRange` 0 2)) (`KismetMathLibrary.MakeTransform` (`|GetArrayItem` (`self.ClosestPointLocation_0`) (`self.CurrentPlantNum`)) (struct) (`KismetMathLibrary.Conv_DoubleToVector` (/ (`|GetArrayItem` (`self.ClosestPointDistance_0`) (`self.CurrentPlantNum`)) 16.0))) "Undefined" "OverrideRootScale" null (`KismetMathLibrary.FTrunc` (`KismetMathLibrary.MapRangeClamped` (`KismetMathLibrary.Conv_IntToDouble` (`self.CurrentPlantNum`)) 0.0 (`KismetMathLibrary.Conv_IntToDouble` (- (`self.TotalNumPlants`) 1)) 5.0 1.0)) true null))
  (`/Game/Blueprints/Plants/Succulents/BP_ShortSucculentM_.GrowSucculent` _returnvalue 10.0 0.0)
  (bind _result (`/Engine/EditorBlueprintResources/StandardMacros.IncrementInt` (`self.CurrentPlantNum`))
    (:`  `
      (if (not (> (`self.TotalNumPlants`) _result))
        (`KismetSystemLibrary.K2_SetTimerDelegate` (delegate `SpawnNewPlant`))))))

(fn `CalculateLocations`
  (params (Index :type Integer))
  (locals (IndexLocal :type Integer) (ClosestLocation :type "Vector Structure") (SumClosestDistance :type "Float (double-precision)") (LengthToEdge :type "Float (double-precision)") (ClosestDistanceTemp :type "Float (double-precision)" :default 10000.0) (LargestDistanceToClosestCircle :type "Float (double-precision)" :default 0.0) (SumClosestPrevious :type "Float (double-precision)") (Count :type Integer))
  (bind _returnvalue (+ (`local.LengthToEdge`) (`local.ClosestDistanceTemp`)))
  (bind _output (`|GetArrayItem` (`self.Verts`) (`local.IndexLocal`)))
  (set `self.ClosestPointDistance` 0.0)
  (for (_array_element _array_index) (`self.Verts`)
    (set `local.IndexLocal` _array_index)
    (if (and (== (`|GetArrayItem` (`self.Triangles`) _array_index) 0) (!= _array_element (0.0 0.0 0.0) :`ErrorTolerance` 0.01))
      (set `local.LengthToEdge` (`KismetMathLibrary.VSize` (- (`|GetArrayItem` (`self.Verts`) (`local.IndexLocal`)) (`SplineComponent.FindLocationClosestToWorldLocation` (`self.SplineWithMesh`) (`|GetArrayItem` (`self.Verts`) (`local.IndexLocal`)) "World"))))
      (if (> (`local.Index`) 0)
        (set `local.ClosestDistanceTemp` 10000.0)
        (for (_array_element_2 _array_index_2) (`self.ClosestPointLocation_0`)
          (bind _returnvalue_2 (- (`KismetMathLibrary.VSize` (- (`|GetArrayItem` (`self.Verts`) (`local.IndexLocal`)) _array_element_2)) (`|GetArrayItem` (`self.ClosestPointDistance_0`) _array_index_2)))
          (if (and (> _returnvalue_2 0.0) (< _returnvalue_2 (`local.LengthToEdge`)) (< _returnvalue_2 (`local.ClosestDistanceTemp`)))
            (set `local.ClosestDistanceTemp` _returnvalue_2)))
        (if (> _returnvalue (`local.SumClosestPrevious`))
          (set `local.SumClosestPrevious` _returnvalue)
          (if (< (`local.SumClosestPrevious`) (* (`local.LengthToEdge`) 2.0))
            (set `self.ClosestPointDistance` (`local.ClosestDistanceTemp`))
            (set `self.ClosestPointLocation` _output)
            (else
              (set `self.ClosestPointDistance` (`local.LengthToEdge`))
              (set `self.ClosestPointLocation` _output))))
        (elif (> (`local.LengthToEdge`) (`self.ClosestPointDistance`))
          (set `self.ClosestPointDistance` (`local.LengthToEdge`))
          (set `self.ClosestPointLocation` (`|GetArrayItem` (`self.Verts`) (`local.IndexLocal`)))))
      (else
        (`KismetArrayLibrary.Array_Set` (`self.Verts`) (`local.IndexLocal`)))))
  (`KismetArrayLibrary.Array_Set` (`self.ClosestPointDistance_0`) (`local.Index`) (`self.ClosestPointDistance`) true)
  (`KismetArrayLibrary.Array_Set` (`self.ClosestPointLocation_0`) (`local.Index`) (+ (`self.ClosestPointLocation`) (0.0 0.0 1.0)) true)
  (for (_array_element_3 _array_index_3) (`self.Verts`)
    (if (< (`KismetMathLibrary.VSize` (- (`|GetArrayItem` (`self.ClosestPointLocation_0`) (`local.Index`)) _array_element_3)) (`|GetArrayItem` (`self.ClosestPointDistance_0`) (`local.Index`)))
      (`KismetArrayLibrary.Array_Set` (`self.Verts`) _array_index_3))))

(fn `OverlapsCircle`
  (params (NewParam :type "Array of Vector Structure") (NewParam1 :type "Array of Float (double-precision)")))

(fn `UserConstructionScript`
  (set `self.Size` (`KismetMathLibrary.RandomFloatInRange` 8.0 18.0)))