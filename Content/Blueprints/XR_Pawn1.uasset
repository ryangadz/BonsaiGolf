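; XR pawn for a putting game that spawns a BP_Course and handles placing and putting a physics ball.
; The right face button requests a controller raycast and spawns the course at its hit point, while either shoulder button line-traces to teleport the ball.
; Tick enables putting when the ball nearly stops, showing an arrow steered by the right thumbstick relative to the camera.
; The right trigger applies an impulse along that direction, scaled by stick deflection.
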(event `RequestRaycast`)

(event `self.ReceiveBeginPlay`
  (set `MotionControllerComponent.MotionSource` "AnyHand" (`self.MotionController_0`))
  (bind _returnvalue (`AddComponent|NODE_AddStaticMeshComponent-1` :`RelativeTransform` (`KismetMathLibrary.MakeTransform` (0.0 0.0 100.0))))
  (set `self.BallS` _returnvalue)
  (bind _returnvalue_2 (`AddComponent|NODE_AddStaticMeshComponent-2` :`bManualAttachment` true :`RelativeTransform` (`KismetMathLibrary.MakeTransform` (0.0 0.0 0.0) (struct) (0.0 0.0 0.0))))
  (bind _output_get (set `self.Direction Arrow` _returnvalue_2))
  (bind _returnvalue_3 (`KismetMaterialLibrary.CreateDynamicMaterialInstance` (`PrimitiveComponent.GetMaterial` _output_get 0)))
  (set `self.Arrow Material` _returnvalue_3)
  (`SceneComponent.K2_AttachToComponent` _output_get (`self.BallS`) "None" "SnapToTarget" "KeepWorld" "KeepWorld" true))

(event `Key|MotionController_Right_Shoulder`
  (params (Key :type "Key Structure")))

(event `Key|MotionController_Right_FaceButton1`
  (params (Key :type "Key Structure"))
  (bind _motioncontroller_0 (`self.MotionController_0`))
  (:`Pressed`
    (`RaycastComponent.RequestRaycast` (`self.Raycast`) (make `RaycastQueryParams` (`SceneComponent.K2_GetComponentLocation` _motioncontroller_0) (`SceneComponent.GetForwardVector` _motioncontroller_0) (0.0 0.0 1.0) 1 1 1.0) (delegate `RaycastResults`))
    (`|SpawnActorFromClass` "/Game/Blueprints/BP_Course.BP_Course_C" (`KismetMathLibrary.MakeTransform` (+ (`.HitPoint` (break `RaycastHitResult` (stale `RaycastResults` HitResult))) (0.0 0.0 10.0)) (struct) (0.66 0.66 0.66)) "Undefined" "OverrideRootScale" null null)))

(event `ScaleLaser`)

(event `Key|MotionController_Right_Thumbstick_Down`
  (params (Key :type "Key Structure")))

(event `Key|MotionController_Right_Thumbstick`
  (params (Key :type "Key Structure")))

(event `RaycastResults`
  (params (HitResult :type "RaycastHitResult Structure")))

(event `Key|MotionController_Left_Shoulder`
  (params (Key :type "Key Structure"))
  (bind _balls (`self.BallS`))
  (bind _motioncontroller_0 (`self.MotionController_0`))
  (bind _material (`self.Material`))
  (bind _returnvalue (`SceneComponent.K2_GetComponentLocation` _motioncontroller_0))
  (:`Pressed`
    (`MaterialInstanceDynamic.SetVectorParameterValue` _material "color" (struct :`R` 1.0 :`A` 1.0) :!label _label)
    (bind _outhit (`KismetSystemLibrary.LineTraceSingleForObjects` :`Start` _returnvalue :`End` (+ _returnvalue (* (`SceneComponent.GetForwardVector` _motioncontroller_0) 1000.0)) :`ObjectTypes` (`|MakeArray` "ObjectTypeQuery1" :!type "EObjectTypeQuery Enum") :`DrawDebugType` "ForDuration" :`bIgnoreSelf` false :`DrawTime` 2.0))
    (`SceneComponent.K2_SetWorldTransform` _balls (`KismetMathLibrary.MakeTransform` (+ (`.ImpactPoint` (`GameplayStatics.BreakHitResult` _outhit)) (0.0 0.0 10.0)) (struct) (0.66 0.66 0.66)) false true)
    (`PrimitiveComponent.SetPhysicsLinearVelocity` _balls (0.0 0.0 0.0) false "None"))
  (:`Released`
    (`MaterialInstanceDynamic.SetVectorParameterValue` _material "None" (struct :`R` 1.0 :`G` 1.0 :`B` 1.0 :`A` 1.0) :!label _label_2)))

(event `Key|MotionController_Right_Shoulder`
  (params (Key :type "Key Structure"))
  (:`Pressed`
    (goto _label))
  (:`Released`
    (goto _label_2)))

(event `Key|MotionController_Right_Shoulder`
  (params (Key :type "Key Structure")))

(event `self.ReceiveTick`
  (params (DeltaSeconds :type "Float (single-precision)"))
  (bind _direction_arrow (`self.Direction Arrow`))
  (bind _thumbx (`self.ThumbX`))
  (bind _thumby (`self.ThumbY`))
  (bind (_returnvalue_roll _returnvalue_pitch _returnvalue_yaw) (`KismetMathLibrary.BreakRotator` (`KismetMathLibrary.MakeRotFromY` (- (`SceneComponent.K2_GetComponentLocation` (`self.BallS`)) (`SceneComponent.K2_GetComponentLocation` (`self.XR_Camera`))))))
  (if (> (`KismetMathLibrary.VSizeSquared` (`SceneComponent.GetComponentVelocity` (`self.BallS`))) 0.05)
    (set `self.ReadyToPutt?` false)
    (set `self.ThumbX` 0.0)
    (set `self.ThumbY` 0.0)
    (`SceneComponent.SetWorldScale3D` (`self.Direction Arrow`) (0.0 0.0 0.0))
    (else
      (set `self.ReadyToPutt?` true)
      (`SceneComponent.SetVisibility` (`self.Direction Arrow`) true false)
      (`SceneComponent.K2_SetWorldRotation` _direction_arrow (`KismetMathLibrary.MakeRotator` 90.0 0.0 (- (+ _returnvalue_yaw (`KismetMathLibrary.DegAtan2` _thumbx _thumby)) 90.0)) false false)
      (`SceneComponent.SetWorldScale3D` _direction_arrow (`KismetMathLibrary.MakeVector` 1.0 1.0 (* (`KismetMathLibrary.Sqrt` (+ (`KismetMathLibrary.MultiplyMultiply_FloatFloat` _thumbx 2.0) (`KismetMathLibrary.MultiplyMultiply_FloatFloat` _thumby 2.0))) 10.0))))))

(event `InputAxisKey|MotionController_Left_Thumbstick_X`
  (params (AxisValue :type "Float (single-precision)")))

(event `InputAxisKey|MotionController_Right_Thumbstick_X`
  (params (AxisValue :type "Float (single-precision)"))
  (set `self.ThumbX` AxisValue))

(event `InputAxisKey|MotionController_Left_Thumbstick_Y`
  (params (AxisValue :type "Float (single-precision)")))

(event `InputAxisKey|MotionController_Right_Thumbstick_Y`
  (params (AxisValue :type "Float (single-precision)"))
  (set `self.ThumbY` AxisValue))

(event `Key|MotionController_Left_Trigger`
  (params (Key :type "Key Structure")))

(event `Key|MotionController_Right_Trigger`
  (params (Key :type "Key Structure"))
  (bind _thumbx (`self.ThumbX`))
  (bind _thumby (`self.ThumbY`))
  (bind (_returnvalue_roll _returnvalue_pitch _returnvalue_yaw) (`KismetMathLibrary.BreakRotator` (`KismetMathLibrary.MakeRotFromY` (- (`SceneComponent.K2_GetComponentLocation` (`self.BallS`)) (`SceneComponent.K2_GetComponentLocation` (`self.XR_Camera`))))))
  (:`Pressed`
    (if (`self.ReadyToPutt?`)
      (`PrimitiveComponent.AddImpulse` (`self.BallS`) (* (`KismetMathLibrary.GreaterGreater_VectorRotator` (1.0 0.0 0.0) (`KismetMathLibrary.MakeRotator` 0.0 0.0 (+ _returnvalue_yaw (`KismetMathLibrary.DegAtan2` _thumbx _thumby)))) (* (`KismetMathLibrary.Sqrt` (+ (`KismetMathLibrary.MultiplyMultiply_FloatFloat` _thumbx 2.0) (`KismetMathLibrary.MultiplyMultiply_FloatFloat` _thumby 2.0))) 15.0)) "None" false)
      (`SceneComponent.SetWorldScale3D` (`self.Direction Arrow`) (0.0 0.0 0.0))
      (set `self.ReadyToPutt?` false))))

(event `self.BallS.OnComponentDeactivated`
  (params (Component :type "ActorComponent Object Reference")))

(event `self.BallS.OnComponentSleep`
  (params (SleepingComponent :type "PrimitiveComponent Object Reference") (BoneName :type Name)))

(event `self.BallS.OnComponentWake`
  (params (WakingComponent :type "PrimitiveComponent Object Reference") (BoneName :type Name)))

(fn `UserConstructionScript`
  (`StaticMeshComponent.SetStaticMesh` (`StaticMeshActor.StaticMeshComponent` (`self.StaticMesh`)) "/Game/Assets/Mesh/DirArrow.DirArrow")
  (bind _returnvalue (`KismetMaterialLibrary.CreateDynamicMaterialInstance` "/Game/Materials/M_DirectionArrow.M_DirectionArrow"))
  (bind _output_get (set `self.Material` _returnvalue))
  (`PrimitiveComponent.SetMaterial` (`self.Cube`) 0 _output_get)
  (`PrimitiveComponent.SetMaterial` (`StaticMeshActor.StaticMeshComponent` (`self.StaticMesh`)) 0 _output_get))