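; Test actor that generates lake and ground procedural meshes from two spline outlines in its Construction Script.
; BuildMeshFromOutline turns each spline into vertices, triangles, UVs and vertex colors for a new procedural mesh component with its own material.
; The ground pass also calls MakePointGrid but ignores its result.
; Disconnected leftovers include seeded rock and grass instance scattering driven by vertex color, an alternate lake mesh, and debug bounds drawing.
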(fn `UserConstructionScript`
  (bind _splineground (`self.SplineGround`))
  (`|ExecutionSequence`
    (:`then_0`
      (bind (_verts _triangles _uvs _vertexcolor) (`/Game/Blueprints/Libraries/BFL_MeshBuilding.BuildMeshFromOutline` (`self.SplineLake`)))
      (bind _returnvalue (`AddComponent|NODE_AddProceduralMeshComponent-0` :`bManualAttachment` true))
      (`ProceduralMeshComponent.CreateMeshSection_LinearColor` :`self` _returnvalue :`Vertices` _verts :`Triangles` _triangles :`UV0` _uvs :`VertexColors` _vertexcolor)
      (`PrimitiveComponent.SetMaterial` _returnvalue 0 "/Game/Materials/Test/M_ProceduraMeshLake.M_ProceduraMeshLake"))
    (:`then_1`
      (`/Game/Blueprints/Libraries/BFL_MeshBuilding.MakePointGrid` _splineground 5.0)
      (bind (_verts_2 _triangles_2 _uvs_2 _vertexcolor_2) (`/Game/Blueprints/Libraries/BFL_MeshBuilding.BuildMeshFromOutline` _splineground))
      (bind _returnvalue_2 (`AddComponent|NODE_AddProceduralMeshComponent-1` :`bManualAttachment` true))
      (`ProceduralMeshComponent.CreateMeshSection_LinearColor` :`self` _returnvalue_2 :`Vertices` _verts_2 :`Triangles` _triangles_2 :`UV0` _uvs_2 :`VertexColors` _vertexcolor_2)
      (`PrimitiveComponent.SetMaterial` _returnvalue_2 0 "/Game/Materials/Test/M_ProceduraMeshGround.M_ProceduraMeshGround"))))