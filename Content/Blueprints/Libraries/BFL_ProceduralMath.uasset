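; Blueprint function library of procedural placement math built on the golden angle and golden ratio.
; Phyllotaxis places a numbered point on a flat spiral, using the simplified golden angle plus seeded angular jitter.
; RandomGoldenSnake recursively fills a location array with randomly yawed steps, dividing length by the golden ratio each step.
; Grouping fills an array with 2D Sobol-distributed locations at unit scale, ignoring its InitialScale input.
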(fn `GoldenAngle`
  (returns (Degrees :type "Float (double-precision)") (Radians :type "Float (double-precision)"))
  (bind _returnvalue (`KismetMathLibrary.Sqrt` 5.0))
  (return (* 180.0 (- 3.0 _returnvalue)) (* (`KismetMathLibrary.GetPI`) (- 3.0 _returnvalue))))

(fn `GoldenAngleSimple`
  (returns (Degrees :type "Float (double-precision)") (Radians :type "Float (double-precision)"))
  (return 137.5 2.4))

(fn `GoldenRatio`
  (returns (out :type "Float (double-precision)"))
  (return (/ (+ (`KismetMathLibrary.Sqrt` 5.0) 1.0) 2.0)))

(fn `Grouping`
  (params (Number :type Integer) (`Initial Scale` :type "Float (double-precision)"))
  (returns (`Location +Scale` :type "Array of /Game/Blueprints/S_Grouping Structure"))
  (locals (LocationScale :type "Array of /Game/Blueprints/S_Grouping Structure"))
  (for _index (range (+ Number 1))
    (bind (_returnvalue_x _returnvalue_y) (`KismetMathLibrary.BreakVector2D` (`ImportanceSamplingLibrary.RandomSobolCell2D` _index 1 (0.0 0.0) (10.0 1.0))))
    (`KismetArrayLibrary.Array_Set` (`local.LocationScale`) _index (make `/Game/Blueprints/S_Grouping` (`KismetMathLibrary.MakeVector` _returnvalue_x _returnvalue_y) 1.0) true))
  (return (`local.LocationScale`)))

(fn `Phyllotaxis`
  (params (Number :type Integer :default 5) (Variation :type "Float (double-precision)") (Seed :type Integer) (Spacing :type "Float (double-precision)" :default 1.0))
  (returns (Location :type "Vector Structure"))
  (bind _degrees (`self.GoldenAngleSimple` null))
  (bind _variation (`local.Variation`))
  (bind _returnvalue (* (* Number (/ _degrees 360.0)) (`local.Spacing`)))
  (bind _returnvalue_2 (+ (* Number _degrees) (`KismetMathLibrary.RandomFloatInRangeFromStream` (* _variation -1.0) _variation (`KismetMathLibrary.MakeRandomStream` (+ (`local.Seed`) (`local.Number`))))))
  (return (`KismetMathLibrary.MakeVector` (* (`KismetMathLibrary.DegCos` _returnvalue_2) _returnvalue) (* _returnvalue (`KismetMathLibrary.DegSin` _returnvalue_2)))))

(fn `RandomGoldenSnake`
  (params (Length :type "Float (double-precision)") (LocationArrayIn :type "Array of Vector Structure") (NumSteps :type Integer :default 5) (CurrentStep :type Integer))
  (bind _currentstep (`local.CurrentStep`))
  (bind _locationarrayin (`local.LocationArrayIn`))
  (bind _currentstep_2 (`local.CurrentStep`))
  (bind _locationarrayin_2 (`local.LocationArrayIn`))
  (bind _returnvalue (/ Length (`self.GoldenRatio` null)))
  (bind _returnvalue_2 (* (`KismetMathLibrary.RandomFloatInRange` -1.0 1.0) 270.0))
  (if (>= _currentstep_2 (`local.NumSteps`))
    (return)
    (else
      (if (> CurrentStep 1)
        (`KismetArrayLibrary.Array_Set` _locationarrayin_2 _currentstep_2 (+ (* (`KismetMathLibrary.GreaterGreater_VectorRotator` (`KismetMathLibrary.Normal` (* (- (`|GetArrayItem` _locationarrayin _currentstep) (`|GetArrayItem` _locationarrayin (- _currentstep 1))) -1.0)) (`KismetMathLibrary.MakeRotator` 0.0 0.0 _returnvalue_2)) _returnvalue) (`|GetArrayItem` _locationarrayin_2 (- _currentstep_2 1))) true)
        (else
          (`KismetArrayLibrary.Array_Set` LocationArrayIn CurrentStep (* (`KismetMathLibrary.GreaterGreater_VectorRotator` (1.0 0.0 0.0) (`KismetMathLibrary.MakeRotator` 0.0 0.0 _returnvalue_2)) _returnvalue) true)))
      (`/Engine/EditorBlueprintResources/StandardMacros.IncrementInt` (`local.CurrentStep`)
        (:`  `
          (`self.RandomGoldenSnake` _returnvalue (`local.LocationArrayIn`) (`local.NumSteps`) (`local.CurrentStep`)))))))