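; Blueprint function library for drawing spline outlines with a motion controller, placed at the hand, a forward offset, or a world-static line-trace hit.
; BeginOutline seeds a two-point spline, optionally snapping the first point to an axis.
; ContinueOutline drags the last point with smoothed tangents, locking new points at a set spacing, optionally flattened to the first point's height.
; With auto-close, CheckForLoop closes the spline near its start; CheckForLoop_0 duplicates it.
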(fn `BeginOutline`
  (params (Spline :type "SplineComponent Object Reference") (LocationType :type "/Game/Blueprints/Enum_MotionControllerData Enum" :default "NewEnumerator0") (ControllerTrans :type "Transform Structure") (LockedSplinePoints :type "Integer (by ref)") (LastSplineLocation :type "Vector Structure (by ref)") (`SnapToAxis?` :type Boolean) (Axis :type "Vector Structure" :default (0.0 0.0 1.0)))
  (bind _spline (`local.Spline`))
  (bind _axis (`local.Axis`))
  (bind (_validlocation_ _location) (`self.LocationFromMotionController` (`local.LocationType`) (`local.ControllerTrans`) 50.0))
  (`SplineComponent.ClearSplinePoints` Spline true)
  (if `SnapToAxis?`
    (`SplineComponent.AddSplinePointAtIndex` (`local.Spline`) (* (`KismetMathLibrary.Normal` _axis) (`KismetMathLibrary.Dot_VectorVector` (- _location (`Actor.K2_GetActorLocation` (`ActorComponent.GetOwner` Spline))) _axis)) 0 "Local" true)
    (else
      (`SplineComponent.AddSplinePointAtIndex` _spline _location 0 "World" true)))
  (`SplineComponent.AddSplinePointAtIndex` _spline _location 1 "World" true)
  (`|VariableSetRef` (`local.LockedSplinePoints`) 2)
  (`|VariableSetRef` (`local.LastSplineLocation`) _location))

(fn `CheckForLoop`
  (params (Spline :type "SplineComponent Object Reference") (LockedSplinePoints :type Integer))
  (returns (Continue :type Boolean))
  (locals (`ContinueDrawing?` :type Boolean))
  (bind _spline (`local.Spline`))
  (bind _spline_2 (`local.Spline`))
  (bind _spline_3 (`local.Spline`))
  (bind _spline_4 (`local.Spline`))
  (bind _lockedsplinepoints (`local.LockedSplinePoints`))
  (bind _spline_5 (`local.Spline`))
  (bind _returnvalue (- (`local.LockedSplinePoints`) 1))
  (bind _returnvalue_2 (`SplineComponent.GetLocationAtSplinePoint` _spline_2 (- _lockedsplinepoints 1) "World"))
  (bind _returnvalue_3 (`SplineComponent.GetLocationAtSplinePoint` _spline_2 (- _lockedsplinepoints 2) "World"))
  (bind _returnvalue_4 (+ _returnvalue_2 _returnvalue_3))
  (if (and (> LockedSplinePoints 3) (<= (`KismetMathLibrary.VSize` (- (`SplineComponent.GetLocationAtSplinePoint` _spline 0 "World") (`SplineComponent.GetLocationAtSplinePoint` _spline (- (`local.LockedSplinePoints`) 1) "World"))) 10.0))
    (set `local.ContinueDrawing?` false)
    (if (not (> (`KismetMathLibrary.VSize` _returnvalue_4) 5.0))
      (`SplineComponent.SetLocationAtSplinePoint` _spline_3 (- (`local.LockedSplinePoints`) 2) (/ _returnvalue_4 2.0) "World" false)
      (`SplineComponent.SetTangentAtSplinePoint` _spline_3 _returnvalue (* (`KismetMathLibrary.Normal` (/ (+ (`SplineComponent.GetTangentAtSplinePoint` _spline_5 (- (`local.LockedSplinePoints`) 2) "World") (`SplineComponent.GetTangentAtSplinePoint` _spline_5 (- (`local.LockedSplinePoints`) 1) "World")) 2.0)) (+ (/ (`KismetMathLibrary.VSize` (- _returnvalue_2 _returnvalue_3)) 2.0) 10.0)) "World" true)
      (`SplineComponent.RemoveSplinePoint` _spline_3 _returnvalue true))
    (`SplineComponent.SetClosedLoop` _spline_3 true true)
    (`SplineComponent.SetTangentAtSplinePoint` (`local.Spline`) 0 (`KismetMathLibrary.GetVectorArrayAverage` (`|MakeArray` (`SplineComponent.GetTangentAtSplinePoint` _spline_4 0 "World") (`SplineComponent.GetTangentAtSplinePoint` _spline_4 (- (`local.LockedSplinePoints`) 1) "World"))) "World" true)
    (else
      (bind _output_get (set `local.ContinueDrawing?` true))
      (return _output_get))))

(fn `CheckForLoop_0`
  (params (Spline :type "SplineComponent Object Reference") (LockedSplinePoints :type Integer))
  (returns (Continue :type Boolean))
  (locals (`ContinueDrawing?` :type Boolean))
  (bind _spline (`local.Spline`))
  (bind _spline_2 (`local.Spline`))
  (bind _spline_3 (`local.Spline`))
  (bind _spline_4 (`local.Spline`))
  (bind _lockedsplinepoints (`local.LockedSplinePoints`))
  (bind _spline_5 (`local.Spline`))
  (bind _returnvalue (- (`local.LockedSplinePoints`) 1))
  (bind _returnvalue_2 (`SplineComponent.GetLocationAtSplinePoint` _spline_2 (- _lockedsplinepoints 1) "World"))
  (bind _returnvalue_3 (`SplineComponent.GetLocationAtSplinePoint` _spline_2 (- _lockedsplinepoints 2) "World"))
  (bind _returnvalue_4 (+ _returnvalue_2 _returnvalue_3))
  (if (and (> LockedSplinePoints 3) (<= (`KismetMathLibrary.VSize` (- (`SplineComponent.GetLocationAtSplinePoint` _spline 0 "World") (`SplineComponent.GetLocationAtSplinePoint` _spline (- (`local.LockedSplinePoints`) 1) "World"))) 10.0))
    (set `local.ContinueDrawing?` false)
    (if (not (> (`KismetMathLibrary.VSize` _returnvalue_4) 5.0))
      (`SplineComponent.SetLocationAtSplinePoint` _spline_3 (- (`local.LockedSplinePoints`) 2) (/ _returnvalue_4 2.0) "World" false)
      (`SplineComponent.SetTangentAtSplinePoint` _spline_3 _returnvalue (* (`KismetMathLibrary.Normal` (/ (+ (`SplineComponent.GetTangentAtSplinePoint` _spline_5 (- (`local.LockedSplinePoints`) 2) "World") (`SplineComponent.GetTangentAtSplinePoint` _spline_5 (- (`local.LockedSplinePoints`) 1) "World")) 2.0)) (+ (/ (`KismetMathLibrary.VSize` (- _returnvalue_2 _returnvalue_3)) 2.0) 10.0)) "World" true)
      (`SplineComponent.RemoveSplinePoint` _spline_3 _returnvalue true))
    (`SplineComponent.SetClosedLoop` _spline_3 true true)
    (`SplineComponent.SetTangentAtSplinePoint` (`local.Spline`) 0 (`KismetMathLibrary.GetVectorArrayAverage` (`|MakeArray` (`SplineComponent.GetTangentAtSplinePoint` _spline_4 0 "World") (`SplineComponent.GetTangentAtSplinePoint` _spline_4 (- (`local.LockedSplinePoints`) 1) "World"))) "World" true)
    (else
      (bind _output_get (set `local.ContinueDrawing?` true))
      (return _output_get))))

(fn `ContinueOutline`
  (params (Spline :type "SplineComponent Object Reference") (MotionControlTrans :type "Transform Structure") (LocationType :type "/Game/Blueprints/Enum_MotionControllerData Enum" :default "NewEnumerator0") (SplinePoints :type "Integer (by ref)") (LastLocation :type "Vector Structure (by ref)") (`AutoCloseLoop?` :type Boolean) (`Flatten?` :type Boolean) (PointSpacing :type "Float (double-precision)" :default 10.0))
  (returns (`Finished?` :type Boolean))
  (locals (Finshed :type Boolean))
  (bind _splinepoints (`local.SplinePoints`))
  (bind _spline (`local.Spline`))
  (bind _splinepoints_2 (`local.SplinePoints`))
  (bind _spline_2 (`local.Spline`))
  (bind _spline_3 (`local.Spline`))
  (bind (_validlocation_ _location) (`self.LocationFromMotionController` (`local.LocationType`) (`local.MotionControlTrans`)))
  (bind (_returnvalue_x _returnvalue_y _returnvalue_z) (`KismetMathLibrary.BreakVector` (`SplineComponent.GetLocationAtSplinePoint` (`local.Spline`) 0 "World")))
  (bind _returnvalue (- (`local.SplinePoints`) 1))
  (bind _out (`self.FlattenVector` _location _returnvalue_z (`local.Flatten?`)))
  (bind _returnvalue_2 (- (`SplineComponent.GetDistanceAlongSplineAtSplinePoint` _spline (- _splinepoints_2 1)) (`SplineComponent.GetDistanceAlongSplineAtSplinePoint` _spline (- _splinepoints_2 2))))
  (bind _returnvalue_3 (- _out (`SplineComponent.GetLocationAtSplinePoint` (`local.Spline`) (- (`local.SplinePoints`) 2) "World")))
  (bind _returnvalue_4 (`KismetMathLibrary.Normal` (- (`SplineComponent.GetLocationAtSplinePoint` (`local.Spline`) (- (`local.SplinePoints`) 1) "World") (`SplineComponent.GetLocationAtSplinePoint` (`local.Spline`) (- (`local.SplinePoints`) 3) "World"))))
  (if `AutoCloseLoop?`
    (bind _continue (`self.CheckForLoop` Spline SplinePoints))
    (if _continue
      _
      (else
        (bind _output_get (set `local.Finshed` true))
        (return _output_get))))
  (if (and (>= (- (`SplineComponent.GetDistanceAlongSplineAtSplinePoint` _spline_3 (- _splinepoints 1)) (`SplineComponent.GetDistanceAlongSplineAtSplinePoint` _spline_3 (- _splinepoints 2))) (`local.PointSpacing`)) _validlocation_)
    (`SplineComponent.AddSplinePointAtIndex` (`local.Spline`) _out (`local.SplinePoints`) "World" true)
    (`/Engine/EditorBlueprintResources/StandardMacros.IncrementInt` (`local.SplinePoints`))
    (else
      (`SplineComponent.SetLocationAtSplinePoint` _spline_2 _returnvalue _out "World" true)
      (`SplineComponent.SetTangentAtSplinePoint` _spline_2 _returnvalue (* (`KismetMathLibrary.Normal` _returnvalue_3) _returnvalue_2) "World" true)
      (`SplineComponent.SetTangentsAtSplinePoint` (`local.Spline`) (- (`local.SplinePoints`) 2) (* _returnvalue_4 (`local.PointSpacing`)) (* _returnvalue_4 _returnvalue_2) "World" true)
      (`|VariableSetRef` (`local.LastLocation`) _returnvalue_3))))

(fn `FlattenVector`
  (params (InVec :type "Vector Structure") (Z :type "Float (double-precision)") (`Flatten?` :type Boolean))
  (returns (Out :type "Vector Structure"))
  (locals (Newvector :type "Vector Structure"))
  (if `Flatten?`
    (set `local.Newvector` (`KismetMathLibrary.MakeVector` (.x InVec) (.y InVec) Z))
    (else
      (set `local.Newvector` InVec)))
  (return (`local.Newvector`)))

(fn `LocationFromMotionController`
  (params (MotionControllerType :type "/Game/Blueprints/Enum_MotionControllerData Enum" :default "NewEnumerator0") (Transform :type "Transform Structure") (Offset :type "Float (double-precision)"))
  (returns (`ValidLocation?` :type Boolean) (Location :type "Vector Structure"))
  (locals (Location_ :type "Vector Structure") (`Valid?` :type Boolean))
  (bind (_transform_location _transform_rotation) (`KismetMathLibrary.BreakTransform` (`local.Transform`)))
  (bind _transform_location_2 (`KismetMathLibrary.BreakTransform` (`local.Transform`)))
  (bind (_transform_location_3 _transform_rotation_2) (`KismetMathLibrary.BreakTransform` (`local.Transform`)))
  (switch `/Game/Blueprints/Enum_MotionControllerData` MotionControllerType
    (:`NewEnumerator0`
      (set `local.Location_` _transform_location_2)
      (set `local.Valid?` true))
    (:`NewEnumerator1`
      (set `local.Location_` (+ _transform_location (* (`KismetMathLibrary.GetForwardVector` _transform_rotation) (`local.Offset`))))
      (set `local.Valid?` true))
    (:`NewEnumerator2`
      (bind _outhit (`KismetSystemLibrary.LineTraceSingleForObjects` :`Start` _transform_location_3 :`End` (+ _transform_location_3 (* (`KismetMathLibrary.GetForwardVector` _transform_rotation_2) 500.0)) :`ObjectTypes` (`|MakeArray` "ObjectTypeQuery1" :!type "EObjectTypeQuery Enum") :`bIgnoreSelf` false :`DrawTime` 2.0))
      (bind _output_get (set `local.Valid?` (`GameplayStatics.BreakHitResult` _outhit)))
      (if _output_get
        (set `local.Location_` (`.Location` (`GameplayStatics.BreakHitResult` _outhit))))))
  (return (`local.Valid?`) (`local.Location_`)))