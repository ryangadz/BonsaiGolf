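; Blueprint function library with a function that picks the next point for a spline that follows world-static surfaces.
; It steps one segment length from the last point in a seeded random direction within a cone around the last direction.
; Line traces through that point along icosahedron-derived offsets find the nearest surface hit.
; It returns that location and normal as the up vector, flagging none found when the location stays zero.
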(fn `FindNextSplineLocation`
  (params (SegmentLength :type "Float (double-precision)") (LastLocation :type "Vector Structure") (LastDirection :type "Vector Structure") (Seed :type Integer))
  (returns (NextLocation :type "Vector Structure") (NextUpVector :type "Vector Structure") (NoneFound :type Boolean))
  (locals (PreLocation :type "Vector Structure") (ClosestDistance :type "Float (double-precision)") (NextLoc :type "Vector Structure") (NextUpVec :type "Vector Structure"))
  (bind _prelocation (`local.PreLocation`))
  (bind _nextloc (`local.NextLoc`))
  (bind _output_get (set `local.ClosestDistance` (* SegmentLength 1.5)))
  (set `local.PreLocation` (+ LastLocation (* (`KismetMathLibrary.RandomUnitVectorInConeInDegreesFromStream` LastDirection 45.0 (`KismetMathLibrary.MakeRandomStream` Seed)) SegmentLength)))
  (for _array_element (`STC_MathFunctions.CalcIcosahedron` _output_get)
    (bind (_outhit _returnvalue) (`KismetSystemLibrary.LineTraceSingleForObjects` null (- _prelocation _array_element) (+ _prelocation _array_element) (`|MakeArray` "ObjectTypeQuery1" :!type "EObjectTypeQuery Enum") true))
    (if _returnvalue
      (bind _returnvalue_2 (`KismetMathLibrary.VSize` (- (`.Location` (`GameplayStatics.BreakHitResult` _outhit)) (`local.PreLocation`))))
      (if (<= _returnvalue_2 (`local.ClosestDistance`))
        (set `local.ClosestDistance` _returnvalue_2)
        (set `local.NextLoc` (`.Location` (`GameplayStatics.BreakHitResult` _outhit)))
        (set `local.NextUpVec` (`.Normal` (`GameplayStatics.BreakHitResult` _outhit))))))
  (return _nextloc (`local.NextUpVec`) (== _nextloc (0.0 0.0 0.0))))