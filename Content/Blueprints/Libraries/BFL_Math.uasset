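; Math Blueprint function library whose CircleFrom3Points function is meant to find a circle's center, radius and existence from three points.
; It flattens points to XY, builds a line from Point1, Point2 and their perpendicular, then runs a line-plane intersection.
; The function looks unfinished: no plane is wired in, Point3 feeds only unused nodes, and Radius returns the intersection's T rather than a distance.
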(fn `CircleFrom3Points`
  (params (Point1 :type "Vector Structure") (Point2 :type "Vector Structure") (Point3 :type "Vector Structure"))
  (returns (`center point` :type "Vector Structure") (Radius :type "Float (double-precision)") (`Circle Exists` :type Boolean))
  (bind _returnvalue (`KismetMathLibrary.MakeVector` Point1_X Point1_Y))
  (bind _returnvalue_2 (- _returnvalue (`KismetMathLibrary.MakeVector` Point2_X Point2_Y)))
  (bind _returnvalue_3 (+ (+ _returnvalue (* _returnvalue_2 (/ (`KismetMathLibrary.VSize` _returnvalue_2) 2.0))) (`KismetMathLibrary.Cross_VectorVector` (0.0 0.0 1.0) _returnvalue_2)))
  (bind (_t _intersection _returnvalue_4) (`KismetMathLibrary.LinePlaneIntersection` _returnvalue_3 (* _returnvalue_3 100.0) (make `Plane` 0.0)))
  (return _intersection _t _returnvalue_4))