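; Blueprint function library that packs a set number of circles inside a spline in an Apollonian style, outputting locations and radii.
; ApollonianPacking builds a point grid from the spline, then calls GetNextCircle once per circle.
; GetNextCircle greedily scores uncovered points by distance to the spline and placed circles, sizing each circle from those distances.
; Grid points inside each new circle are flagged -1 so later searches skip them.
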(fn `ApollonianPacking`
  (params (Locations :type "Array of Vector Structure (by ref)") (Radii :type "Array of Float (double-precision) (by ref)") (Spline :type "SplineComponent Object Reference") (Number :type Integer :default 5))
  (locals (Verts :type "Array of Vector Structure") (InsideIndices :type "Array of Integer"))
  (`KismetArrayLibrary.Array_Resize` Locations Number)
  (`KismetArrayLibrary.Array_Resize` Radii Number)
  (bind (_insideindices _gridx _verts) (`/Game/Blueprints/Libraries/BFL_MeshBuilding.MakePointGrid` Spline))
  (set `local.InsideIndices` _insideindices)
  (set `local.Verts` _verts)
  (for _index (range Number)
    (bind (_nextlocation _nextradius) (`self.GetNextCircle` (`local.Verts`) (`local.InsideIndices`) (`local.Locations`) Radii (`local.Spline`) _index))
    (`KismetArrayLibrary.Array_Set` (`local.Locations`) _index _nextlocation)
    (`KismetArrayLibrary.Array_Set` (`local.Radii`) _index _nextradius)))

(fn `GetNextCircle`
  (params (Verts :type "Array of Vector Structure") (InsideIndices :type "Array of Integer (by ref)") (Locations :type "Array of Vector Structure (by ref)") (Radii :type "Array of Float (double-precision) (by ref)") (Spline :type "SplineComponent Object Reference") (Index :type Integer))
  (returns (NextLocation :type "Vector Structure") (NextRadius :type "Float (double-precision)"))
  (locals (VertsIndex :type Integer) (LengthToEdge :type "Float (double-precision)") (RadiusTemp :type "Float (double-precision)") (SumClosestPrevious :type "Float (double-precision)") (NextLocation_ :type "Vector Structure") (NextRadius_ :type "Float (double-precision)"))
  (bind _returnvalue (+ (`local.LengthToEdge`) (`local.RadiusTemp`)))
  (bind _output (`|GetArrayItem` (`local.Verts`) (`local.VertsIndex`)))
  (for _index (range (`KismetArrayLibrary.Array_Length` InsideIndices))
    (set `local.VertsIndex` _index)
    (if (== (`|GetArrayItem` (`local.InsideIndices`) (`local.VertsIndex`)) 0)
      (set `local.LengthToEdge` (`KismetMathLibrary.VSize` (- _output (`SplineComponent.FindLocationClosestToWorldLocation` (`local.Spline`) _output "World"))))
      (if (> (`local.Index`) 0)
        (set `local.RadiusTemp` 10000.0)
        (for _index_2 (range (`KismetArrayLibrary.Array_Length` (`local.Locations`)))
          (bind _returnvalue_2 (- (`KismetMathLibrary.VSize` (- (`|GetArrayItem` (`local.Verts`) (`local.VertsIndex`)) (`|GetArrayItem` (`local.Locations`) _index_2))) (`|GetArrayItem` (`local.Radii`) _index_2)))
          (if (and (> _returnvalue_2 0.0) (< _returnvalue_2 (`local.LengthToEdge`)) (< _returnvalue_2 (`local.RadiusTemp`)))
            (set `local.RadiusTemp` _returnvalue_2)))
        (if (> _returnvalue (`local.SumClosestPrevious`))
          (set `local.SumClosestPrevious` _returnvalue)
          (if (< (`local.SumClosestPrevious`) (* (`local.LengthToEdge`) 2.0))
            (set `local.NextRadius_` (`local.RadiusTemp`))
            (else
              (set `local.NextRadius_` (`local.LengthToEdge`))))
          (set `local.NextLocation_` (`|GetArrayItem` (`local.Verts`) (`local.VertsIndex`))))
        (elif (> (`local.LengthToEdge`) (`local.NextRadius_`))
          (set `local.NextRadius_` (`local.LengthToEdge`))
          (set `local.NextLocation_` (`|GetArrayItem` (`local.Verts`) (`local.VertsIndex`)))))))
  (`KismetArrayLibrary.Array_Set` (`local.Radii`) (`local.Index`) (`local.NextRadius_`) true)
  (`KismetArrayLibrary.Array_Set` (`local.Locations`) (`local.Index`) (`local.NextLocation_`) true)
  (for _index_3 (range (`KismetArrayLibrary.Array_Length` (`local.InsideIndices`)))
    (if (and (== (`|GetArrayItem` (`local.InsideIndices`) _index_3) 0) (< (`KismetMathLibrary.VSize` (- (`|GetArrayItem` (`local.Verts`) _index_3) (`local.NextLocation_`))) (`local.NextRadius_`)))
      (`KismetArrayLibrary.Array_Set` (`local.InsideIndices`) _index_3 -1)))
  (return (`local.NextLocation_`) (`local.NextRadius_`)))