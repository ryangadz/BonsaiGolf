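; Blueprint function library that computes vertices and triangle indices for procedural meshes from spline outlines, disks and cylinders.
; MakePointGrid lays a triangular lattice over spline bounds, classifying points as inside, edge or outside; BuildMeshFromOutline triangulates it, skipping outside and all-edge triangles.
; MakePointGridS, unused here, stores closest spline locations for edge points, whereas MakePointGrid stores spline directions.
; NearestPointOnGrid searches points by squared distance; SnapPointGrid and CalculateHoleVerts are unfinished stubs.
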(fn `BuildMeshFromOutline`
  (params (SplineWithMesh :type "SplineWithMesh Object Reference") (TriangleSize :type "Float (double-precision)" :default 5.0))
  (returns (Verts :type "Array of Vector Structure") (Triangles :type "Array of Integer"))
  (locals (GridX :type Integer) (GridPoints :type "Array of Integer") (Index :type Integer) (TrianglesL :type "Array of Integer"))
  (bind _gridpoints (`local.GridPoints`))
  (bind _index (`local.Index`))
  (bind _index_2 (`local.Index`))
  (bind _trianglesl (`local.TrianglesL`))
  (bind _gridpoints_2 (`local.GridPoints`))
  (bind _index_3 (`local.Index`))
  (bind _trianglesl_2 (`local.TrianglesL`))
  (bind _output (`|GetArrayItem` _gridpoints (`local.Index`)))
  (bind _returnvalue (- (`local.Index`) (+ (`local.GridX`) 1)))
  (bind _returnvalue_2 (- _index_3 (+ (`local.GridX`) 1)))
  (bind _output_2 (`|GetArrayItem` _gridpoints (+ _index 1)))
  (bind _output_3 (`|GetArrayItem` _gridpoints_2 _returnvalue_2))
  (bind _output_4 (`|GetArrayItem` _gridpoints_2 (- _returnvalue_2 -1)))
  (bind _returnvalue_3 (- _index (- (+ (`local.GridX`) 1) (mod (/ (`local.Index`) (+ (`local.GridX`) 1)) 2))))
  (bind _returnvalue_4 (+ (+ (* (mod (/ (`local.Index`) (+ (`local.GridX`) 1)) 2) -1) 1) _index_3))
  (bind _output_5 (`|GetArrayItem` _gridpoints _returnvalue_3))
  (bind _output_6 (`|GetArrayItem` _gridpoints_2 _returnvalue_4))
  (bind (_points _verts _gridx) (`self.MakePointGrid` SplineWithMesh TriangleSize))
  (set `local.GridPoints` _points)
  (bind _output_get (set `local.GridX` _gridx))
  (for _index_4 (range (+ _output_get 1) (+ (- (`KismetArrayLibrary.Array_Length` (`local.GridPoints`)) 2) 1))
    (set `local.Index` _index_4)
    (`|ExecutionSequence`
      (:`then_0`
        (if (and (!= _output_6 -1) (!= _output_3 -1) (!= _output_4 -1) (!= (+ _output_6 _output_3 _output_4) 3))
          (`KismetArrayLibrary.Array_Add` _trianglesl_2 _returnvalue_4)
          (`KismetArrayLibrary.Array_Add` _trianglesl_2 (- _returnvalue -1))
          (`KismetArrayLibrary.Array_Add` _trianglesl_2 _returnvalue)))
      (:`then_1`
        (if (and (!= _output -1) (!= _output_2 -1) (!= _output_5 -1) (!= (+ _output _output_2 _output_5) 3))
          (`KismetArrayLibrary.Array_Add` _trianglesl _index_2)
          (`KismetArrayLibrary.Array_Add` _trianglesl (+ _index_2 1))
          (`KismetArrayLibrary.Array_Add` _trianglesl _returnvalue_3)))))
  (return _verts (`local.TrianglesL`)))

(fn `CalculateHoleVerts`)

(fn `MakeCylinderVerts`
  (params (CenterPoint :type "Vector Structure") (Radius :type "Float (double-precision)" :default 1.0) (Sides :type Integer :default 6) (Height :type "Float (double-precision)"))
  (returns (Vertices :type "Array of Vector Structure") (Triangles :type "Array of Integer"))
  (locals (Verts :type "Array of Vector Structure") (Angle :type "Float (double-precision)") (Tris :type "Array of Integer"))
  (bind _radius (`local.Radius`))
  (bind _verts (`local.Verts`))
  (bind _tris (`local.Tris`))
  (bind _tris_2 (`local.Tris`))
  (bind _sides (`local.Sides`))
  (`KismetArrayLibrary.Array_Resize` (`local.Verts`) (* Sides 2))
  (set `local.Angle` (/ 360.0 (`KismetMathLibrary.Conv_IntToDouble` Sides)))
  (for _index (range Sides)
    (bind _returnvalue (* _index (`local.Angle`)))
    (bind _returnvalue_2 (+ (`KismetMathLibrary.MakeVector` (* (`KismetMathLibrary.DegCos` _returnvalue) _radius) (* _radius (`KismetMathLibrary.DegSin` _returnvalue))) (`local.CenterPoint`)))
    (`KismetArrayLibrary.Array_Set` _verts _index _returnvalue_2)
    (`KismetArrayLibrary.Array_Set` _verts (+ _index (`local.Sides`)) (+ _returnvalue_2 (`KismetMathLibrary.MakeVector` 0.0 0.0 (`local.Height`)))))
  (for _index_2 (range (* (- (`local.Sides`) 1) -1) 1)
    (bind _returnvalue_3 (`KismetMathLibrary.Abs_Int` _index_2))
    (`KismetArrayLibrary.Array_Add` _tris_2 _returnvalue_3)
    (bind _returnvalue_4 (+ _returnvalue_3 _sides))
    (`KismetArrayLibrary.Array_Add` _tris_2 _returnvalue_4)
    (bind _returnvalue_5 (+ _sides (mod (+ _returnvalue_4 1) _sides)))
    (`KismetArrayLibrary.Array_Add` _tris_2 _returnvalue_5)
    (`KismetArrayLibrary.Array_Add` _tris _returnvalue_5)
    (`KismetArrayLibrary.Array_Add` _tris (mod (+ _returnvalue_3 1) (`local.Sides`)))
    (`KismetArrayLibrary.Array_Add` _tris _returnvalue_3))
  (return (`local.Verts`) (`local.Tris`)))

(fn `MakePlanarDiskVerts`
  (params (CenterPoint :type "Vector Structure") (Radius :type "Float (double-precision)" :default 1.0) (Sides :type Integer :default 6))
  (returns (Vertices :type "Array of Vector Structure") (Triangles :type "Array of Integer"))
  (locals (Verts :type "Array of Vector Structure") (Angle :type "Float (double-precision)") (Tris :type "Array of Integer"))
  (bind _verts (`local.Verts`))
  (bind _radius (`local.Radius`))
  (bind _tris (`local.Tris`))
  (`KismetArrayLibrary.Array_Resize` _verts (+ Sides 1))
  (`KismetArrayLibrary.Array_Set` _verts (`local.Sides`) (`local.CenterPoint`))
  (set `local.Angle` (/ 360.0 (`KismetMathLibrary.Conv_IntToDouble` (`local.Sides`))))
  (for _index (range (`local.Sides`))
    (bind _returnvalue (* _index (`local.Angle`)))
    (`KismetArrayLibrary.Array_Set` (`local.Verts`) _index (+ (`KismetMathLibrary.MakeVector` (* (`KismetMathLibrary.DegCos` _returnvalue) _radius) (* _radius (`KismetMathLibrary.DegSin` _returnvalue))) (`local.CenterPoint`))))
  (for _index_2 (range (`local.Sides`))
    (`KismetArrayLibrary.Array_Add` _tris _index_2)
    (`KismetArrayLibrary.Array_Add` _tris (mod (+ _index_2 1) (`local.Sides`)))
    (`KismetArrayLibrary.Array_Add` _tris))
  (return (`local.Verts`) (`local.Tris`)))

(fn `MakePointGrid`
  (params (SplineWithMesh :type "SplineWithMesh Object Reference") (TriangleSize :type "Float (double-precision)" :default 2.0))
  (returns (points :type "Array of Integer") (Verts :type "Array of Vector Structure") (GridX :type Integer))
  (locals (PointIndex :type "Array of Integer") (CurrentPoint :type Integer :default -1) (Vertices :type "Array of Vector Structure") (`60 Degrees` :type "Float (double-precision)" :default 60.0) (NumX :type Integer) (NumY :type Integer) (IndexY :type Integer) (CurrentLoc :type "Vector Structure") (IndexX :type Integer) (`Inside?` :type Boolean) (`Edge?` :type Boolean) (CurrentEdgeLoc :type "Vector Structure"))
  (bind _returnvalue (`KismetMathLibrary.FClamp` TriangleSize 2.0 30.0))
  (bind _numy (`local.NumY`))
  (bind _numx (`local.NumX`))
  (bind _returnvalue_2 (`KismetMathLibrary.FClamp` (`local.TriangleSize`) 2.0 30.0))
  (bind _returnvalue_3 (`SplineComponent.FindDirectionClosestToWorldLocation` (`local.SplineWithMesh`) (`local.CurrentLoc`) "World"))
  (bind _returnvalue_4 (/ _returnvalue_2 2.0))
  (bind _returnvalue_5 (- (`SplineComponent.FindLocationClosestToWorldLocation` (`local.SplineWithMesh`) (`local.CurrentLoc`) "World") (`local.CurrentLoc`)))
  (set `local.NumX` (`KismetMathLibrary.FCeil` (+ (/ (.x (`.BoxExtent` (`KismetSystemLibrary.GetComponentBounds` SplineWithMesh))) _returnvalue) 1.0)))
  (set `local.NumY` (`KismetMathLibrary.FCeil` (+ (/ (.y (`.BoxExtent` (`KismetSystemLibrary.GetComponentBounds` SplineWithMesh))) (* (/ _returnvalue 2.0) (`KismetMathLibrary.DegTan` (`local.60 Degrees`)))) 1.0)))
  (`|ExecutionSequence`
    (:`then_0`
      (for _index (range (* _numy -1) (+ _numy 1))
        (set `local.IndexY` _index)
        (for _index_2 (range (* _numx -1) (+ _numx 1))
          (set `local.IndexX` _index_2)
          (set `local.CurrentLoc` (`KismetMathLibrary.MakeVector` (+ (.x (`KismetSystemLibrary.GetComponentBounds` (`local.SplineWithMesh`))) (* (`local.IndexX`) _returnvalue_2) (* (mod (`KismetMathLibrary.Abs_Int` (+ (`local.IndexY`) (`local.NumY`))) 2) _returnvalue_4)) (+ (.y (`KismetSystemLibrary.GetComponentBounds` (`local.SplineWithMesh`))) (* (`local.IndexY`) (* _returnvalue_4 (`KismetMathLibrary.DegTan` (`local.60 Degrees`))))) (.z (`KismetSystemLibrary.GetComponentBounds` (`local.SplineWithMesh`)))))
          (set `local.Inside?` (> (`KismetMathLibrary.Dot_VectorVector` _returnvalue_5 (`KismetMathLibrary.Cross_VectorVector` (0.0 0.0 1.0) _returnvalue_3)) 0.0))
          (set `local.Edge?` (< (`KismetMathLibrary.VSize` _returnvalue_5) (`local.TriangleSize`)))
          (set `local.CurrentEdgeLoc` _returnvalue_3)
          (`/Engine/EditorBlueprintResources/StandardMacros.IncrementInt` (`local.CurrentPoint`)
            (:`  `
              (if (`local.Inside?`)
                ;[0.05399 1 0] Inside of Outline
                (`KismetArrayLibrary.Array_Set` (`local.Vertices`) (`local.CurrentPoint`) (`local.CurrentLoc`) true)
                (`KismetArrayLibrary.Array_Set` (`local.PointIndex`) (`local.CurrentPoint`) 0 true)
                (elif (`local.Edge?`)
                  ;[1 0.9181 0] Edge of Outline
                  (`KismetArrayLibrary.Array_Set` (`local.Vertices`) (`local.CurrentPoint`) (`local.CurrentEdgeLoc`) true)
                  (`KismetArrayLibrary.Array_Set` (`local.PointIndex`) (`local.CurrentPoint`) 1 true)
                  (else
                    ;[1 0 0] Outside of Outline
                    (`KismetArrayLibrary.Array_Set` (`local.Vertices`) (`local.CurrentPoint`) (`local.CurrentLoc`) true)
                    (`KismetArrayLibrary.Array_Set` (`local.PointIndex`) (`local.CurrentPoint`) -1 true)))))))))
    (:`then_1`
      (return (`local.PointIndex`) (`local.Vertices`) (* (`local.NumX`) 2)))))

(fn `MakePointGridS`
  (params (SplineWithMesh :type "SplineComponent Object Reference") (TriangleSize :type "Float (double-precision)" :default 2.0))
  (returns (points :type "Array of Integer") (Verts :type "Array of Vector Structure") (GridX :type Integer))
  (locals (PointIndex :type "Array of Integer") (CurrentPoint :type Integer :default -1) (Vertices :type "Array of Vector Structure") (`60 Degrees` :type "Float (double-precision)" :default 60.0) (NumX :type Integer) (NumY :type Integer) (IndexY :type Integer) (CurrentLoc :type "Vector Structure") (IndexX :type Integer) (`Inside?` :type Boolean) (`Edge?` :type Boolean) (CurrentEdgeLoc :type "Vector Structure"))
  (bind _returnvalue (`KismetMathLibrary.FClamp` TriangleSize 2.0 30.0))
  (bind _numy (`local.NumY`))
  (bind _numx (`local.NumX`))
  (bind _returnvalue_2 (`KismetMathLibrary.FClamp` (`local.TriangleSize`) 2.0 30.0))
  (bind _returnvalue_3 (`SplineComponent.FindLocationClosestToWorldLocation` (`local.SplineWithMesh`) (`local.CurrentLoc`) "World"))
  (bind _returnvalue_4 (/ _returnvalue_2 2.0))
  (bind _returnvalue_5 (- _returnvalue_3 (`local.CurrentLoc`)))
  (set `local.NumX` (`KismetMathLibrary.FCeil` (+ (/ (.x (`.BoxExtent` (`KismetSystemLibrary.GetComponentBounds` SplineWithMesh))) _returnvalue) 1.0)))
  (set `local.NumY` (`KismetMathLibrary.FCeil` (+ (/ (.y (`.BoxExtent` (`KismetSystemLibrary.GetComponentBounds` SplineWithMesh))) (* (/ _returnvalue 2.0) (`KismetMathLibrary.DegTan` (`local.60 Degrees`)))) 1.0)))
  (`|ExecutionSequence`
    (:`then_0`
      (for _index (range (* _numy -1) (+ _numy 1))
        (set `local.IndexY` _index)
        (for _index_2 (range (* _numx -1) (+ _numx 1))
          (set `local.IndexX` _index_2)
          (set `local.CurrentLoc` (`KismetMathLibrary.MakeVector` (+ (.x (`KismetSystemLibrary.GetComponentBounds` (`local.SplineWithMesh`))) (* (`local.IndexX`) _returnvalue_2) (* (mod (`KismetMathLibrary.Abs_Int` (+ (`local.IndexY`) (`local.NumY`))) 2) _returnvalue_4)) (+ (.y (`KismetSystemLibrary.GetComponentBounds` (`local.SplineWithMesh`))) (* (`local.IndexY`) (* _returnvalue_4 (`KismetMathLibrary.DegTan` (`local.60 Degrees`))))) (.z (`KismetSystemLibrary.GetComponentBounds` (`local.SplineWithMesh`)))))
          (set `local.CurrentEdgeLoc` _returnvalue_3)
          (set `local.Inside?` (> (`KismetMathLibrary.Dot_VectorVector` _returnvalue_5 (`KismetMathLibrary.Cross_VectorVector` (0.0 0.0 1.0) (`SplineComponent.FindDirectionClosestToWorldLocation` (`local.SplineWithMesh`) (`local.CurrentLoc`) "World"))) 0.0))
          (set `local.Edge?` (< (`KismetMathLibrary.VSize` _returnvalue_5) (`local.TriangleSize`)))
          (`/Engine/EditorBlueprintResources/StandardMacros.IncrementInt` (`local.CurrentPoint`)
            (:`  `
              (if (`local.Inside?`)
                ;[0.05399 1 0] Inside of Outline
                (`KismetArrayLibrary.Array_Set` (`local.Vertices`) (`local.CurrentPoint`) (`local.CurrentLoc`) true)
                (`KismetArrayLibrary.Array_Set` (`local.PointIndex`) (`local.CurrentPoint`) 0 true)
                (elif (`local.Edge?`)
                  ;[1 0.9181 0] Edge of Outline
                  (`KismetArrayLibrary.Array_Set` (`local.Vertices`) (`local.CurrentPoint`) (`local.CurrentEdgeLoc`) true)
                  (`KismetArrayLibrary.Array_Set` (`local.PointIndex`) (`local.CurrentPoint`) 1 true)
                  (else
                    ;[1 0 0] Outside of Outline
                    (`KismetArrayLibrary.Array_Set` (`local.Vertices`) (`local.CurrentPoint`) (`local.CurrentLoc`) true)
                    (`KismetArrayLibrary.Array_Set` (`local.PointIndex`) (`local.CurrentPoint`) -1 true)))))))))
    (:`then_1`
      (return (`local.PointIndex`) (`local.Vertices`) (* (`local.NumX`) 2)))))

(fn `NearestPointOnGrid`
  (params (`Point Grid` :type "Array of Vector Structure") (`Desired Point` :type "Vector Structure") (`Triangle SIze` :type "Float (double-precision)"))
  (returns (`Nearest Point` :type "Vector Structure") (`Nearest Point Index` :type Integer))
  (locals (NearestPoint :type "Vector Structure") (NearestIndex :type Integer) (ClosestDisSquared :type "Float (double-precision)"))
  (set `local.ClosestDisSquared` `Triangle SIze`)
  (for (_array_element _array_index) `Point Grid`
    (bind _returnvalue (`KismetMathLibrary.VSizeSquared` (- (`local.Desired Point`) _array_element)))
    (if (< _returnvalue (`local.ClosestDisSquared`))
      (set `local.ClosestDisSquared` _returnvalue)
      (set `local.NearestPoint` _array_element)
      (set `local.NearestIndex` _array_index)))
  (return (`local.NearestPoint`) (`local.NearestIndex`)))

(fn `SnapPointGrid`
  (params (`Point Grid` :type "Array of Vector Structure") (Origin :type "Vector Structure") (Location :type "Vector Structure") (TriangleSize :type Integer))
  ;[1 0 0] this doesnt make sense for multiple holes
  (for (_array_element _array_index) `Point Grid`
    (`KismetArrayLibrary.Array_Set` `Point Grid` _array_index (+ _array_element (0.0 0.0 0.0)))))