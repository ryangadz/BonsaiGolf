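; BP_MeshTest is a test actor for procedural mesh generation and collision tracing.
; The construction script builds a single equilateral triangle with collision and a concrete material; its planar disk vertex result goes unused.
; Each tick, a short vertical debug trace against WorldStatic objects sweeps sinusoidally along Y through the actor's location, without ignoring the actor itself.
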(event `self.ReceiveTick`
  (params (DeltaSeconds :type "Float (single-precision)"))
  (bind (_returnvalue_x _returnvalue_y _returnvalue_z) (`KismetMathLibrary.BreakVector` (`self.K2_GetActorLocation`)))
  (bind _returnvalue (+ (* (`KismetMathLibrary.DegSin` (* (`KismetSystemLibrary.GetGameTimeInSeconds`) 360.0)) 20.0) _returnvalue_y))
  (`KismetSystemLibrary.LineTraceSingleForObjects` :`Start` (`KismetMathLibrary.MakeVector` _returnvalue_x _returnvalue (+ _returnvalue_z 10.0)) :`End` (`KismetMathLibrary.MakeVector` _returnvalue_x _returnvalue (- _returnvalue_z 10.0)) :`ObjectTypes` (`|MakeArray` "ObjectTypeQuery1" :!type "EObjectTypeQuery Enum") :`DrawDebugType` "ForOneFrame" :`bIgnoreSelf` false))

(fn `UserConstructionScript`
  (`/Game/Blueprints/Libraries/BFL_MeshBuilding.MakePlanarDiskVerts` (0.0 0.0 0.0) 15.0 24)
  (bind _returnvalue (`AddComponent|NODE_AddProceduralMeshComponent-0` :`RelativeTransform` (`KismetMathLibrary.MakeTransform` (0.0 0.0 0.0) (struct))))
  (`ProceduralMeshComponent.CreateMeshSection_LinearColor` :`self` _returnvalue :`Vertices` (`|MakeArray` (15.0 0.0 0.0) (`KismetMathLibrary.RotateAngleAxis` (15.0 0.0 0.0) 240.0 (0.0 0.0 1.0)) (`KismetMathLibrary.RotateAngleAxis` (15.0 0.0 0.0) 120.0 (0.0 0.0 1.0))) :`Triangles` (`|MakeArray` 0 1 2) :`bCreateCollision` true)
  (`PrimitiveComponent.SetMaterial` _returnvalue 0 "/Game/Materials/M_Concrete.M_Concrete"))