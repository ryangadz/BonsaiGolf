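; BP_Tree is an actor that procedurally grows a single wandering spline of meshes at runtime.
; BeginPlay adds a SplineWithMesh component at a random rotation.
; After a short game-time delay, Tick appends one point per frame up to a cap, stepping a fixed distance along a random cone around the last point's direction.
; Each new point triggers the component's AddMesh; leftover bobbing and debug-print nodes never run.
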(event `self.ReceiveBeginPlay`
  (bind _returnvalue (`AddComponent|NODE_AddSplineWithMesh-0` :`RelativeTransform` (`KismetMathLibrary.MakeTransform` (0.0 0.0 0.0) (`KismetMathLibrary.RandomRotator` false))))
  (set `self.Spline with mesh` _returnvalue))

(event `self.ReceiveTick`
  (params (DeltaSeconds :type "Float (single-precision)"))
  (bind _spline_with_mesh (`self.Spline with mesh`))
  (bind _returnvalue (`SplineComponent.GetNumberOfSplinePoints` _spline_with_mesh))
  (bind _returnvalue_2 (- _returnvalue 1))
  (if (> (`KismetSystemLibrary.GetGameTimeInSeconds`) 10.0)
    (if (< (`SplineComponent.GetNumberOfSplinePoints` (`self.Spline with mesh`)) 350)
      (`SplineComponent.AddSplinePointAtIndex` _spline_with_mesh (+ (`SplineComponent.GetLocationAtSplinePoint` _spline_with_mesh _returnvalue_2 "World") (* (`KismetMathLibrary.RandomUnitVectorInConeInDegrees` (`SplineComponent.GetDirectionAtSplinePoint` _spline_with_mesh _returnvalue_2 "World") 30.0) (`KismetMathLibrary.RandomFloatInRange` 10.0 10.0))) _returnvalue "World" true)
      (`SplineWithMesh.AddMesh` (`self.Spline with mesh`) self))))

(fn `UserConstructionScript`)