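; Paint stroke actor that gives a spline-based mesh a varied color and look, built entirely in the construction script.
; A random stream seeded from the spline's summed world coordinates jitters the Color hue and picks one of twenty variant numbers, so variation follows placement.
; Each rail segment gets a dynamic material instance carrying variant, color, segment index and segment count, stored in the SplineWithMesh material array.
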(fn `UserConstructionScript`
  (bind (_h _s _v _a) (`KismetMathLibrary.RGBToHSV` (`self.Color`)))
  (bind (_returnvalue_x _returnvalue_y _returnvalue_z) (`KismetMathLibrary.BreakVector` (`SceneComponent.K2_GetComponentLocation` (`self.SplineWithMesh`))))
  (bind _number (`SplineTwistCorrectBPLibrary.CalcRailLength` (`self.SplineWithMesh`) 100.0))
  (bind (_returnvalue_x_2 _returnvalue_y_2 _returnvalue_z_2) (`KismetMathLibrary.BreakVector` (`SceneComponent.K2_GetComponentLocation` (`self.SplineWithMesh`))))
  (set `self.Color` (`KismetMathLibrary.HSVToRGB` (mod (+ _h (- 360.0 (`KismetMathLibrary.RandomFloatInRangeFromStream` -30.0 30.0 (`KismetMathLibrary.MakeRandomStream` (`KismetMathLibrary.FTrunc` (+ _returnvalue_x_2 _returnvalue_y_2 _returnvalue_z_2)))))) 359.0) _s _v _a))
  (set `self.Random` (`KismetMathLibrary.RandomIntegerInRangeFromStream` 0 19 (`KismetMathLibrary.MakeRandomStream` (`KismetMathLibrary.FTrunc` (+ _returnvalue_x _returnvalue_y _returnvalue_z)))))
  (for _index (range _number)
    (bind _returnvalue (`KismetMaterialLibrary.CreateDynamicMaterialInstance` (`self.Material`)))
    (`MaterialInstanceDynamic.SetScalarParameterValue` _returnvalue "Num" (`KismetMathLibrary.Conv_IntToDouble` (`self.Random`)))
    (`MaterialInstanceDynamic.SetScalarParameterValue` _returnvalue "TotalSec" (`KismetMathLibrary.Conv_IntToDouble` _number))
    (`MaterialInstanceDynamic.SetScalarParameterValue` _returnvalue "CurrentSec" (`KismetMathLibrary.Conv_IntToDouble` _index))
    (`MaterialInstanceDynamic.SetVectorParameterValue` _returnvalue "Color" (`self.Color`))
    (`KismetArrayLibrary.Array_Set` (`SplineWithMesh.MaterialArray` (`self.SplineWithMesh`)) _index _returnvalue true)))