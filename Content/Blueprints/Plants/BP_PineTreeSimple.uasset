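; BP_PineTreeSimple is a procedurally built pine tree, generated entirely in the Construction Script.
; It rebuilds a slightly bent three-point spline and calls AddMesh on it, then adds branches as Foliage instances along it.
; A BranchDistribution curve sets each branch's position and shrinking scale, while spline direction gives roll and pitch and golden-angle yaw steps spiral them.
; It prints the actor's bounds extent afterwards.
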(fn `UserConstructionScript`
  (bind _numberofbranches (`self.NumberOfBranches`))
  (bind _spline (`self.Spline`))
  (bind _spline_2 (`self.Spline`))
  (`SplineComponent.ClearSplinePoints` _spline true)
  (`SplineComponent.AddSplinePointAtIndex` _spline (0.0 0.0 0.0) 0 "Local" true)
  (`SplineComponent.AddSplinePointAtIndex` _spline (0.0 -1.0 10.0) 1 "Local" true)
  (`SplineComponent.AddSplinePointAtIndex` _spline (-1.0 -2.0 20.0) 2 "Local" true)
  (`SplineWithMesh.AddMesh` _spline null)
  (for _index (range (+ _numberofbranches 1))
    (bind _returnvalue (/ (`KismetMathLibrary.Conv_IntToDouble` _index) (`KismetMathLibrary.Conv_IntToDouble` _numberofbranches)))
    (bind _returnvalue_2 (`CurveFloat.GetFloatValue` (`self.BranchDistribution`) _returnvalue))
    (bind (_returnvalue_roll _returnvalue_pitch) (`KismetMathLibrary.BreakRotator` (`KismetMathLibrary.MakeRotFromZ` (`SplineComponent.GetDirectionAtTime` _spline_2 _returnvalue "Local" false))))
    (`InstancedStaticMeshComponent.AddInstance` (`self.Foliage`) (`KismetMathLibrary.MakeTransform` (`SplineComponent.GetLocationAtTime` _spline_2 _returnvalue_2 "Local" false) (`KismetMathLibrary.MakeRotator` _returnvalue_roll _returnvalue_pitch (* _index 137.5)) (`KismetMathLibrary.Conv_DoubleToVector` (- 1.1 _returnvalue_2)))))
  (`KismetSystemLibrary.PrintString` (`KismetStringLibrary.Conv_VectorToString` (`.BoxExtent` (`self.GetActorBounds` self false)))))