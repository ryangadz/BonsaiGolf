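; Procedural tree actor that grows roots and a leafy, branching crown in its construction script, seeded by the last character of its name.
; NewRoot recursively builds spline-mesh segments, spacing child branches around their parent at the 137.5° golden angle.
; Roots follow FindNextSplineLocation, falling back to the random gravity-biased cone steps that branches use; outermost branches add instanced, hue-shifted leaves.
; RebuildTree clears and regrows it with different segment lengths.
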(event `self.ReceiveTick`
  (params (DeltaSeconds :type "Float (single-precision)")))

(event `Rebuild Tree`
  (bind _returnvalue (`self.K2_GetActorLocation`))
  (bind _returnvalue_2 (`KismetMathLibrary.MakeRandomStream` (`self.Initial Seed`)))
  (for _array_element (`self.RootArray`)
    (`SplineComponent.ClearSplinePoints` _array_element true)
    (`SplineWithMesh.AddMesh` _array_element null))
  (`InstancedStaticMeshComponent.ClearInstances` (`self.Leaves`))
  (bind _output_get (set `self.NewVar_0` (* (`KismetMathLibrary.RandomFloatInRangeFromStream` 0.75 1.5 _returnvalue_2) 2.6)))
  (`self.NewRoot` (0.0 0.0 -1.0) _returnvalue (1.0 0.0 0.0) 3 0 (`self.scale`) -1.0 true _output_get)
  (`self.NewRoot` (0.0 0.0 1.0) _returnvalue (1.0 0.0 0.0) 4 0 (`self.scale`) (`KismetMathLibrary.RandomFloatInRangeFromStream` 0.05 0.2 _returnvalue_2) false (* _output_get 1.1)))

(fn `Find Next Spline Location In Air`
  (params (Index :type Integer) (Spline :type "SplineComponent Object Reference") (Direction :type "Vector Structure") (`Current Iteration` :type Integer) (Gravity :type "Float (double-precision)") (SegmentLength :type "Float (double-precision)" :default 5.0))
  (returns (ReturnValue :type "Vector Structure"))
  (return (+ (`SplineComponent.GetLocationAtSplinePoint` (`local.Spline`) (- Index 1) "World") (* (`KismetMathLibrary.RandomUnitVectorInConeInDegreesFromStream` (`KismetMathLibrary.VLerp` Direction (`KismetMathLibrary.MakeVector` 0.0 0.0 Gravity) (`KismetMathLibrary.MultiplyMultiply_FloatFloat` (/ (`KismetMathLibrary.Conv_IntToDouble` (`local.Index`)) (`KismetMathLibrary.Conv_IntToDouble` (- (`self.NumSegments`) (* (`local.Current Iteration`) 4)))) 0.3)) 30.0 (`KismetMathLibrary.MakeRandomStream` (+ (`self.Initial Seed`) (`local.Index`)))) SegmentLength))))

(fn `FirstPointLocation`
  (params (`Current Iteration` :type Integer) (Direction :type "Vector Structure") (UpDirection :type "Vector Structure") (SegmentLength :type "Float (double-precision)"))
  (returns (ReturnValue :type "Vector Structure"))
  (return (* (`KismetMathLibrary.RotateAngleAxis` (`local.Direction`) (* (`KismetMathLibrary.Clamp` `Current Iteration` 0 1) 45.0) (`KismetMathLibrary.Cross_VectorVector` Direction UpDirection)) SegmentLength)))

(fn `Last Location and Direction`
  (params (Index :type Integer) (Spline :type "SplineComponent Object Reference"))
  (returns (Location :type "Vector Structure") (Direction :type "Vector Structure"))
  (bind _returnvalue (- Index 1))
  (return (`SplineComponent.GetLocationAtSplinePoint` Spline _returnvalue "World") (`SplineComponent.GetDirectionAtSplinePoint` Spline _returnvalue "World")))

(fn `NewRoot`
  (params (Direction :type "Vector Structure") (Location :type "Vector Structure") (UpDirection :type "Vector Structure") (Iterations :type Integer :default 0) (CurrentIteration :type Integer) (Scale :type "Float (double-precision)") (Gravity :type "Float (double-precision)" :default -1.0) (`Roots?` :type Boolean) (SegmentLength :type "Float (double-precision)"))
  (locals (LocalRoot :type "SplineWithMesh Object Reference") (Index :type Integer))
  (bind _index (`local.Index`))
  (bind _localroot (`local.LocalRoot`))
  (bind _returnvalue (`self.Find Next Spline Location In Air` (`local.Index`) (`local.LocalRoot`) (`local.Direction`) (`local.CurrentIteration`) (`local.Gravity`) (`local.SegmentLength`)))
  (bind (_location _direction) (`self.Last Location and Direction` (`local.Index`) (`local.LocalRoot`)))
  (bind _returnvalue_2 (+ (`local.CurrentIteration`) 1))
  (bind _returnvalue_3 (+ (`local.CurrentIteration`) 1))
  (bind _returnvalue_4 (* _index (`local.CurrentIteration`)))
  (bind (_returnvalue_x _returnvalue_y) (`KismetMathLibrary.BreakVector` (- (`self.K2_GetActorLocation`) _returnvalue)))
  (bind (_direction_2 _location_2 _updirection _outputpin) (`self.PrepareNextRoot` (`local.LocalRoot`) (`local.Index`) _returnvalue_3))
  (bind _returnvalue_5 (+ (* (`self.Initial Seed`) _index) _index))
  (bind _returnvalue_6 (`KismetMathLibrary.MakeRandomStream` (* _returnvalue_5 _returnvalue_4 (`KismetMathLibrary.FTrunc` (* _returnvalue_x _returnvalue_y)))))
  (`|ExecutionSequence`
    (:`then_0`
      (bind _returnvalue_7 (`AddComponent|NODE_AddSplineWithMesh-1` :`bManualAttachment` true :`RelativeTransform` (`KismetMathLibrary.MakeTransform` (- (`local.Location`) (`self.K2_GetActorLocation`)))))
      (bind _output_get (set `local.LocalRoot` _returnvalue_7))
      (`KismetArrayLibrary.Array_Add` (`self.RootArray`) _returnvalue_7)
      (set `SplineWithMesh.Scale` (`local.Scale`) _output_get)
      (`SplineComponent.ClearSplinePoints` (`local.LocalRoot`) true)
      (`SplineComponent.AddSplinePointAtIndex` _localroot (`local.Location`) 0 "World" false)
      (`SplineComponent.SetUpVectorAtSplinePoint` _localroot 0 (`local.UpDirection`) "World" false)
      (`SplineComponent.AddSplinePointAtIndex` _localroot (+ (`local.Location`) (`self.FirstPointLocation` (`local.CurrentIteration`) (`local.Direction`) (`local.UpDirection`) (`local.SegmentLength`))) 1 "World" false)
      (`SplineComponent.SetUpVectorAtSplinePoint` _localroot 1 (`local.UpDirection`) "World" true)
      (for _index_2 (range 2 (+ (`KismetMathLibrary.Clamp` (- (`self.NumSegments`) (* (`local.CurrentIteration`) 4)) 2 (`self.NumSegments`)) 1))
        (set `local.Index` _index_2)
        (if (`local.Roots?`)
          (bind (_nextlocation _nextupvector _returnvalue_8) (`STC_MathFunctions.FindNextSplineLocation` (`local.SegmentLength`) _location _direction (+ (`self.Initial Seed`) (`local.Index`))))
          (if _returnvalue_8
            (`SplineComponent.AddSplinePointAtIndex` (`local.LocalRoot`) _nextlocation (`local.Index`) "World" false)
            (`SplineComponent.SetUpVectorAtSplinePoint` (`local.LocalRoot`) (`local.Index`) _nextupvector "World" true)
            (else
              (`SplineComponent.AddSplinePointAtIndex` (`local.LocalRoot`) _returnvalue (`local.Index`) "World" false :!label _label)
              (`SplineComponent.SetUpVectorAtSplinePoint` (`local.LocalRoot`) (`local.Index`) (1.0 0.0 0.0) "World" true)
              (if (`local.Roots?`)
                _
                (elif (< 2 (`local.CurrentIteration`))
                  (`InstancedStaticMeshComponent.AddInstanceWorldSpace` (`self.Leaves`) (`KismetMathLibrary.MakeTransform` _returnvalue (`KismetMathLibrary.MakeRotator` (`KismetMathLibrary.RandomFloatInRangeFromStream` -22.0 -30.0 (`KismetMathLibrary.MakeRandomStream` _returnvalue_5)) (`KismetMathLibrary.RandomFloatInRangeFromStream` -12.0 25.0 (`KismetMathLibrary.MakeRandomStream` _returnvalue_4)) (`KismetMathLibrary.RandomFloatInRangeFromStream` -350.0 200.0 _returnvalue_6)) (`KismetMathLibrary.Conv_DoubleToVector` (* (`KismetMathLibrary.RandomFloatInRangeFromStream` 0.08 0.25 _returnvalue_6) (`local.SegmentLength`)))))))))
          (else
            (goto _label)))
        (`SplineWithMesh.AddMesh` (`local.LocalRoot`) null)))
    (:`then_1`
      (if (< _returnvalue_2 (`local.Iterations`))
        (for _index_3 (range 1 (+ (`KismetMathLibrary.Clamp` (- (* (`local.Iterations`) 2) _returnvalue_2) 1 4) 1))
          (set `local.Index` _index_3)
          (`self.NewRoot` _direction_2 _location_2 _updirection (`local.Iterations`) _returnvalue_3 _outputpin (`local.Gravity`) (`local.Roots?`) (`local.SegmentLength`)))))))

(fn `PrepareNextRoot`
  (params (Spline :type "SplineWithMesh Object Reference") (Index :type Integer) (CurrentIteration :type Integer))
  (returns (Direction :type "Vector Structure") (Location :type "Vector Structure") (UpDirection :type "Vector Structure") (OutputPin :type "Float (double-precision)"))
  (bind _initial_seed (`self.Initial Seed`))
  (bind _index (`local.Index`))
  (bind _returnvalue (* _index 2))
  (bind _returnvalue_2 (`SplineComponent.GetDirectionAtSplinePoint` (`local.Spline`) (* (`local.Index`) 2) "World"))
  (bind _returnvalue_x (`KismetMathLibrary.BreakVector` (`CurveVector.GetVectorValue` (`SplineWithMesh.ScaleCurve` (`local.Spline`)) (/ (`KismetMathLibrary.Conv_IntToDouble` (* (`local.Index`) 2)) (`KismetMathLibrary.Conv_IntToDouble` (`KismetMathLibrary.Clamp` (- (`self.NumSegments`) (* (`local.CurrentIteration`) 2)) 1 20))))))
  (return (`KismetMathLibrary.RotateAngleAxis` (`SplineComponent.GetUpVectorAtSplinePoint` (`local.Spline`) (* (`local.Index`) 2) "Local") (+ (* (+ _index (`self.Initial Seed`)) 137.5) (`KismetMathLibrary.RandomFloatInRangeFromStream` -30.0 30.0 (`KismetMathLibrary.MakeRandomStream` (+ _returnvalue (* _initial_seed _index _returnvalue _initial_seed))))) _returnvalue_2) (`SplineComponent.GetLocationAtSplinePoint` (`local.Spline`) (* (`local.Index`) 2) "World") _returnvalue_2 (* (`SplineWithMesh.Scale` (`local.Spline`)) _returnvalue_x)))

(fn `UserConstructionScript`
  (bind _returnvalue (`self.K2_GetActorLocation`))
  (bind _leaves (`self.Leaves`))
  (bind _returnvalue_2 (`KismetMathLibrary.MakeRandomStream` (`self.Initial Seed`)))
  (bind _returnvalue_3 (`KismetSystemLibrary.GetObjectName` self))
  (bind (_returnvalue_x _returnvalue_y _returnvalue_z) (`KismetMathLibrary.BreakVector` (`SceneComponent.K2_GetComponentLocation` (`self.DefaultSceneRoot`))))
  (bind _returnvalue_4 (`KismetMathLibrary.RandomFloatInRangeFromStream` 0.5 1.0 _returnvalue_2))
  (bind _output_get (set `self.Initial Seed` (`KismetStringLibrary.Conv_StringToInt` (`KismetStringLibrary.GetSubstring` _returnvalue_3 (- (`KismetStringLibrary.Len` _returnvalue_3) 1)))))
  (bind _returnvalue_5 (`KismetMathLibrary.MakeRandomStream` _output_get))
  (`self.K2_SetActorRotation` (`KismetMathLibrary.MakeRotator` 0.0 0.0 (`KismetMathLibrary.RandomFloatInRangeFromStream` -180.0 180.0 _returnvalue_5)))
  (`StaticMeshComponent.SetStaticMesh` (`self.Leaves`) (`|GetArrayItem` (`self.LeafMesh`) (`KismetMathLibrary.RandomIntegerFromStream` 2 _returnvalue_5)))
  (bind _returnvalue_6 (`PrimitiveComponent.CreateDynamicMaterialInstance` _leaves 0 "/Game/Materials/M_Pine.M_Pine" "None"))
  (`PrimitiveComponent.SetMaterial` _leaves 0 _returnvalue_6)
  (`MaterialInstanceDynamic.SetScalarParameterValue` _returnvalue_6 "HueShift" (`KismetMathLibrary.RandomFloatInRangeFromStream` 0.07 -0.5 (`KismetMathLibrary.MakeRandomStream` (+ (`self.Initial Seed`) (`KismetMathLibrary.FTrunc` (* _returnvalue_x _returnvalue_y _returnvalue_z))))))
  (bind _output_get_2 (set `self.scale` _returnvalue_4))
  (`self.NewRoot` (0.0 0.0 -1.0) _returnvalue (1.0 0.0 0.0) 3 0 _output_get_2 -1.0 true (* _returnvalue_4 2.8))
  (`self.NewRoot` (0.0 0.0 1.0) _returnvalue (1.0 0.0 0.0) 4 0 _output_get_2 (`KismetMathLibrary.RandomFloatInRangeFromStream` 0.05 0.2 _returnvalue_2) false (* _returnvalue_4 3.8)))