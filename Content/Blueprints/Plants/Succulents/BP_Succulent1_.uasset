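; Procedural succulent plant, built entirely in the construction script from a seed parsed from the actor's name suffix.
; The seed picks one of three types, setting the Leaves mesh and a tinted dynamic material, and a leaf count scaled by Age.
; Each leaf is a separate static mesh component on a Phyllotaxis spiral, with a curve driving scale, spread and height.
; Instanced-leaf and spline-tangent nodes are left unconnected.
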(fn `UserConstructionScript`
  (bind _returnvalue (`KismetMathLibrary.Conv_IntToDouble` (`self.Type`)))
  (bind _returnvalue_2 (`KismetSystemLibrary.GetObjectName` self))
  (bind (_returnvalue_roll _returnvalue_pitch _returnvalue_yaw) (`KismetMathLibrary.BreakRotator` (`KismetMathLibrary.MakeRotFromX` (`/Game/Blueprints/Libraries/BFL_ProceduralMath.Phyllotaxis` (`self.Index`) 3.0 (`self.Seed`)))))
  (bind (_returnvalue_x _returnvalue_y) (`KismetMathLibrary.BreakVector` (`CurveVector.GetVectorValue` (`self.ScaleTransformCurve`) (/ (`KismetMathLibrary.Conv_IntToDouble` (`self.Index`)) (`KismetMathLibrary.Conv_IntToDouble` (`self.NumLeaves`))))))
  (bind (_returnvalue_x_2 _returnvalue_y_2 _returnvalue_z) (`KismetMathLibrary.BreakVector` (`CurveVector.GetVectorValue` (`self.ScaleTransformCurve`) (/ (`KismetMathLibrary.Conv_IntToDouble` (`self.Index`)) (`KismetMathLibrary.Conv_IntToDouble` (`self.NumLeaves`))))))
  (bind _returnvalue_3 (+ (`KismetStringLibrary.FindSubstring` _returnvalue_2 "_" false true) 1))
  (bind _output_get (set `self.Seed` (`KismetStringLibrary.Conv_StringToInt` (`KismetStringLibrary.GetSubstring` _returnvalue_2 _returnvalue_3 (- (`KismetStringLibrary.Len` _returnvalue_2) _returnvalue_3)))))
  (bind _returnvalue_4 (`KismetMathLibrary.MakeRandomStream` _output_get))
  (bind _output_get_2 (set `self.Type` (`KismetMathLibrary.RandomIntegerInRangeFromStream` 0 2 _returnvalue_4)))
  (`StaticMeshComponent.SetStaticMesh` (`self.Leaves`) (`|GetArrayItem` (`self.MeshArray`) _output_get_2))
  (bind _returnvalue_5 (`KismetMaterialLibrary.CreateDynamicMaterialInstance` "/Game/Materials/M_Succulent.M_Succulent"))
  (`MaterialInstanceDynamic.SetScalarParameterValue` _returnvalue_5 "Desaturation" (/ _returnvalue 4.0))
  (`MaterialInstanceDynamic.SetScalarParameterValue` _returnvalue_5 "HueShift" (+ (* _returnvalue (- (mod _returnvalue 2.0) 1.0) 0.3) (`KismetMathLibrary.RandomFloatInRangeFromStream` -0.15 0.15 _returnvalue_4)))
  (`PrimitiveComponent.SetMaterial` (`self.Leaves`) 0 _returnvalue_5)
  (bind _output_get_3 (set `self.NumLeaves` (* (`KismetMathLibrary.RandomIntegerInRangeFromStream` 10 16 _returnvalue_4) (`self.Age`))))
  (for _index (range (+ _output_get_3 1))
    (set `self.Index` _index)
    (`AddComponent|NODE_AddStaticMeshComponent-0` :`RelativeTransform` (`KismetMathLibrary.MakeTransform` (+ (* (`/Game/Blueprints/Libraries/BFL_ProceduralMath.Phyllotaxis` (`self.Index`) 3.0 (`self.Seed`)) _returnvalue_y) (`KismetMathLibrary.MakeVector` 0.0 0.0 (* _returnvalue_z 2.0))) (`KismetMathLibrary.MakeRotator` 0.0 (* (/ (`KismetMathLibrary.Conv_IntToDouble` (`self.Index`)) (`KismetMathLibrary.Conv_IntToDouble` (`self.NumLeaves`))) -80.0) _returnvalue_yaw) (`KismetMathLibrary.Conv_DoubleToVector` (* _returnvalue_x_2 6.0))))))