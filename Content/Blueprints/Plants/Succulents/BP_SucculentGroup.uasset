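; BP_SucculentGroup is an actor that spawns a cluster of succulents of one randomly chosen type on BeginPlay.
; It clears any tracked succulents, spawns one untracked oldest plant, then a tracked, owned ring placed by a Phyllotaxis spiral function.
; Age falls with spiral index within a clamped range, so later plants are younger.
; An unused child-actor version remains in the Construction Script, disconnected.
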(event `self.ReceiveBeginPlay`
  (bind _output (`|GetArrayItem` (`self.Type`) (`self.TypeNum`)))
  (for _array_element (`self.SucculentArray`)
    (`self.K2_DestroyActor` _array_element))
  (set `self.TypeNum` (`KismetMathLibrary.RandomIntegerInRange` 0 2))
  (`|SpawnActorFromClass` _output (`KismetMathLibrary.MakeTransform` (0.0 0.0 0.0)) "Undefined" "OverrideRootScale" null 5 false null)
  (for _index (range 30 39)
    (bind _returnvalue (`|SpawnActorFromClass` _output (`KismetMathLibrary.MakeTransform` (`/Game/Blueprints/Libraries/BFL_ProceduralMath.Phyllotaxis` _index 30.0 0 3.0)) "Undefined" "OverrideRootScale" self (`KismetMathLibrary.Clamp` (- 5 (- _index 29)) 1 3) false null))
    (`KismetArrayLibrary.Array_Add` (`self.SucculentArray`) _returnvalue)))

(fn `UserConstructionScript`)