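; Procedural short succulent plant that builds its leaves as mesh instances and animates their growth.
; The construction script seeds from the actor name's numeric suffix, lays out an Age-scaled leaf count by phyllotaxis and a vector curve, and applies a hue-shifted material.
; Leaves start in a compressed pose; GrowSucculent runs a timeline that lerps them to stored transforms via GrowthTransform.
; Only the final update per frame dirties render state, and actor tick stops on finish.
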(event `self.ReceiveTick`
  (params (DeltaSeconds :type "Float (single-precision)")))

(event `self.ReceiveBeginPlay`)

(event `GrowSucculent`
  (params (Size :type "Float (double-precision)") (Delay :type "Float (double-precision)"))
  (bind (_direction _growth) (`Timeline|Timeline_0` :!via `PlayFromStart`)
    (:`Update`
      (for _index (range (`self.NumLeaves`))
        (bind (_location _rotation _scale) (`self.GrowthTransform` (- (- (`self.NumLeaves`) 1) _index) _growth))
        (`InstancedStaticMeshComponent.UpdateInstanceTransform` (`self.Leaves`) _index (`KismetMathLibrary.MakeTransform` _location _rotation _scale) false false false))
      (bind (_location_2 _rotation_2 _scale_2) (`self.GrowthTransform` 0 _growth))
      (`InstancedStaticMeshComponent.UpdateInstanceTransform` (`self.Leaves`) (- (`self.NumLeaves`) 1) (`KismetMathLibrary.MakeTransform` _location_2 _rotation_2 _scale_2) false true false))
    (:`Finished`
      (`self.SetActorTickEnabled` false))))

(event `AddLeaf`
  (bind _output (`|GetArrayItem` (`self.InstanceTransform`) (`self.NextLeafInstance`)))
  (bind (_returnvalue_x _returnvalue_y) (`KismetMathLibrary.BreakVector` (* (.location _output) 0.1)))
  (bind (_returnvalue_x_2 _returnvalue_y_2 _returnvalue_z) (`KismetMathLibrary.BreakVector` (* (.location _output) -1.0)))
  (bind _returnvalue (* (.y (.scale _output)) 0.6))
  (`InstancedStaticMeshComponent.AddInstance` (`self.Leaves`) (`KismetMathLibrary.MakeTransform` (`KismetMathLibrary.MakeVector` _returnvalue_x _returnvalue_y _returnvalue_z) (`KismetMathLibrary.MakeRotator` 0.0 0.0 (.yaw (.rotation _output))) (`KismetMathLibrary.MakeVector` (* (.x (.scale _output)) 0.1) _returnvalue _returnvalue)))
  (`/Engine/EditorBlueprintResources/StandardMacros.DecrementInt` (`self.NextLeafInstance`)))

(fn `GrowthTransform`
  (params (Index :type Integer) (Alpha :type "Float (double-precision)"))
  (returns (Location :type "Vector Structure") (Rotation :type "Rotator Structure") (Scale :type "Vector Structure"))
  (bind (_output_location _output_rotation _output_scale) (`KismetMathLibrary.BreakTransform` (`|GetArrayItem` (`self.InstanceTransform`) Index)))
  (bind (_returnvalue_x _returnvalue_y) (`KismetMathLibrary.BreakVector` (* _output_location 0.1)))
  (bind (_returnvalue_x_2 _returnvalue_y_2 _returnvalue_z) (`KismetMathLibrary.BreakVector` (* _output_location -1.0)))
  (bind _returnvalue (* (.y _output_scale) 0.6))
  (return (`KismetMathLibrary.VLerp` (`KismetMathLibrary.MakeVector` _returnvalue_x _returnvalue_y _returnvalue_z) _output_location (`local.Alpha`)) (`KismetMathLibrary.RLerp` (`KismetMathLibrary.MakeRotator` 0.0 0.0 (.yaw _output_rotation)) _output_rotation (`local.Alpha`)) (`KismetMathLibrary.VLerp` (`KismetMathLibrary.MakeVector` (* (.x _output_scale) 0.1) _returnvalue _returnvalue) _output_scale (`local.Alpha`))))

(fn `UserConstructionScript`
  (bind _leaves (`self.Leaves`))
  (bind _returnvalue (`KismetSystemLibrary.GetObjectName` self))
  (bind (_returnvalue_roll _returnvalue_pitch _returnvalue_yaw) (`KismetMathLibrary.BreakRotator` (`KismetMathLibrary.MakeRotFromX` (`/Game/Blueprints/Libraries/BFL_ProceduralMath.Phyllotaxis` (`self.Index`) 3.0 (`self.Seed`)))))
  (bind (_returnvalue_x _returnvalue_y) (`KismetMathLibrary.BreakVector` (`CurveVector.GetVectorValue` (`self.ScaleTransformCurve`) (/ (`KismetMathLibrary.Conv_IntToDouble` (`self.Index`)) (`KismetMathLibrary.Conv_IntToDouble` (`self.NumLeaves`))))))
  (bind (_returnvalue_x_2 _returnvalue_y_2 _returnvalue_z) (`KismetMathLibrary.BreakVector` (`CurveVector.GetVectorValue` (`self.ScaleTransformCurve`) (/ (`KismetMathLibrary.Conv_IntToDouble` (`self.Index`)) (`KismetMathLibrary.Conv_IntToDouble` (`self.NumLeaves`))))))
  (bind _returnvalue_2 (+ (`KismetStringLibrary.FindSubstring` _returnvalue "_" false true) 1))
  (bind _returnvalue_3 (`KismetMathLibrary.MakeRotator` 0.0 (* (/ (`KismetMathLibrary.Conv_IntToDouble` (`self.Index`)) (`KismetMathLibrary.Conv_IntToDouble` (`self.NumLeaves`))) -80.0) _returnvalue_yaw))
  (bind _returnvalue_4 (`KismetMathLibrary.Conv_DoubleToVector` (* _returnvalue_x_2 6.0 (`self.OriginalScale`))))
  (bind _returnvalue_5 (* (+ (* (`/Game/Blueprints/Libraries/BFL_ProceduralMath.Phyllotaxis` (`self.Index`) 3.0 (`self.Seed`)) _returnvalue_y) (`KismetMathLibrary.MakeVector` 0.0 0.0 _returnvalue_z)) (`self.OriginalScale`)))
  (bind (_returnvalue_x_3 _returnvalue_y_3) (`KismetMathLibrary.BreakVector` (* _returnvalue_5 0.1)))
  (bind (_returnvalue_x_4 _returnvalue_y_4 _returnvalue_z_2) (`KismetMathLibrary.BreakVector` (* _returnvalue_5 -1.0)))
  (bind _returnvalue_6 (* (.y _returnvalue_4) 0.6))
  (bind _output_get (set `self.Seed` (`KismetStringLibrary.Conv_StringToInt` (`KismetStringLibrary.GetSubstring` _returnvalue _returnvalue_2 (- (`KismetStringLibrary.Len` _returnvalue) _returnvalue_2)))))
  (set `self.OriginalScale` (`KismetMathLibrary.MultiplyMultiply_FloatFloat` (/ 5.0 (`KismetMathLibrary.Conv_IntToDouble` (`self.Age`))) 0.4))
  (`StaticMeshComponent.SetStaticMesh` _leaves (`self.LeafMesh`))
  (`InstancedStaticMeshComponent.ClearInstances` _leaves)
  (bind _returnvalue_7 (`KismetMaterialLibrary.CreateDynamicMaterialInstance` "/Game/Materials/M_Succulent.M_Succulent"))
  (`MaterialInstanceDynamic.SetTextureParameterValue` _returnvalue_7 "Texture" (`self.Texture`))
  (bind _returnvalue_8 (`KismetMathLibrary.MakeRandomStream` _output_get))
  (`MaterialInstanceDynamic.SetScalarParameterValue` _returnvalue_7 "HueShift" (`KismetMathLibrary.RandomFloatInRangeFromStream` -0.1 0.1 _returnvalue_8))
  (`PrimitiveComponent.SetMaterial` (`self.Leaves`) 0 _returnvalue_7)
  (bind _output_get_2 (set `self.NumLeaves` (* (`KismetMathLibrary.RandomIntegerInRangeFromStream` 10 16 _returnvalue_8) (`self.Age`))))
  (`KismetArrayLibrary.Array_Resize` (`self.InstanceTransform`) _output_get_2)
  (for _index (range _output_get_2)
    (bind _output_get_3 (set `self.Index` _index))
    (`KismetArrayLibrary.Array_Set` (`self.InstanceTransform`) _output_get_3 (`KismetMathLibrary.MakeTransform` _returnvalue_5 _returnvalue_3 _returnvalue_4))
    (bind _returnvalue_9 (`InstancedStaticMeshComponent.AddInstance` (`self.Leaves`) (`KismetMathLibrary.MakeTransform` (`KismetMathLibrary.MakeVector` _returnvalue_x_3 _returnvalue_y_3 _returnvalue_z_2) (`KismetMathLibrary.MakeRotator` 0.0 0.0 (.yaw _returnvalue_3)) (`KismetMathLibrary.MakeVector` (* (.x _returnvalue_4) 0.1) _returnvalue_6 _returnvalue_6)))))
  (set `self.NextLeafInstance` _output_get_3))