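; Older VR radial tool-selection menu that shows tool icons in a ring with a floating name label.
; ChangeToolLayout spawns a BP_MenuIcon per tool class; hovering scales icons via ResizeIcons and updates the label from class defaults.
; Tick turns the label toward the XR camera, easing its height with controller tilt.
; Legacy MeshIcons logic remains in ResizeTools and icon removal, though live icon creation fills only MenuIcons.
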(event `Resize Icons`
  (params (HoverIconIndex :type Integer))
  (bind _output (`|GetArrayItem` (`self.MenuIcons`) (`self.HoverIconCurrent`)))
  (bind _output_2 (`|GetArrayItem` (`self.MenuIcons`) HoverIconIndex))
  (if (!= HoverIconIndex (`self.HoverIconCurrent`))
    (`/Engine/EditorBlueprintResources/StandardMacros.IsValid` _output_2
      (:`Is Valid`
        (`/Game/Blueprints/RadialMenu/BP_MenuIcon.ScaleUp` _output_2))
      (:`Is Not Valid`
        _))
    (`/Engine/EditorBlueprintResources/StandardMacros.IsValid` _output
      (:`Is Valid`
        (`/Game/Blueprints/RadialMenu/BP_MenuIcon.ScaleDown` _output))
      (:`Is Not Valid`
        _))
    (bind _output_get (set `self.HoverIconCurrent` HoverIconIndex))
    (`self.DisplayText` _output_get)))

(event `self.ReceiveBeginPlay`)

(event `ScaleIconUp`
  (bind (_direction _scale) (`Timeline|Timeline_0` :!via `PlayFromStart` :!label _label)
    (:`Update`
      (`SceneComponent.SetRelativeScale3D` (`|GetArrayItem` (`self.MeshIcons`) (`self.HoverIconCurrent`)) (* (`self.OriginalScale`) _scale)))))

(event `ScaleIconDown`
  (goto _label :!via `Reverse`))

(event `/Game/Blueprints/Libraries/BPI_RadialMenu.ResizeTools`
  (params (ToolToScale :type Integer) (SubClasses :type "Array of /Game/Blueprints/Pawns/Master_Pawn Class Reference (by ref)"))
  (set `self.ToolIndex` ToolToScale)
  (for (_array_element _array_index) (`self.MeshIcons`)
    (if (== _array_index ToolToScale)
      (`SceneComponent.SetRelativeScale3D` _array_element (0.045 0.045 0.045))
      (bind _output (`|GetArrayItem` (`self.MaterialInstance`) _array_index))
      (`MaterialInstanceDynamic.SetScalarParameterValue` _output "Desaturation" 0.0)
      (`self.DisplayText` (`self.ToolIndex`))
      (else
        (`SceneComponent.SetRelativeScale3D` _array_element (0.03 0.03 0.03))
        (`MaterialInstanceDynamic.SetScalarParameterValue` _output "Desaturation" 1.0)))))

(event `/Game/Blueprints/Libraries/BPI_RadialMenu.Change NumTools`
  (params (NumTools :type Integer)))

(event `/Game/Blueprints/Libraries/BPI_RadialMenu.ChangeToolIcons`
  (params (SubClasses :type "Array of /Game/Blueprints/Pawns/Master_Pawn Class Reference (by ref)")))

(event `self.ReceiveTick`
  (params (DeltaSeconds :type "Float (single-precision)"))
  (bind _centerofcontroller (`self.CenterOfController`))
  (if (`SceneComponent.IsVisible` (`self.Title`))
    (bind _asmaster_pawn (cast `/Game/Blueprints/Pawns/Master_Pawn` (`Controller.K2_GetPawn` (`GameplayStatics.GetPlayerController` 0))))
    (`SceneComponent.K2_SetWorldLocationAndRotation` (`self.Title`) (+ (`SceneComponent.K2_GetComponentLocation` _centerofcontroller) (`KismetMathLibrary.MakeVector` 0.0 0.0 (`KismetMathLibrary.Lerp` 4.0 8.0 (- 1.0 (`KismetMathLibrary.Sqrt` (- 1.0 (`KismetMathLibrary.Square` (- (`KismetMathLibrary.Abs` (`KismetMathLibrary.Dot_VectorVector` (`SceneComponent.GetUpVector` _centerofcontroller) (0.0 0.0 1.0))) 1.0)))))))) (`KismetMathLibrary.MakeRotFromX` (- (`SceneComponent.K2_GetComponentLocation` (`/Game/Blueprints/Pawns/Master_Pawn.XR_Camera` _asmaster_pawn)) (`SceneComponent.K2_GetComponentLocation` (`self.Title`)))) false false)))

(fn `AddNewIcon`
  (params (ToolIndex :type Integer) (SubClasses :type "Array of /Game/Blueprints/Pawns/Master_Pawn Class Reference"))
  (bind _toolradius (`self.ToolRadius`))
  (bind _returnvalue (* ToolIndex (`self.AngleBetweenTools`)))
  (bind _returnvalue_2 (`/Game/Blueprints/Libraries/BFL_Menu.Convert Texture` (`.Icon` (defaults `/Game/Blueprints/RadialMenu/BP_RadialMenuOLD` (`|GetArrayItem` (`local.SubClasses`) (`local.ToolIndex`))))))
  (bind _returnvalue_3 (`AddComponent|NODE_AddSceneComponent-0` :`RelativeTransform` (`KismetMathLibrary.MakeTransform` (`KismetMathLibrary.MakeVector` (+ (* (`KismetMathLibrary.DegCos` _returnvalue) _toolradius) -2.0) (* (`KismetMathLibrary.DegSin` _returnvalue) _toolradius)) (struct :`Yaw` 90.0))))
  (bind _returnvalue_4 (`|SpawnActorFromClass` "/Game/Blueprints/RadialMenu/BP_MenuIcon.BP_MenuIcon_C" (`KismetMathLibrary.MakeTransform` (0.0 0.0 0.0)) "Undefined" "OverrideRootScale" null _returnvalue_2 null null))
  (`KismetArrayLibrary.Array_Set` (`self.MenuIcons`) ToolIndex _returnvalue_4 true)
  (set `/Game/Blueprints/RadialMenu/BP_MenuIcon.TextureIcon` _returnvalue_2 _returnvalue_4)
  (`SceneComponent.K2_AttachToComponent` (`Actor.RootComponent` _returnvalue_4) _returnvalue_3 "None" "KeepRelative" "KeepRelative" "KeepRelative" false))

(fn `ChangeToolLayout`
  (params (NumTools :type Integer) (SubClasses :type "Array of /Game/Blueprints/Pawns/Master_Pawn Class Reference") (AngleBetweenTools :type "Float (double-precision)"))
  (bind _returnvalue (`KismetArrayLibrary.Array_Length` SubClasses))
  (bind _returnvalue_2 (`KismetArrayLibrary.Array_Length` (`self.MeshIcons`)))
  (set `self.SubClasses` SubClasses)
  (set `self.AngleBetweenTools` AngleBetweenTools)
  (set `self.NumTools` _returnvalue)
  (for _index (range _returnvalue)
    (`self.AddNewIcon` _index (`local.SubClasses`)))
  (if (< _returnvalue _returnvalue_2)
    (for _index_2 (range _returnvalue (+ _returnvalue_2 1))
      (`self.RemoveOldIcon` _index_2))))

(fn `DeselectAllIcons`)

(fn `DisplayText`
  (params (CurrentTool :type Integer) (`Hide?` :type Boolean))
  (bind _title (`self.Title`))
  (bind _output (`|GetArrayItem` (`self.SubClasses`) CurrentTool))
  (if `Hide?`
    (`SceneComponent.SetVisibility` _title false false)
    (elif (`KismetSystemLibrary.IsValidClass` _output)
      (`TextRenderComponent.K2_SetText` _title (`KismetSystemLibrary.MakeLiteralText` (`KismetTextLibrary.Conv_StringToText` (`|GetEnumeratorNameAsString` (`.Icon` (defaults `/Game/Blueprints/RadialMenu/BP_RadialMenuOLD` _output))))))
      (`SceneComponent.SetVisibility` _title true false))))

(fn `NewFunction_0`)

(fn `RemoveOldIcon`
  (params (ToolIndex :type Integer))
  (bind _output (`|GetArrayItem` (`self.MeshIcons`) ToolIndex))
  (`/Engine/EditorBlueprintResources/StandardMacros.IsValid` _output
    (:`Is Valid`
      (`SceneComponent.SetVisibility` _output false false))))

(fn `UserConstructionScript`
  (bind _returnvalue (`AddComponent|NODE_AddTextRenderComponent-3` :`RelativeTransform` (`KismetMathLibrary.MakeTransform` (8.0 0.0 0.0))))
  (bind _output_get (set `self.Title` _returnvalue)))