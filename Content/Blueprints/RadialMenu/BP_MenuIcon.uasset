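; Icon actor for a radial menu that animates its mesh scale and desaturation.
; The construction script creates a dynamic material on the mesh, applies the icon texture and starts it fully desaturated.
; ScaleUp plays a timeline that scales the mesh relative to its original size and drives the Desaturation parameter, and ScaleDown reverses that timeline.
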(event `self.ReceiveBeginPlay`)

(event `ScaleUp`
  (bind (_direction _scale _desaturation) (`Timeline|Timeline_0` :!via `PlayFromStart` :!label _label)
    (:`Update`
      (`SceneComponent.SetRelativeScale3D` (`self.StaticMeshComponent`) (* (`self.OriginalScale`) _scale))
      (`MaterialInstanceDynamic.SetScalarParameterValue` (`self.DynamicMaterial`) "Desaturation" _desaturation))))

(event `ScaleDown`
  (goto _label :!via `Reverse`))

(fn `UserConstructionScript`
  (bind _staticmeshcomponent (`self.StaticMeshComponent`))
  (bind _returnvalue (`PrimitiveComponent.CreateDynamicMaterialInstance` _staticmeshcomponent 0 (`PrimitiveComponent.GetMaterial` _staticmeshcomponent 0) "None"))
  (bind _output_get (set `self.DynamicMaterial` _returnvalue))
  (`MaterialInstanceDynamic.SetTextureParameterValue` _output_get "Texture" (`self.TextureIcon`))
  (`MaterialInstanceDynamic.SetScalarParameterValue` (`self.DynamicMaterial`) "Desaturation" 1.0))