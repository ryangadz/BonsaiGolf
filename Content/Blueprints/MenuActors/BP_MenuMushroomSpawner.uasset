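; BP_MenuMushroomSpawner is a menu actor that places BP_CustomMushroom actors on surfaces aimed at with a motion controller.
; A trigger press traces a short ray forward from the controller transform against WorldStatic objects.
; On a hit, it spawns a mushroom at the impact point, upright to the surface normal and oriented along the aim, then stores it.
; Axis-driven scaling and clearing the stored reference are disconnected, so trigger axis and release do nothing.
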(event `self.TriggerActionPress`
  (params (MotionControlTrans :type "Transform Structure"))
  (bind _returnvalue (+ MotionControlTrans_Location (`KismetMathLibrary.GreaterGreater_VectorRotator` (500.0 0.0 0.0) MotionControlTrans_Rotation)))
  (bind _outhit (`KismetSystemLibrary.LineTraceSingleForObjects` MotionControlTrans_Location _returnvalue (`|MakeArray` "ObjectTypeQuery1" :!type "EObjectTypeQuery Enum")))
  (if (`GameplayStatics.BreakHitResult` _outhit)
    (bind _returnvalue_2 (`|SpawnActorFromClass` "/Game/Blueprints/MenuActors/BP_CustomMushroom.BP_CustomMushroom_C" (`KismetMathLibrary.MakeTransform` (`.ImpactPoint` (`GameplayStatics.BreakHitResult` _outhit)) (`KismetMathLibrary.MakeRotFromZX` (`.ImpactNormal` (`GameplayStatics.BreakHitResult` _outhit)) (- _returnvalue MotionControlTrans_Location))) "Undefined" "OverrideRootScale" null null))
    (set `self.MushroomActor` _returnvalue_2)))

(event `self.TriggerAxis`
  (params (MotionControlTrans :type "Transform Structure") (AxisValue :type "Float (single-precision)")))

(event `self.TriggerActionRelease`)

(fn `UserConstructionScript`
  (`parent.UserConstructionScript`))