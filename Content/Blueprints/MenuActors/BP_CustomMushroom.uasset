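; Procedural mushroom actor that bends the revolved shape from the last BP_Revolve actor found along a random stem.
; The construction script builds a four-point randomly leaning spline, plus offset and corrected splines that the live mesh path ignores.
; BeginPlay maps the template's radial coordinates onto that spline at random scale, creating a collidable procedural mesh with green material and repositioned point light.
; Older mesh, animation and collision experiments remain disconnected.
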(event `self.ReceiveBeginPlay`
  (bind _mushroomtemplate (`self.MushroomTemplate`))
  (bind _proceduralmesh (`self.ProceduralMesh`))
  (set `self.Scale` (`KismetMathLibrary.RandomFloatInRange` 0.5 1.0))
  (bind _outactors (`GameplayStatics.GetAllActorsOfClass` "/Game/Blueprints/MenuActors/Build/Revolve/BP_Revolve.BP_Revolve_C"))
  (bind _output_get (set `self.MushroomTemplate` (`|GetArrayItem` _outactors (- (`KismetArrayLibrary.Array_Length` _outactors) 1))))
  (`/Engine/EditorBlueprintResources/StandardMacros.IsValid` _output_get
    (:`Is Valid`
      (bind _vertices (`/Game/Blueprints/Libraries/BFL_MeshBuilding.RadialToCartesian` (`/Game/Blueprints/MenuActors/Build/Revolve/BP_Revolve.RadialMeshCoords` _output_get) (`self.Spline`) (`self.Scale`) (`/Game/Blueprints/MenuActors/Build/Revolve/BP_Revolve.DrawnSpline` _output_get)))
      (`ProceduralMeshComponent.CreateMeshSection_LinearColor` :`self` _proceduralmesh :`Vertices` _vertices :`Triangles` (`/Game/Blueprints/MenuActors/Build/Revolve/BP_Revolve.Triangles` _mushroomtemplate) :`Normals` (`/Game/Blueprints/MenuActors/Build/Revolve/BP_Revolve.Normals` _mushroomtemplate) :`bCreateCollision` true)
      (bind _returnvalue (`KismetMaterialLibrary.CreateDynamicMaterialInstance` "/Game/Materials/M_Mushroom.M_Mushroom"))
      (`PrimitiveComponent.SetMaterial` _proceduralmesh 0 _returnvalue)
      (`SceneComponent.K2_SetRelativeLocation` (`self.PointLight`) (`SplineComponent.GetLocationAtSplinePoint` (`self.Spline`) 2 "Local") false false)
      (`MaterialInstanceDynamic.SetVectorParameterValue` _returnvalue "Color" (struct :`R` 0.2217 :`G` 1.0 :`B` 0.117775 :`A` 1.0)))))

(event `self.ReceiveTick`
  (params (DeltaSeconds :type "Float (single-precision)")))

(fn `AdjustUpVectors`
  (for _index (range 4)
    (`SplineComponent.SetUpVectorAtSplinePoint` (`self.Spline`) _index (`KismetMathLibrary.Cross_VectorVector` (`self.GetActorUpVector`) (0.0 0.0 1.0)) "World" true)))

(fn `UserConstructionScript`
  (bind _spline (`self.Spline`))
  (bind _spline_2 (`self.Spline`))
  (bind _spline_3 (`self.Spline`))
  (bind _splineoffset (`self.splineOffset`))
  (bind _returnvalue (+ (`SplineComponent.GetLocationAtSplinePoint` _spline_3 1 "World") (* (`KismetMathLibrary.Normal` (+ (`SplineComponent.GetDirectionAtSplinePoint` _spline_3 1 "World") (0.0 0.0 1.0))) (`KismetMathLibrary.RandomFloatInRange` 8.0 12.0))))
  (bind _returnvalue_2 (`AddComponent|NODE_AddSplineComponent-0`))
  (set `self.splineOffset` _returnvalue_2)
  (bind _returnvalue_3 (`AddComponent|NODE_AddSplineComponent-1`))
  (set `self.FinalSpline` _returnvalue_3)
  (`SplineComponent.ClearSplinePoints` _spline true)
  (`SplineComponent.SetDefaultUpVector` _spline (`self.GetActorRightVector`) "World")
  (`SplineComponent.AddSplinePointAtIndex` _spline (0.0 0.0 0.0) 0 "Local" true)
  (`SplineComponent.AddSplinePointAtIndex` _spline (`KismetMathLibrary.MakeVector` 0.0 0.0 (`KismetMathLibrary.RandomFloatInRange` 8.0 12.0)) 1 "Local" true)
  (`SplineComponent.AddSplinePointAtIndex` _spline _returnvalue 2 "World" true)
  (`SplineComponent.AddSplinePointAtIndex` _spline (+ _returnvalue (* (`KismetMathLibrary.RandomUnitVectorInConeInDegrees` (0.0 0.0 1.0) 30.0) 10.0)) 3 "World" true)
  (`self.AdjustUpVectors`)
  (`SplineTwistCorrectBPLibrary.BuildOffsetSpline` _spline_2 _splineoffset 0.0 2.0)
  (`SplineTwistCorrectBPLibrary.BuildCorrectedSpline` _spline_2 _splineoffset (`self.FinalSpline`) 1.0))