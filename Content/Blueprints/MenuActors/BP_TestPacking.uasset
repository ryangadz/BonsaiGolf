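; Test actor that packs circles inside a spline shape and previews them as static mesh components; gameplay events are empty.
; The construction script builds a point grid from the spline, then calls GetNextCircle eight times with the grid, inside indices and location and radius arrays.
; Each result places a mesh scaled to the circle's diameter.
; TestRef and a debug print of the indices are leftover, never-run experiments.
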(fn `TestRef`
  (params (NewParam :type "Array of Integer (by ref)"))
  (for (_ _array_index) NewParam
    (`KismetArrayLibrary.Array_Set` NewParam _array_index)))

(fn `UserConstructionScript`
  (bind (_insideindices _gridx _verts) (`/Game/Blueprints/Libraries/BFL_MeshBuilding.MakePointGrid` (`self.Spline`) 1.0))
  (bind _output_get (set `self.NewVar_0` _insideindices))
  (bind _output_get_2 (set `self.NewVar_1` _verts))
  (for _index (range 8)
    (bind (_nextlocation _nextradius) (`/Game/Blueprints/Libraries/BPFL_ProceduralArrays.GetNextCircle` _output_get_2 _output_get (`self.NewVar_2`) (`self.NewVar_3`) (`self.Spline`) _index))
    (`AddComponent|NODE_AddStaticMeshComponent-0` :`RelativeTransform` (`KismetMathLibrary.MakeTransform` _nextlocation (struct) (`KismetMathLibrary.Conv_DoubleToVector` (* _nextradius 2.0))))))