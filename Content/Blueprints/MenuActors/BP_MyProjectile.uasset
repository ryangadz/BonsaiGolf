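; BP_MyProjectile is a projectile actor that launches a physics-simulated, hue-tinted mesh when it begins play.
; BeginPlay adds a static mesh component at runtime from the StaticMesh variable and gives it a dynamic M_Ball material driven by HueShift.
; An impulse along the actor's forward vector, scaled by Velocity, then launches that component.
; The FireProjectile event takes a mesh and hue but has no implementation.
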(event `self.ReceiveBeginPlay`
  (bind _returnvalue (`AddComponent|NODE_AddStaticMeshComponent-0` :`RelativeTransform` (`KismetMathLibrary.MakeTransform` (5.0 0.0 0.0))))
  (`StaticMeshComponent.SetStaticMesh` _returnvalue (`self.StaticMesh`))
  (`PrimitiveComponent.SetSimulatePhysics` _returnvalue true)
  (bind _returnvalue_2 (`PrimitiveComponent.CreateDynamicMaterialInstance` _returnvalue 0 "/Game/Materials/M_Ball.M_Ball" "None"))
  (`MaterialInstanceDynamic.SetScalarParameterValue` _returnvalue_2 "HueShift" (`self.HueShift`))
  (`PrimitiveComponent.SetMaterial` _returnvalue 0 _returnvalue_2)
  (`PrimitiveComponent.AddImpulse` _returnvalue (* (`self.GetActorForwardVector`) (`self.Velocity`)) "None" false))

(event `FireProjectile`
  (params (StaticMesh :type "StaticMesh Object Reference") (HueShift :type "Float (double-precision)")))

(fn `UserConstructionScript`)