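; BP_Menu_Build is a menu actor that shows a Build material on a mesh kept oriented to the player camera.
; The construction script creates a dynamic instance of M_Build, sets it to white with no desaturation, and applies it to the rotated mesh.
; Tick billboards the mesh using a camera-to-mesh look-at rotation with a pitch offset.
; Its Focus and Unfocus events are empty.
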(event `self.ReceiveTick`
  (params (DeltaSeconds :type "Float (single-precision)"))
  (bind _defaultmeshcomponent (`self.DefaultMeshComponent`))
  (bind (_returnvalue_roll _returnvalue_pitch _returnvalue_yaw) (`KismetMathLibrary.BreakRotator` (`KismetMathLibrary.FindLookAtRotation` (`SceneComponent.K2_GetComponentLocation` (`PlayerCameraManager.TransformComponent` (`GameplayStatics.GetPlayerCameraManager` 0))) (`SceneComponent.K2_GetComponentLocation` _defaultmeshcomponent))))
  (`SceneComponent.K2_SetWorldRotation` _defaultmeshcomponent (`KismetMathLibrary.MakeRotator` _returnvalue_roll (+ _returnvalue_pitch 90.0) _returnvalue_yaw) false false))

(event `self.Focus`)

(event `self.Unfocus`)

(fn `UserConstructionScript`
  (bind _returnvalue (`PrimitiveComponent.CreateDynamicMaterialInstance` (`self.DefaultMeshComponent`) 0 "/Game/Materials/MenuMaterials/M_Build.M_Build" "None"))
  (bind _output_get (set `self.DynamicMaterial` _returnvalue))
  (`MaterialInstanceDynamic.SetScalarParameterValue` _output_get "Desaturation" 0.0)
  (`PrimitiveComponent.SetMaterial` (`self.DefaultMeshComponent`) 0 _output_get)
  (`SceneComponent.K2_SetRelativeRotation` (`self.DefaultMeshComponent`) (struct :`Pitch` 90.0) false false)
  (`MaterialInstanceDynamic.SetVectorParameterValue` (`self.DynamicMaterial`) "Color" (struct :`R` 1.0 :`G` 1.0 :`B` 1.0 :`A` 1.0)))