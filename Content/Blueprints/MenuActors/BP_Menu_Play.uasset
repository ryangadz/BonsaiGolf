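; BP_Menu_Play is a menu actor that fires a projectile when the motion controller trigger is pressed.
; TriggerActionPress spawns BP_MyProjectile at the motion controller transform, passing the actor's default mesh, a fixed velocity and its color hue shift.
; The construction script runs the parent's logic, then applies the M_Ball material to the default mesh, while Tick only forwards to the parent.
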(event `self.ReceiveTick`
  (params (DeltaSeconds :type "Float (single-precision)"))
  (`parent.ReceiveTick` DeltaSeconds))

(event `self.TriggerActionPress`
  (params (MotionControlTrans :type "Transform Structure"))
  (`|SpawnActorFromClass` "/Game/Blueprints/MenuActors/BP_MyProjectile.BP_MyProjectile_C" MotionControlTrans "Undefined" "OverrideRootScale" null (`StaticMeshComponent.StaticMesh` (`self.DefaultMeshComponent`)) 6.0 (`self.ColorHueShift`) null))

(fn `UserConstructionScript`
  (`parent.UserConstructionScript`)
  (`PrimitiveComponent.SetMaterial` (`self.DefaultMeshComponent`) 0 "/Game/Materials/M_Ball.M_Ball"))