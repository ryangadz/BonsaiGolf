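; BP_Menu_Erase is a menu actor that acts as a toggleable erase tool for motion-controller laser interaction.
; Select toggles the tool, turning its dynamic material and the pawn's laser red when active, while Unfocus resets both.
; While selected, a trigger press line-traces forward from the controller and destroys the hit WorldDynamic actor.
; Tick orients the mesh along the player camera's line of sight with a pitch offset.
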(event `self.ReceiveTick`
  (params (DeltaSeconds :type "Float (single-precision)"))
  (bind _defaultmeshcomponent (`self.DefaultMeshComponent`))
  (bind (_returnvalue_roll _returnvalue_pitch _returnvalue_yaw) (`KismetMathLibrary.BreakRotator` (`KismetMathLibrary.FindLookAtRotation` (`SceneComponent.K2_GetComponentLocation` (`PlayerCameraManager.TransformComponent` (`GameplayStatics.GetPlayerCameraManager` 0))) (`SceneComponent.K2_GetComponentLocation` _defaultmeshcomponent))))
  (`SceneComponent.K2_SetWorldRotation` _defaultmeshcomponent (`KismetMathLibrary.MakeRotator` _returnvalue_roll (+ _returnvalue_pitch 90.0) _returnvalue_yaw) false false))

(event `self.Select`
  (bind _returnvalue (`GameplayStatics.GetPlayerPawn` 0))
  (bind _dynamicmaterial (`self.DynamicMaterial`))
  (if (`self.ToolSelected?`)
    (set `self.ToolSelected?` false)
    (message `/Game/Blueprints/BPI_MasterPawn.ChangeLaserColor` _returnvalue (struct :`R` 10.0 :`G` 10.0 :`B` 10.0 :`A` 1.0))
    (`MaterialInstanceDynamic.SetVectorParameterValue` _dynamicmaterial "Color" (struct :`R` 1.0 :`G` 1.0 :`B` 1.0 :`A` 1.0))
    (else
      (set `self.ToolSelected?` true)
      (message `/Game/Blueprints/BPI_MasterPawn.ChangeLaserColor` _returnvalue (struct :`R` 20.0 :`A` 1.0))
      (`MaterialInstanceDynamic.SetVectorParameterValue` _dynamicmaterial "Color" (struct :`R` 1.0 :`A` 1.0)))))

(event `self.TriggerActionPress`
  (params (MotionControlTrans :type "Transform Structure"))
  (bind _returnvalue (`KismetMathLibrary.GetForwardVector` MotionControlTrans_Rotation))
  (if (`self.ToolSelected?`)
    (bind (_outhit _returnvalue_2) (`KismetSystemLibrary.LineTraceSingleForObjects` (+ MotionControlTrans_Location (* _returnvalue 15.0)) (+ MotionControlTrans_Location (* _returnvalue 500.0)) (`|MakeArray` "ObjectTypeQuery2" :!type "EObjectTypeQuery Enum")))
    (if _returnvalue_2
      (`self.K2_DestroyActor` (`.HitActor` (`GameplayStatics.BreakHitResult` _outhit))))))

(event `self.Focus`)

(event `self.Unfocus`
  (set `self.ToolSelected?` false)
  (message `/Game/Blueprints/BPI_MasterPawn.ChangeLaserColor` (`GameplayStatics.GetPlayerPawn` 0) (struct :`R` 10.0 :`G` 10.0 :`B` 10.0 :`A` 1.0))
  (`MaterialInstanceDynamic.SetVectorParameterValue` (`self.DynamicMaterial`) "Color" (struct :`R` 1.0 :`G` 1.0 :`B` 1.0 :`A` 1.0)))

(fn `UserConstructionScript`
  (bind _defaultmeshcomponent (`self.DefaultMeshComponent`))
  (`parent.UserConstructionScript`)
  (bind _returnvalue (`PrimitiveComponent.CreateDynamicMaterialInstance` _defaultmeshcomponent 0 "/Game/Materials/MenuMaterials/M_Clear.M_Clear" "None"))
  (bind _output_get (set `self.DynamicMaterial` _returnvalue))
  (`MaterialInstanceDynamic.SetScalarParameterValue` _output_get "Desaturation" 0.0)
  (`PrimitiveComponent.SetMaterial` _defaultmeshcomponent 0 _output_get)
  (`SceneComponent.K2_SetRelativeRotation` (`self.DefaultMeshComponent`) (struct :`Pitch` 90.0) false false)
  (`MaterialInstanceDynamic.SetVectorParameterValue` (`self.DynamicMaterial`) "Color" (struct :`R` 1.0 :`G` 1.0 :`B` 1.0 :`A` 1.0)))