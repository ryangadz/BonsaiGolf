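; BP_Menu_Lighting is a motion-controller menu actor that places lighting actors in the world.
; Focus and Unfocus show and hide its particle system, and the construction script sets the actor to half scale.
; On trigger press, it line-traces 500 units along the controller's forward vector against static and dynamic world objects.
; It then spawns BP_Lighting_Actor at the impact point without checking whether the trace hit.
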(event `self.Focus`
  (`SceneComponent.SetVisibility` (`self.ParticleSystem`) true false))

(event `self.Unfocus`
  (`SceneComponent.SetVisibility` (`self.ParticleSystem`) false false))

(event `self.TriggerActionPress`
  (params (MotionControlTrans :type "Transform Structure"))
  (bind _outhit (`KismetSystemLibrary.LineTraceSingleForObjects` MotionControlTrans_Location (+ MotionControlTrans_Location (* (`KismetMathLibrary.GetForwardVector` MotionControlTrans_Rotation) 500.0)) (`|MakeArray` "ObjectTypeQuery1" "ObjectTypeQuery2" :!type "EObjectTypeQuery Enum")))
  (`|SpawnActorFromClass` "/Game/Blueprints/MenuActors/Lighting/BP_Lighting_Actor.BP_Lighting_Actor_C" (`KismetMathLibrary.MakeTransform` (`.ImpactPoint` (`GameplayStatics.BreakHitResult` _outhit))) "Undefined" "OverrideRootScale" null null))

(fn `UserConstructionScript`
  (`parent.UserConstructionScript`)
  (`self.SetActorScale3D` (0.5 0.5 0.5)))