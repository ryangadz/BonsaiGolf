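; Motion-controller drawing actor that turns a hand-drawn outline into a mounded ground patch with scattered child actors, apparently a forest test.
; Trigger press starts a spline outline, trigger axis extends it, and release or loop closure detaches the actor and builds a pebble-textured procedural mesh.
; A curve sampled by vertex red raises the mound in proportion to spline size.
; GetNextCircle then places five child actors, scaled by circle radius.
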(event `/RadialMenu/BPI_MenuItems.TriggerActionPress`
  (params (MotionControlTrans :type "Transform Structure"))
  (set `self.ControllerTrans` MotionControlTrans)
  (`/Engine/EditorBlueprintResources/StandardMacros.DoOnce` false
    (:`Completed`
      (bind _returnvalue (`AddComponent|NODE_AddSplineComponent-0` :`bManualAttachment` true))
      (bind _output_get (set `self.Spline` _returnvalue))
      (`/Game/Blueprints/Libraries/BPFL_OutlineDraw.BeginOutline` _output_get (`self.LocationType`) (`self.ControllerTrans`) (`self.LockedSplinePoints`) (`self.LastSplineLocation`)))))

(event `/RadialMenu/BPI_MenuItems.TriggerActionRelease`
  ;[1 1 1] TODO - add in more points to complete outline
  (`self.FinishAndDetach`))

(event `/RadialMenu/BPI_MenuItems.TriggerAxis`
  (params (MotionControlTrans :type "Transform Structure") (AxisValue :type "Float (single-precision)"))
  (if (>= (`self.LockedSplinePoints`) 2)
    (bind _finished_ (`/Game/Blueprints/Libraries/BPFL_OutlineDraw.ContinueOutline` (`self.Spline`) MotionControlTrans (`self.LocationType`) (`self.LockedSplinePoints`) (`self.LastSplineLocation`) true))
    (if _finished_
      (`self.FinishAndDetach`))))

(event `FinishAndDetach`
  (bind _newvar_0 (`self.NewVar_0`))
  (bind _spline (`self.Spline`))
  (bind _spline_2 (`self.Spline`))
  (`/Engine/EditorBlueprintResources/StandardMacros.DoOnce` false
    (:`Completed`
      (`self.K2_DetachFromActor` "KeepRelative")
      (bind _returnvalue (`AddComponent|NODE_AddProceduralMeshComponent-2` :`bManualAttachment` true))
      (bind (_verts _triangles _uvs _vertexcolor _insideindices) (`/Game/Blueprints/Libraries/BFL_MeshBuilding.BuildMeshFromOutline` _spline_2 2.0))
      (for _index (range (`KismetArrayLibrary.Array_Length` _verts))
        (bind (_output_x _output_y _output_z) (`KismetMathLibrary.BreakVector` (`|GetArrayItem` _verts _index)))
        (bind _output_r (break `LinearColor` (`|GetArrayItem` _vertexcolor _index)))
        (`KismetArrayLibrary.Array_Set` _newvar_0 _index (`KismetMathLibrary.MakeVector` _output_x _output_y (+ _output_z (* (`CurveFloat.GetFloatValue` (`self.MoundCurvature`) _output_r) (`.SphereRadius` (`KismetSystemLibrary.GetComponentBounds` _spline_2)) 0.5))) true))
      (`ProceduralMeshComponent.CreateMeshSection_LinearColor` :`self` _returnvalue :`Vertices` _newvar_0 :`Triangles` _triangles :`UV0` _uvs :`VertexColors` _vertexcolor)
      (`PrimitiveComponent.SetMaterial` _returnvalue 0 "/Game/Materials/M_PebblesUV.M_PebblesUV")
      (for _index_2 (range 5)
        (bind (_nextlocation _nextradius) (`/Game/Blueprints/Libraries/BPFL_ProceduralArrays.GetNextCircle` _verts _insideindices (`self.Locations`) (`self.Radii`) _spline _index_2))
        (`AddComponent|NODE_AddChildActorComponent-1` :`RelativeTransform` (`KismetMathLibrary.MakeTransform` _nextlocation (`KismetMathLibrary.MakeRotator` 0.0) (`KismetMathLibrary.Conv_DoubleToVector` (* (/ _nextradius (`.SphereRadius` (`KismetSystemLibrary.GetComponentBounds` _spline))) 6.0))))))))

(fn `FlattenVector`
  (params (In :type "Vector Structure"))
  (returns (Out :type "Vector Structure"))
  (return (`KismetMathLibrary.MakeVector` (.x In) (.y In) (`self.Zvalue`))))

(fn `Last 2 Points`
  (returns (Distance :type "Float (double-precision)"))
  (bind _spline (`self.Spline`))
  (bind _numsplinepoints (`self.NumSplinePoints`))
  (return (- (`SplineComponent.GetDistanceAlongSplineAtSplinePoint` _spline (- _numsplinepoints 1)) (`SplineComponent.GetDistanceAlongSplineAtSplinePoint` _spline (- _numsplinepoints 2)))))

(fn `PointFromMotionController`
  (params (Type :type "/Game/Blueprints/Enum_MotionControllerData Enum" :default "NewEnumerator0"))
  (returns (ReturnValue :type "Vector Structure") (ValidLocation :type Boolean))
  (locals (Location :type "Vector Structure" :default (0.0 0.0 0.0)) (`Valid?` :type Boolean :default false))
  (bind _motioncontroller (`self.MotionController`))
  (bind _returnvalue (`SceneComponent.K2_GetComponentLocation` _motioncontroller))
  (bind _returnvalue_2 (`SceneComponent.GetForwardVector` _motioncontroller))
  (switch `/Game/Blueprints/Enum_MotionControllerData` Type
    (:`NewEnumerator0`
      (set `local.Location` (`SceneComponent.K2_GetComponentLocation` (`self.MotionController`)))
      (set `local.Valid?` true))
    (:`NewEnumerator1`
      (set `local.Location` (+ _returnvalue (* _returnvalue_2 30.0)))
      (set `local.Valid?` true))
    (:`NewEnumerator2`
      (bind _outhit (`KismetSystemLibrary.LineTraceSingleForObjects` :`Start` _returnvalue :`End` (+ _returnvalue (* _returnvalue_2 500.0)) :`ObjectTypes` (`|MakeArray` "ObjectTypeQuery1" :!type "EObjectTypeQuery Enum") :`DrawDebugType` "ForOneFrame" :`DrawTime` 1.0))
      (bind _output_get (set `local.Valid?` (`GameplayStatics.BreakHitResult` _outhit)))
      (if _output_get
        (set `local.Location` (+ (`.Location` (`GameplayStatics.BreakHitResult` _outhit)) (0.0 0.0 1.5))))))
  (return (`local.Location`) (`local.Valid?`)))

(fn `UserConstructionScript`)