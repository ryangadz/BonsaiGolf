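; BP_ForestTest is an XR controller laser pointer test actor that shows where the controller points.
; BeginPlay adds a scaled static mesh as BallLocator.
; Each Tick traces forward from XRControl against WorldStatic, stretches Laser to the hit distance and places BallLocator there, or uses full length and hides it.
; RelativeRoll feeds the laser's roll but returns zero; its camera-facing roll math is left unconnected.
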(event `self.ReceiveBeginPlay`
  (`parent.ReceiveBeginPlay`)
  (bind _returnvalue (`AddComponent|NODE_AddStaticMeshComponent-0` :`bManualAttachment` true :`RelativeTransform` (`KismetMathLibrary.MakeTransform` (0.0 0.0 0.0) (struct) (2.0 2.0 2.0))))
  (set `self.BallLocator` _returnvalue))

(event `self.ReceiveTick`
  (params (DeltaSeconds :type "Float (single-precision)"))
  (bind _laser (`self.Laser`))
  (bind _xr_control (`self.XR_Control`))
  (bind _balllocator (`self.BallLocator`))
  (bind _returnvalue (`SceneComponent.K2_GetComponentLocation` _xr_control))
  (`parent.ReceiveTick` DeltaSeconds)
  (bind _outhit (`KismetSystemLibrary.LineTraceSingleForObjects` _returnvalue (+ _returnvalue (* (`SceneComponent.GetForwardVector` _xr_control) 500.0)) (`|MakeArray` "ObjectTypeQuery1" :!type "EObjectTypeQuery Enum")))
  (`SceneComponent.K2_SetRelativeRotation` (`self.Laser`) (`KismetMathLibrary.MakeRotator` (`self.RelativeRoll`)) false false)
  (if (`GameplayStatics.BreakHitResult` _outhit)
    (bind _output_get (set `self.DistanceToController` (`.Distance` (`GameplayStatics.BreakHitResult` _outhit))))
    (`SceneComponent.SetWorldScale3D` _laser (`KismetMathLibrary.MakeVector` _output_get 0.5 0.5))
    (`SceneComponent.SetVisibility` _balllocator true false)
    (`SceneComponent.K2_SetWorldLocation` _balllocator (`.Location` (`GameplayStatics.BreakHitResult` _outhit)) false false)
    (else
      (`SceneComponent.SetWorldScale3D` _laser (500.0 0.5 0.5))
      (`SceneComponent.SetVisibility` _balllocator false false))))

(fn `RelativeRoll`
  (returns (Out :type "Float (double-precision)"))
  (return 0.0))

(fn `UserConstructionScript`
  (`parent.UserConstructionScript`))