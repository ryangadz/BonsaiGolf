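; BP_MenuTerrainEdit is a menu actor that sculpts BP_Terrain with a motion controller.
; Trigger press line-traces from the controller and enables editing on a terrain hit, until release.
; While editing, the trigger axis re-traces and calls Sculpt with impact point, normal, axis value as pressure and a profile curve.
; Its mesh is tinted green at construction, and Tick keeps it upright and sets a material Animate parameter from focus.
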(event `/RadialMenu/BPI_MenuItems.TriggerActionPress`
  (params (MotionControlTrans :type "Transform Structure"))
  (bind _location (.location MotionControlTrans))
  (bind _outhit (`KismetSystemLibrary.LineTraceSingleForObjects` _location (+ _location (* (`KismetMathLibrary.GetForwardVector` (.rotation MotionControlTrans)) 500.0)) (`|MakeArray` "ObjectTypeQuery1" :!type "EObjectTypeQuery Enum")))
  (bind _asbp_terrain (cast `/Game/Blueprints/MenuActors/BP_Terrain` (`.HitActor` (`GameplayStatics.BreakHitResult` _outhit)))
    (:`then`
      (set `self.TerrainActor` _asbp_terrain)
      (set `self.Editing?` true))
    (:`CastFailed`
      (set `self.TerrainActor` null)
      (set `self.Editing?` false))))

(event `/RadialMenu/BPI_MenuItems.TriggerActionRelease`
  (set `self.Editing?` false))

(event `/RadialMenu/BPI_MenuItems.TriggerAxis`
  (params (MotionControlTrans :type "Transform Structure") (AxisValue :type "Float (single-precision)"))
  (bind _location (.location MotionControlTrans))
  (if (`self.Editing?`)
    (bind _outhit (`KismetSystemLibrary.LineTraceSingleForObjects` :`Start` _location :`End` (+ _location (* (`KismetMathLibrary.GetForwardVector` (.rotation MotionControlTrans)) 500.0)) :`ObjectTypes` (`|MakeArray` "ObjectTypeQuery1" :!type "EObjectTypeQuery Enum") :`DrawDebugType` "ForOneFrame"))
    (bind _asbp_terrain (cast `/Game/Blueprints/MenuActors/BP_Terrain` (`.HitActor` (`GameplayStatics.BreakHitResult` _outhit)))
      (:`then`
        (bind _output_get (set `self.TerrainActor` _asbp_terrain))
        (`/Game/Blueprints/MenuActors/BP_Terrain.Sculpt` _output_get (`.ImpactPoint` (`GameplayStatics.BreakHitResult` _outhit)) (`.ImpactNormal` (`GameplayStatics.BreakHitResult` _outhit)) AxisValue (`self.ProfileCurve`)))
      (:`CastFailed`
        (set `self.TerrainActor` null)))))

(event `self.ReceiveTick`
  (params (DeltaSeconds :type "Float (single-precision)"))
  (bind (_returnvalue_roll _returnvalue_pitch _returnvalue_yaw) (`KismetMathLibrary.BreakRotator` (`self.K2_GetActorRotation`)))
  (bind _dynamicmaterial (`self.DynamicMaterial`))
  (`SceneComponent.K2_SetWorldRotation` (`self.DefaultMeshComponent`) (`KismetMathLibrary.MakeRotator` 0.0 0.0 _returnvalue_yaw) false false)
  (if (`self.InFocus?`)
    (`MaterialInstanceDynamic.SetScalarParameterValue` _dynamicmaterial "Animate" 1.0)
    (else
      (`MaterialInstanceDynamic.SetScalarParameterValue` _dynamicmaterial "Animate" 0.0))))

(fn `UserConstructionScript`
  (bind _defaultmeshcomponent (`self.DefaultMeshComponent`))
  (`parent.UserConstructionScript`)
  (bind _returnvalue (`KismetMaterialLibrary.CreateDynamicMaterialInstance` (`PrimitiveComponent.GetMaterial` _defaultmeshcomponent 0)))
  (bind _output_get (set `self.Material` _returnvalue))
  (`PrimitiveComponent.SetMaterial` _defaultmeshcomponent 0 _output_get)
  (`MaterialInstanceDynamic.SetVectorParameterValue` _output_get "Color" (struct :`R` 0.001685 :`G` 1.0 :`A` 1.0)))