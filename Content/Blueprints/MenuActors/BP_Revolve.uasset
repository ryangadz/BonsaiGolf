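; Motion-controller lathe tool that lets the player draw a profile once and revolve it into a procedural mushroom-material mesh.
; Trigger press starts an axis-snapped outline spline, axis input extends it, and release closes it on the Z axis.
; RevolveSpline then builds the collidable mesh, detaches the actor and hides the guides.
; Construction script sizes the plane and cylinder guides and optionally builds a mesh; older revolve and spline-bending code sits disconnected.
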(event `RevolveSpline`
  (`/Game/Blueprints/Libraries/BFL_MeshBuilding.RevolveCurveAboutAxis` null 6 24 (`self.Vertices`) (`self.Triangles`) (0.0 0.0 1.0) (`self.RadialMeshCoords`) (`self.Normals`))
  (bind _returnvalue (`AddComponent|NODE_AddProceduralMeshComponent-4` :`bManualAttachment` true))
  (bind _output_get (set `self.Mesh` _returnvalue))
  (`SceneComponent.K2_AttachToComponent` _output_get (`self.DefaultSceneRoot`) "None" "KeepRelative" "KeepRelative" "KeepRelative" true)
  (`ProceduralMeshComponent.CreateMeshSection_LinearColor` :`self` _output_get :`Vertices` (`self.Vertices`) :`Triangles` (`self.Triangles`) :`Normals` (`self.Normals`) :`bCreateCollision` true)
  (`PrimitiveComponent.SetMaterial` _output_get 0 "/Game/Materials/M_Mushroom.M_Mushroom")
  (`self.K2_DetachFromActor` "KeepWorld" "KeepWorld" "KeepWorld")
  (`SceneComponent.SetVisibility` (`self.Plane`) false false)
  (`SceneComponent.SetVisibility` (`self.Cylinder`) false false)
  (`SceneComponent.SetVisibility` (`self.RevolveArrow`) false false))

(event `/RadialMenu/BPI_MenuItems.TriggerActionPress`
  (params (MotionControlTrans :type "Transform Structure"))
  (`/Engine/EditorBlueprintResources/StandardMacros.DoOnce` false
    (:`Completed`
      (bind _returnvalue (`AddComponent|NODE_AddSplineWithMesh-0` :`bManualAttachment` true))
      (`SceneComponent.K2_AttachToComponent` _returnvalue (`self.DefaultSceneRoot`) "None" "KeepRelative" "KeepRelative" "KeepRelative" true)
      (bind _output_get (set `self.DrawnSpline` _returnvalue))
      (`/Game/Blueprints/Libraries/BPFL_OutlineDraw.BeginOutline` _output_get (`self.LocationType`) MotionControlTrans (`self.LockedSplinePoints`) (`self.LastSplineLocation`) true))))

(event `/RadialMenu/BPI_MenuItems.TriggerAxis`
  (params (MotionControlTrans :type "Transform Structure") (AxisValue :type "Float (single-precision)"))
  (bind _drawnspline (`self.DrawnSpline`))
  (if (>= (`self.LockedSplinePoints`) 2)
    (`/Game/Blueprints/Libraries/BPFL_OutlineDraw.ContinueOutline` _drawnspline MotionControlTrans (`self.LocationType`) (`self.LockedSplinePoints`) (`self.LastSplineLocation`) false false 5.0)
    (`SplineWithMesh.AddMesh` _drawnspline self)))

(event `/RadialMenu/BPI_MenuItems.TriggerActionRelease`
  (bind _drawnspline (`self.DrawnSpline`))
  (bind (_returnvalue_x _returnvalue_y _returnvalue_z) (`KismetMathLibrary.BreakVector` (`SplineComponent.GetLocationAtSplinePoint` _drawnspline (- (`SplineComponent.GetNumberOfSplinePoints` _drawnspline) 1) "Local")))
  (`/Engine/EditorBlueprintResources/StandardMacros.IsValid` (`self.DrawnSpline`)
    (:`Is Valid`
      (`SplineComponent.AddSplinePoint` _drawnspline (`KismetMathLibrary.MakeVector` 0.0 0.0 _returnvalue_z) "Local" true)
      (`SplineWithMesh.AddMesh` _drawnspline self)
      (`self.RevolveSpline`)
      (set `self.LockedSplinePoints` 0))))

(fn `UserConstructionScript`
  (bind _cylinder (`self.Cylinder`))
  (bind _plane (`self.Plane`))
  (`SceneComponent.K2_SetRelativeLocation` _cylinder (`KismetMathLibrary.MakeVector` 0.0 0.0 (/ (`self.Height`) 2.0)) false false)
  (`SceneComponent.SetRelativeScale3D` _cylinder (`KismetMathLibrary.MakeVector` 0.333333 0.333333 (/ (`self.Height`) 3.0)))
  (`SceneComponent.SetRelativeScale3D` (`self.Plane`) (`KismetMathLibrary.MakeVector` (`self.Height`) (`self.Width`)))
  (bind _returnvalue (`PrimitiveComponent.CreateDynamicMaterialInstance` _plane 0 "/Game/Materials/M_RevolvePlane.M_RevolvePlane" "None"))
  (`MaterialInstanceDynamic.SetScalarParameterValue` _returnvalue "Height" (`self.Width`))
  (`MaterialInstanceDynamic.SetScalarParameterValue` _returnvalue "Width" (`self.Height`))
  (`PrimitiveComponent.SetMaterial` _plane 0 _returnvalue)
  (`MaterialInstanceDynamic.SetScalarParameterValue` _returnvalue "GridThickness" 0.1)
  (if (`self.ConstructionMushroom`)
    (`/Game/Blueprints/Libraries/BFL_MeshBuilding.RevolveCurveAboutAxis` null 6 12 (`self.Vertices`) (`self.Triangles`) (0.0 0.0 1.0) (`self.RadialMeshCoords`) (`self.Normals`))
    (bind _returnvalue_2 (`AddComponent|NODE_AddProceduralMeshComponent-0`))
    (`ProceduralMeshComponent.CreateMeshSection_LinearColor` :`self` _returnvalue_2 :`Vertices` (`self.Vertices`) :`Triangles` (`self.Triangles`) :`Normals` (`self.Normals`))
    (`PrimitiveComponent.SetMaterial` _returnvalue_2 0 "/Game/Materials/M_Mushroom.M_Mushroom")))