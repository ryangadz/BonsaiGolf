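; BP_Terrain is a terrain patch the player outlines with a motion controller and can then sculpt.
; Trigger press starts a spline, and trigger axis input extends it with automatic loop closing.
; Closing the loop or releasing the trigger builds a pebble-textured procedural mesh with collision from the outline.
; Sculpt offsets nearby interior vertices along Z using a falloff curve scaled by pressure, then updates the mesh section.
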(event `/RadialMenu/BPI_MenuItems.TriggerActionPress`
  (params (MotionControlTrans :type "Transform Structure"))
  (set `self.ControllerTrans` MotionControlTrans)
  (`/Engine/EditorBlueprintResources/StandardMacros.DoOnce` false
    (:`Completed`
      (bind _returnvalue (`AddComponent|NODE_AddSplineComponent-0` :`bManualAttachment` true))
      (bind _output_get (set `self.Spline` _returnvalue))
      (`/Game/Blueprints/Libraries/BPFL_OutlineDraw.BeginOutline` _output_get (`self.LocationType`) (`self.ControllerTrans`) (`self.LockedSplinePoints`) (`self.LastSplineLocation`)))))

(event `/RadialMenu/BPI_MenuItems.TriggerActionRelease`
  ;[1 1 1] TODO - add in more points to complete outline
  (`self.FinishAndDetach`))

(event `/RadialMenu/BPI_MenuItems.TriggerAxis`
  (params (MotionControlTrans :type "Transform Structure") (AxisValue :type "Float (single-precision)"))
  (if (>= (`self.LockedSplinePoints`) 2)
    (bind _finished_ (`/Game/Blueprints/Libraries/BPFL_OutlineDraw.ContinueOutline` (`self.Spline`) MotionControlTrans (`self.LocationType`) (`self.LockedSplinePoints`) (`self.LastSplineLocation`) true))
    (if _finished_
      (`self.FinishAndDetach`))))

(event `FinishAndDetach`
  (`/Engine/EditorBlueprintResources/StandardMacros.DoOnce` false
    (:`Completed`
      (bind (_verts _triangles _uvs _vertexcolor _insideindices) (`/Game/Blueprints/Libraries/BFL_MeshBuilding.BuildMeshFromOutline` (`self.Spline`) 2.0))
      (bind _output_get (set `self.Vertices` _verts))
      (set `self.Insides indices` _insideindices)
      (`ProceduralMeshComponent.CreateMeshSection_LinearColor` :`self` (`self.ProceduralMesh`) :`Vertices` _output_get :`Triangles` _triangles :`UV0` _uvs :`VertexColors` _vertexcolor :`bCreateCollision` true)
      (`PrimitiveComponent.SetMaterial` (`self.ProceduralMesh`) 0 "/Game/Materials/M_PebblesUV.M_PebblesUV"))))

(event `Sculpt`
  (params (Location :type "Vector Structure") (Normal :type "Vector Structure") (Pressure :type "Float (double-precision)") (ProfileCurve :type "CurveFloat Object Reference"))
  (bind _vertices (`self.Vertices`))
  (set `self.EditProfileCurve` ProfileCurve)
  (set `self.LocalEditPoint` Location)
  (for (_array_element _array_index) (`self.Insides indices`)
    (if (>= _array_element 0)
      (bind _output_get (set `self.DistanceToEdit` (`KismetMathLibrary.Vector_Distance` (`|GetArrayItem` (`self.Vertices`) _array_index) (`self.LocalEditPoint`))))
      (if (<= _output_get 10.0)
        (`KismetArrayLibrary.Array_Set` _vertices _array_index (+ (`|GetArrayItem` _vertices _array_index) (* (0.0 0.0 1.0) (* (`CurveFloat.GetFloatValue` (`self.EditProfileCurve`) (/ _output_get 10.0)) (`self.EditMultiplier`) Pressure)))))))
  (`ProceduralMeshComponent.UpdateMeshSection_LinearColor` :`self` (`self.ProceduralMesh`) :`Vertices` (`self.Vertices`)))

(fn `FlattenVector`
  (params (In :type "Vector Structure"))
  (returns (Out :type "Vector Structure"))
  (return (`KismetMathLibrary.MakeVector` (.x In) (.y In) (`self.Zvalue`))))

(fn `Last 2 Points`
  (returns (Distance :type "Float (double-precision)"))
  (bind _spline (`self.Spline`))
  (bind _numsplinepoints (`self.NumSplinePoints`))
  (return (- (`SplineComponent.GetDistanceAlongSplineAtSplinePoint` _spline (- _numsplinepoints 1)) (`SplineComponent.GetDistanceAlongSplineAtSplinePoint` _spline (- _numsplinepoints 2)))))

(fn `PointFromMotionController`
  (params (Type :type "/Game/Blueprints/Enum_MotionControllerData Enum" :default "NewEnumerator0"))
  (returns (ReturnValue :type "Vector Structure") (ValidLocation :type Boolean))
  (locals (Location :type "Vector Structure" :default (0.0 0.0 0.0)) (`Valid?` :type Boolean :default false))
  (bind _motioncontroller (`self.MotionController`))
  (bind _returnvalue (`SceneComponent.K2_GetComponentLocation` _motioncontroller))
  (bind _returnvalue_2 (`SceneComponent.GetForwardVector` _motioncontroller))
  (switch `/Game/Blueprints/Enum_MotionControllerData` Type
    (:`NewEnumerator0`
      (set `local.Location` (`SceneComponent.K2_GetComponentLocation` (`self.MotionController`)))
      (set `local.Valid?` true))
    (:`NewEnumerator1`
      (set `local.Location` (+ _returnvalue (* _returnvalue_2 30.0)))
      (set `local.Valid?` true))
    (:`NewEnumerator2`
      (bind _outhit (`KismetSystemLibrary.LineTraceSingleForObjects` :`Start` _returnvalue :`End` (+ _returnvalue (* _returnvalue_2 500.0)) :`ObjectTypes` (`|MakeArray` "ObjectTypeQuery1" :!type "EObjectTypeQuery Enum") :`DrawDebugType` "ForOneFrame" :`DrawTime` 1.0))
      (bind _output_get (set `local.Valid?` (`GameplayStatics.BreakHitResult` _outhit)))
      (if _output_get
        (set `local.Location` (+ (`.Location` (`GameplayStatics.BreakHitResult` _outhit)) (0.0 0.0 1.5))))))
  (return (`local.Location`) (`local.Valid?`)))

(fn `UserConstructionScript`)