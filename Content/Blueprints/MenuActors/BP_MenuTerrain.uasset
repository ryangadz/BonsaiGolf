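; BP_MenuTerrain is a menu actor that spawns and drives BP_Terrain actors from motion controller trigger input.
; Trigger press spawns a new BP_Terrain and passes it the controller transform, then axis and release events forward to that instance.
; Its preview mesh gets a green M_Mound dynamic material on construction.
; Tick keeps the mesh upright at the actor's yaw and toggles the material's Animate parameter with focus.
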(event `/RadialMenu/BPI_MenuItems.TriggerActionPress`
  (params (MotionControlTrans :type "Transform Structure"))
  (bind _returnvalue (`|SpawnActorFromClass` "/Game/Blueprints/MenuActors/BP_Terrain.BP_Terrain_C" (`KismetMathLibrary.MakeTransform` (0.0 0.0 0.0)) "Undefined" "OverrideRootScale" null null))
  (bind _output_get (set `self.TerrainActor` _returnvalue))
  (`/Game/Blueprints/MenuActors/BP_ForestTest2.TriggerActionPress` _output_get MotionControlTrans))

(event `/RadialMenu/BPI_MenuItems.TriggerAxis`
  (params (MotionControlTrans :type "Transform Structure") (AxisValue :type "Float (single-precision)"))
  (bind _terrainactor (`self.TerrainActor`))
  (`/Engine/EditorBlueprintResources/StandardMacros.IsValid` _terrainactor
    (:`Is Valid`
      (`/RadialMenu/BPI_MenuItems.TriggerAxis` _terrainactor MotionControlTrans 0.0))))

(event `/RadialMenu/BPI_MenuItems.TriggerActionRelease`
  (bind _terrainactor (`self.TerrainActor`))
  (`/Engine/EditorBlueprintResources/StandardMacros.IsValid` _terrainactor
    (:`Is Valid`
      (`/Game/Blueprints/MenuActors/BP_Terrain.TriggerActionRelease` _terrainactor))))

(event `self.ReceiveTick`
  (params (DeltaSeconds :type "Float (single-precision)"))
  (bind (_returnvalue_roll _returnvalue_pitch _returnvalue_yaw) (`KismetMathLibrary.BreakRotator` (`self.K2_GetActorRotation`)))
  (bind _dynamicmaterial (`self.DynamicMaterial`))
  (`SceneComponent.K2_SetWorldRotation` (`self.DefaultMeshComponent`) (`KismetMathLibrary.MakeRotator` 0.0 0.0 _returnvalue_yaw) false false)
  (if (`self.InFocus?`)
    (`MaterialInstanceDynamic.SetScalarParameterValue` _dynamicmaterial "Animate" 1.0)
    (else
      (`MaterialInstanceDynamic.SetScalarParameterValue` _dynamicmaterial "Animate" 0.0))))

(fn `UserConstructionScript`
  (`parent.UserConstructionScript`)
  (bind _returnvalue (`KismetMaterialLibrary.CreateDynamicMaterialInstance` "/Game/Materials/MenuMaterials/M_Mound.M_Mound"))
  (bind _output_get (set `self.Material` _returnvalue))
  (`PrimitiveComponent.SetMaterial` (`self.DefaultMeshComponent`) 0 _output_get)
  (`MaterialInstanceDynamic.SetVectorParameterValue` _output_get "Color" (struct :`R` 0.001685 :`G` 1.0 :`A` 1.0)))