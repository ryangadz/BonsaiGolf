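; Menu actor for the revolve tool, managing a BP_Revolve spawned in front of the player camera.
; Select spawns one, Focus shows or spawns it, and Unfocus hides it.
; Tick keeps its yaw aligned with the camera-to-actor direction while SelectedForUse is false.
; Motion-controller trigger events forward to it, with axis value fixed at zero, and release replaces the reference with NewVar1.
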(event `self.ReceiveTick`
  (params (DeltaSeconds :type "Float (single-precision)"))
  (bind _revolveactor (`self.RevolveActor`))
  (bind _returnvalue_location (`KismetMathLibrary.BreakTransform` (`SceneComponent.K2_GetComponentToWorld` (`PlayerCameraManager.TransformComponent` (`GameplayStatics.GetPlayerCameraManager` 0)))))
  (bind (_returnvalue_roll _returnvalue_pitch _returnvalue_yaw) (`KismetMathLibrary.BreakRotator` (`KismetMathLibrary.MakeRotFromX` (- (`self.K2_GetActorLocation` (`self.RevolveActor`)) _returnvalue_location))))
  (`parent.ReceiveTick` DeltaSeconds)
  (`/Engine/EditorBlueprintResources/StandardMacros.IsValid` _revolveactor
    (:`Is Valid`
      (if (not (`self.SelectedForUse`))
        (`self.K2_SetActorRotation` _revolveactor (`KismetMathLibrary.MakeRotator` 0.0 0.0 _returnvalue_yaw) false)))))

(event `self.TriggerActionPress`
  (params (MotionControlTrans :type "Transform Structure"))
  (bind _revolveactor (`self.RevolveActor`))
  (`/Engine/EditorBlueprintResources/StandardMacros.IsValid` _revolveactor
    (:`Is Valid`
      (`/Game/Blueprints/MenuActors/BP_Revolve.TriggerActionPress` _revolveactor MotionControlTrans))))

(event `self.TriggerAxis`
  (params (MotionControlTrans :type "Transform Structure") (AxisValue :type "Float (single-precision)"))
  (bind _revolveactor (`self.RevolveActor`))
  (`/Engine/EditorBlueprintResources/StandardMacros.IsValid` _revolveactor
    (:`Is Valid`
      (`/Game/Blueprints/MenuActors/BP_Revolve.TriggerAxis` _revolveactor MotionControlTrans 0.0))))

(event `self.TriggerActionRelease`
  (bind _revolveactor (`self.RevolveActor`))
  (`/Engine/EditorBlueprintResources/StandardMacros.IsValid` _revolveactor
    (:`Is Valid`
      (`/Game/Blueprints/MenuActors/BP_Revolve.TriggerActionRelease` _revolveactor)
      (set `self.RevolveActor` (`self.NewVar_1`)))))

(event `self.Select`
  (bind _transformcomponent (`PlayerCameraManager.TransformComponent` (`GameplayStatics.GetPlayerCameraManager` 0)))
  (bind _returnvalue_location (`KismetMathLibrary.BreakTransform` (`SceneComponent.K2_GetComponentToWorld` _transformcomponent)))
  (bind _returnvalue (+ _returnvalue_location (* (`SceneComponent.GetForwardVector` _transformcomponent) 150.0)))
  (bind (_returnvalue_roll _returnvalue_pitch _returnvalue_yaw) (`KismetMathLibrary.BreakRotator` (`KismetMathLibrary.MakeRotFromX` (- _returnvalue _returnvalue_location))))
  (bind _returnvalue_2 (`|SpawnActorFromClass` "/Game/Blueprints/MenuActors/BP_Revolve.BP_Revolve_C" (`KismetMathLibrary.MakeTransform` _returnvalue (`KismetMathLibrary.MakeRotator` 0.0 0.0 _returnvalue_yaw)) "Undefined" "OverrideRootScale" null null :!label _label))
  (set `self.RevolveActor` _returnvalue_2))

(event `self.Focus`
  (bind _revolveactor (`self.RevolveActor`))
  (`/Engine/EditorBlueprintResources/StandardMacros.IsValid` _revolveactor
    (:`Is Valid`
      (`SceneComponent.SetVisibility` (`/Game/Blueprints/MenuActors/BP_Revolve.DefaultSceneRoot` _revolveactor) true true))
    (:`Is Not Valid`
      (goto _label))))

(event `self.Unfocus`
  (bind _revolveactor (`self.RevolveActor`))
  (`/Engine/EditorBlueprintResources/StandardMacros.IsValid` _revolveactor
    (:`Is Valid`
      (`SceneComponent.SetVisibility` (`/Game/Blueprints/MenuActors/BP_Revolve.DefaultSceneRoot` _revolveactor) false true))))

(fn `UserConstructionScript`
  (`parent.UserConstructionScript`))