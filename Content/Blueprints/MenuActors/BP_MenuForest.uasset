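; BP_MenuForest is a motion-controller menu actor for placing a forest.
; A trigger press spawns a BP_ForestTest2 and passes it the press, then trigger axis events forward the controller transform to that actor with a zero axis value.
; Tick keeps the menu mesh upright at the actor's yaw and switches its material's Animate parameter on while in focus.
; Child-actor visibility nodes are left unconnected.
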(event `self.TriggerActionPress`
  (params (MotionControlTrans :type "Transform Structure"))
  (bind _returnvalue (`|SpawnActorFromClass` "/Game/Blueprints/MenuActors/BP_ForestTest2.BP_ForestTest2_C" (`KismetMathLibrary.MakeTransform` (0.0 0.0 0.0) (struct) (1.0 1.0 1.0)) "Undefined" "OverrideRootScale" null null))
  (bind _output_get (set `self.ForestActor` _returnvalue))
  (`/Game/Blueprints/MenuActors/BP_ForestTest2.TriggerActionPress` _output_get MotionControlTrans))

(event `self.TriggerAxis`
  (params (MotionControlTrans :type "Transform Structure") (AxisValue :type "Float (single-precision)"))
  (bind _forestactor (`self.ForestActor`))
  (`/Engine/EditorBlueprintResources/StandardMacros.IsValid` _forestactor
    (:`Is Valid`
      (`/RadialMenu/BPI_MenuItems.TriggerAxis` _forestactor MotionControlTrans 0.0))))

(event `self.ReceiveTick`
  (params (DeltaSeconds :type "Float (single-precision)"))
  (bind (_returnvalue_roll _returnvalue_pitch _returnvalue_yaw) (`KismetMathLibrary.BreakRotator` (`self.K2_GetActorRotation`)))
  (bind _dynamicmaterial (`self.DynamicMaterial`))
  (`SceneComponent.K2_SetWorldRotation` (`self.DefaultMeshComponent`) (`KismetMathLibrary.MakeRotator` 0.0 0.0 _returnvalue_yaw) false false)
  (if (`self.InFocus?`)
    (`MaterialInstanceDynamic.SetScalarParameterValue` _dynamicmaterial "Animate" 1.0)
    (else
      (`MaterialInstanceDynamic.SetScalarParameterValue` _dynamicmaterial "Animate" 0.0))))

(fn `UserConstructionScript`
  (`parent.UserConstructionScript`))