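; Blueprint helper functions for an array-backed min-heap of nodes, ordered by the sum of each node's X and Y.
; AddToHeap sifts the item at the count index upward through SortUpHeap and returns the incremented count.
; RemoveFirstItemOfHeap copies the first item into the given index, calls SortDownHeap from that index and returns a decremented, clamped count.
; Both sorts walk parent/child index math, exchanging entries through SwapItemsOfHeap.
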(fn `AddToHeap`
  (params (Nodes :type "Array of /Game/Blueprints/S_Heap Structure") (ItemCount :type Integer))
  (returns (Heap :type "Array of /Game/Blueprints/S_Heap Structure") (ItemCountOut :type Integer))
  (locals (HeapOfNodes :type "Array of  Structure"))
  (`self.SortUpHeap` Nodes ItemCount)
  (return (`local.Nodes`) (+ ItemCount 1)))

(fn `RemoveFirstItemOfHeap`
  (params (Nodes :type "Array of /Game/Blueprints/S_Heap Structure") (Index :type Integer))
  (returns (IndexNew :type Integer))
  (bind _returnvalue (- Index 1))
  (if (> Index 1)
    (`KismetArrayLibrary.Array_Set` Nodes (`local.Index`) (`|GetArrayItem` Nodes))
    (`self.SortDownHeap` (`local.Index`) (`local.Nodes`) _returnvalue))
  (return (`KismetMathLibrary.Clamp` _returnvalue 0 10000)))

(fn `SortDownHeap`
  (params (HeapIndex :type Integer) (Nodes :type "Array of /Game/Blueprints/S_Heap Structure") (NewParam :type Integer))
  (locals (childIndexLeft :type Integer) (childIndexRight :type Integer) (swapIndex :type Integer) (Continue :type Boolean :default true) (Currentindex :type Integer))
  (bind _swapindex (`local.swapIndex`))
  (bind (_output_x _output_y) (break `/Game/Blueprints/S_Heap` (`|GetArrayItem` Nodes (`local.childIndexLeft`))))
  (bind (_output_x_2 _output_y_2) (break `/Game/Blueprints/S_Heap` (`|GetArrayItem` Nodes (`local.swapIndex`))))
  (bind (_output_x_3 _output_y_3) (break `/Game/Blueprints/S_Heap` (`|GetArrayItem` Nodes (`local.Currentindex`))))
  (bind (_output_x_4 _output_y_4) (break `/Game/Blueprints/S_Heap` (`|GetArrayItem` Nodes (`local.childIndexRight`))))
  (set `local.Currentindex` HeapIndex)
  (while (`local.Continue`)
    (bind _output_get (set `local.childIndexLeft` (+ (* (`local.Currentindex`) 2) 1)))
    (set `local.childIndexRight` (+ _output_get 1))
    (if (<= (`local.childIndexLeft`) NewParam)
      (set `local.swapIndex` (`local.childIndexLeft`))
      (if (<= (`local.childIndexRight`) NewParam)
        (`/Engine/EditorBlueprintResources/StandardMacros.CompareInt` (+ _output_x _output_y) (+ _output_x_4 _output_y_4)
          (:`>`
            (set `local.swapIndex` (`local.childIndexRight`)))
          (:`==`
            _)
          (:`<`
            _))
        (`/Engine/EditorBlueprintResources/StandardMacros.CompareInt` (+ _output_x_3 _output_y_3) (+ _output_x_2 _output_y_2)
          (:`>`
            (`self.SwapItemsOfHeap` (`local.Currentindex`) _swapindex (`local.Nodes`))
            (set `local.Currentindex` _swapindex))
          (:`==`
            (set `local.Continue` false :!label _label))
          (:`<`
            (goto _label)))
        (else
          (set `local.Continue` false)))
      (else
        (set `local.Continue` false))))
  (return))

(fn `SortUpHeap`
  (params (NodeArray :type "Array of /Game/Blueprints/S_Heap Structure") (Index :type Integer))
  (locals (ParentIndex :type Integer) (Continue :type Boolean :default true) (IndexLocal :type Integer))
  (bind _parentindex (`local.ParentIndex`))
  (bind _output_get (set `local.IndexLocal` Index))
  (bind _output_get_2 (set `local.ParentIndex` (/ (- Index 1) 2)))
  (while (`local.Continue`)
    (bind (_output_x _output_y) (break `/Game/Blueprints/S_Heap` (`|GetArrayItem` NodeArray _output_get)))
    (bind (_output_x_2 _output_y_2) (break `/Game/Blueprints/S_Heap` (`|GetArrayItem` NodeArray _output_get_2)))
    (`/Engine/EditorBlueprintResources/StandardMacros.CompareInt` (+ _output_x _output_y) (+ _output_x_2 _output_y_2)
      (:`>`
        (set `local.Continue` false :!label _label))
      (:`==`
        (goto _label))
      (:`<`
        (`self.SwapItemsOfHeap` (`local.IndexLocal`) _parentindex NodeArray)
        (set `local.IndexLocal` _parentindex)
        (set `local.ParentIndex` (/ (- _parentindex 1) 2)))))
  (return))

(fn `SwapItemsOfHeap`
  (params (IndexA :type Integer) (IndexB :type Integer) (Nodes :type "Array of /Game/Blueprints/S_Heap Structure"))
  (locals (NewLocalVar_0 :type "/Game/Blueprints/S_Heap Structure") (ItemAIndex :type "/Game/Blueprints/S_Heap Structure"))
  (set `local.ItemAIndex` (`|GetArrayItem` (`local.Nodes`) (`local.IndexA`)))
  (`KismetArrayLibrary.Array_Set` (`local.Nodes`) (`local.IndexA`) (`|GetArrayItem` (`local.Nodes`) (`local.IndexB`)))
  (`KismetArrayLibrary.Array_Set` (`local.Nodes`) (`local.IndexB`) (`local.ItemAIndex`))
  (return))