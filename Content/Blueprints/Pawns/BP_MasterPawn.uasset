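; Base VR/Magic Leap player pawn that carries a radial menu and a laser pointer on its motion controller.
; BeginPlay spawns BP_RadialMenu from a data table and attaches it to the controller; trigger, shoulder, thumbstick and home inputs forward to it.
; Tick rolls the visible laser about its axis to face the camera.
; A LineTrace event scales the laser to hit distance, and ChangeLaserColor tints its dynamic material.
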(event `self.ReceiveTick`
  (params (DeltaSeconds :type "Float (single-precision)"))
  (bind _laser (`self.Laser`))
  (if (`SceneComponent.IsVisible` _laser)
    (`SceneComponent.K2_SetRelativeRotation` _laser (`KismetMathLibrary.MakeRotator` (`self.LaserRelativeRoll`)) false false)))

(event `LineTrace`
  (bind _laser (`self.Laser`))
  (bind _returnvalue (`SceneComponent.K2_GetComponentLocation` _laser))
  (bind (_outhit _returnvalue_2) (`KismetSystemLibrary.LineTraceSingleForObjects` _returnvalue (+ _returnvalue (* (`SceneComponent.GetForwardVector` _laser) 500.0)) (`|MakeArray` "ObjectTypeQuery1" "ObjectTypeQuery2" :!type "EObjectTypeQuery Enum")))
  (if _returnvalue_2
    (`SceneComponent.SetWorldScale3D` (`self.Laser`) (`KismetMathLibrary.MakeVector` (`.Distance` (`GameplayStatics.BreakHitResult` _outhit)) 0.3 0.3))))

(event `self.ReceiveBeginPlay`
  (bind _returnvalue (`SceneComponent.K2_GetComponentToWorld` (`self.MotionController`)))
  (set `MotionControllerComponent.MotionSource` "AnyHand" (`self.MotionController`))
  (bind _returnvalue_2 (`|SpawnActorFromClass` "/RadialMenu/BP_RadialMenu.BP_RadialMenu_C" (`KismetMathLibrary.MakeTransform` (.location _returnvalue) (`KismetMathLibrary.MakeRotator` (.roll (.rotation _returnvalue)) (+ (.pitch (.rotation _returnvalue)) 15.0) (.yaw (.rotation _returnvalue))) (.scale _returnvalue)) "Undefined" "OverrideRootScale" null 0.25 "/Game/Blueprints/Data/DT_SUB_ACTORS1.DT_SUB_ACTORS1" "Main" null))
  (bind _output_get (set `self.RadialMenu` _returnvalue_2))
  (`self.K2_AttachToComponent` _output_get (`self.MotionController`) "None" "KeepRelative" "KeepRelative" "KeepRelative" true)
  (`KismetSystemLibrary.K2_SetTimerDelegate` (`|CreateDelegate` :!event `LineTrace`) 0.25 true))

(event `Key|MotionController_Right_Shoulder`
  (params (Key :type "Key Structure"))
  (bind _radialmenu (`self.RadialMenu`))
  (:`Pressed`
    (`/Engine/EditorBlueprintResources/StandardMacros.IsValid` _radialmenu
      (:`Is Valid`
        (`/RadialMenu/BP_RadialMenu.ShoulderSelect` _radialmenu)))))

(event `Key|MotionController_Right_Trigger`
  (params (Key :type "Key Structure"))
  (bind _radialmenu (`self.RadialMenu`))
  (:`Pressed`
    (`/Engine/EditorBlueprintResources/StandardMacros.IsValid` _radialmenu
      (:`Is Valid`
        (`/RadialMenu/BP_RadialMenu.TriggerAction` _radialmenu (`SceneComponent.K2_GetComponentToWorld` (`self.MotionController`))))))
  (:`Released`
    (`/Engine/EditorBlueprintResources/StandardMacros.IsValid` _radialmenu
      (:`Is Valid`
        (`/RadialMenu/BP_RadialMenu.TriggerActionRelease` _radialmenu)))))

(event `InputAxisKey|MotionController_Right_TriggerAxis`
  (params (AxisValue :type "Float (single-precision)"))
  (bind _radialmenu (`self.RadialMenu`))
  (`/Engine/EditorBlueprintResources/StandardMacros.IsValid` _radialmenu
    (:`Is Valid`
      (`/RadialMenu/BP_RadialMenu.TriggerAxis` _radialmenu (`SceneComponent.K2_GetComponentToWorld` (`self.MotionController`)) AxisValue))))

(event `InputAxisKey|MotionController_Right_Thumbstick_X`
  (params (AxisValue :type "Float (single-precision)"))
  (bind _radialmenu (`self.RadialMenu`))
  (`/Engine/EditorBlueprintResources/StandardMacros.IsValid` _radialmenu
    (:`Is Valid`
      (`/RadialMenu/BP_RadialMenu.UpdateRadialMenu` _radialmenu AxisValue (`self.GetInputAxisKeyValue`)))))

(event `Key|MagicLeap_Right_HomeButton`
  (params (Key :type "Key Structure"))
  (bind _radialmenu (`self.RadialMenu`))
  (:`Pressed`
    (`/Engine/EditorBlueprintResources/StandardMacros.IsValid` _radialmenu
      (:`Is Valid`
        (`/RadialMenu/BP_RadialMenu.GoBack` _radialmenu)))))

(event `/Game/Blueprints/BPI_MasterPawn.ChangeLaserColor`
  (params (NewColor :type "LinearColor Structure"))
  (`MaterialInstanceDynamic.SetVectorParameterValue` (`self.LaserMaterial`) "Color" NewColor))

(event `/Game/Blueprints/BPI_MasterPawn.AddLaser`)

(fn `LaserRelativeRoll`
  (returns (Roll :type "Float (double-precision)"))
  (bind _motioncontroller (`self.MotionController`))
  (bind _motioncontroller_2 (`self.MotionController`))
  (bind _returnvalue (`SceneComponent.GetForwardVector` _motioncontroller_2))
  (bind _returnvalue_2 (`KismetMathLibrary.Normal` (- (`SceneComponent.K2_GetComponentLocation` (`self.Camera`)) (`SceneComponent.K2_GetComponentLocation` _motioncontroller_2)) 0.001))
  (bind _returnvalue_3 (`KismetMathLibrary.Normal` (- _returnvalue_2 (* _returnvalue (`KismetMathLibrary.Dot_VectorVector` _returnvalue_2 _returnvalue))) 0.001))
  (return (* (`KismetMathLibrary.DegAcos` (`KismetMathLibrary.Dot_VectorVector` _returnvalue_3 (`SceneComponent.GetUpVector` _motioncontroller))) (`KismetMathLibrary.SignOfFloat` (`KismetMathLibrary.Dot_VectorVector` _returnvalue_3 (`SceneComponent.GetRightVector` _motioncontroller))))))

(fn `UserConstructionScript`
  (bind _returnvalue (`PrimitiveComponent.CreateDynamicMaterialInstance` (`self.Laser`) 0 "/Game/Materials/M_Laser.M_Laser" "None"))
  (set `self.LaserMaterial` _returnvalue))