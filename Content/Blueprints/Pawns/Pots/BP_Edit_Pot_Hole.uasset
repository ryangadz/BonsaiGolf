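; VR motion-controller pawn for placing pot holes, built as small procedural meshes at the aimed point.
; Tick line-traces world-static objects from the controller and stores the impact point.
; Releasing the right trigger adds a sunken disk and cylinder wall there, with concrete on the disk, without cutting existing geometry.
; Disconnected nodes hold unused logic for selecting a pot and denting its rebuilt grass mesh.
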(event `self.ReceiveTick`
  (params (DeltaSeconds :type "Float (single-precision)"))
  (bind _motioncontroller (`self.MotionController`))
  (bind _returnvalue (`SceneComponent.K2_GetComponentLocation` _motioncontroller))
  (`parent.ReceiveTick` DeltaSeconds)
  (bind _outhit (`KismetSystemLibrary.LineTraceSingleForObjects` :`Start` _returnvalue :`End` (+ _returnvalue (* (`SceneComponent.GetForwardVector` _motioncontroller) 1000.0)) :`ObjectTypes` (`|MakeArray` "ObjectTypeQuery1" :!type "EObjectTypeQuery Enum") :`bTraceComplex` true :`DrawDebugType` "ForOneFrame"))
  (set `self.Desired Point` (`.ImpactPoint` (`GameplayStatics.BreakHitResult` _outhit))))

(event `Key|MotionController_Right_Trigger`
  (params (Key :type "Key Structure"))
  (:`Released`
    (bind (_vertices _triangles) (`/Game/Blueprints/BFL_MeshBuilding.MakePlanarDiskVerts` (- (`self.Desired Point`) (0.0 0.0 10.0)) 10.0 12))
    (bind _returnvalue (`AddComponent|NODE_AddProceduralMeshComponent-1`))
    (`ProceduralMeshComponent.CreateMeshSection_LinearColor` :`self` _returnvalue :`Vertices` _vertices :`Triangles` _triangles)
    (bind (_vertices_2 _triangles_2) (`/Game/Blueprints/BFL_MeshBuilding.MakeCylinderVerts` (- (`self.Desired Point`) (0.0 0.0 10.0)) 10.0 12 10.0))
    (`ProceduralMeshComponent.CreateMeshSection_LinearColor` :`self` _returnvalue :`SectionIndex` 1 :`Vertices` _vertices_2 :`Triangles` _triangles_2)
    (`PrimitiveComponent.SetMaterial` _returnvalue 0 "/Game/Materials/M_Concrete.M_Concrete")))

(fn `UserConstructionScript`
  (`parent.UserConstructionScript`))