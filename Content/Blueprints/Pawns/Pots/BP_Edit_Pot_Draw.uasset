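; VR edit pawn that lets the player draw pots with the right motion controller.
; Pressing the trigger spawns a BP_PotActor at the controller's location and yaw, then begins the pot with that controller.
; While drawing is active, trigger axis events call DrawPot on that actor.
; Releasing stops drawing and resets the DoOnce guard for the next pot, and a custom event can also set the drawing flag.
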(event `/Game/Blueprints/PotInterface.CustomIsDrawingEvent`
  (params (Drawing :type Boolean))
  (set `self.IsDrawing` Drawing))

(event `Key|MotionController_Right_Trigger`
  (params (Key :type "Key Structure"))
  (bind _returnvalue (`SceneComponent.K2_GetComponentToWorld` (`self.MotionController`)))
  (:`Pressed`
    (set `self.IsDrawing` true)
    (`/Engine/EditorBlueprintResources/StandardMacros.DoOnce` false :!label _label
      (:`Completed`
        (bind _returnvalue_2 (`|SpawnActorFromClass` "/Game/Blueprints/BP_PotActor.BP_PotActor_C" (`KismetMathLibrary.MakeTransform` (.location _returnvalue) (`KismetMathLibrary.MakeRotator` 0.0 0.0 (.yaw (.rotation _returnvalue)))) "Undefined" "OverrideRootScale" null null))
        (bind _output_get (set `self.PotActor` _returnvalue_2))
        (`/Game/Blueprints/BP_PotActor.BeginPot` _output_get (`self.MotionController`)))))
  (:`Released`
    (set `self.IsDrawing` false)
    (goto _label :!via `Reset`)))

(event `InputAxisKey|MotionController_Right_TriggerAxis`
  (params (AxisValue :type "Float (single-precision)"))
  (if (`self.IsDrawing`)
    (`/Game/Blueprints/BP_PotActor.DrawPot` (`self.PotActor`))))

(fn `UserConstructionScript`
  (`parent.UserConstructionScript`))