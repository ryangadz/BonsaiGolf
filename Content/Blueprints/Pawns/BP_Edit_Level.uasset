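; VR level-editing pawn that spawns and positions a BP_Course with a motion controller.
; Pressing the right trigger spawns a new, scaled-down course at the last stored Location and keeps it as Level.
; While held, Tick traces forward from the controller against WorldStatic objects with a debug line, updates Location slightly above the hit and interpolates the course toward it.
; Releasing the trigger leaves the course in place.
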(event `self.ReceiveTick`
  (params (DeltaSeconds :type "Float (single-precision)"))
  (bind _motioncontroller (`self.MotionController`))
  (bind _level (`self.Level`))
  (bind _returnvalue (`SceneComponent.K2_GetComponentLocation` _motioncontroller))
  (if (`self.Pressed?`)
    (bind _outhit (`KismetSystemLibrary.LineTraceSingleForObjects` :`Start` _returnvalue :`End` (+ _returnvalue (* (`SceneComponent.GetForwardVector` _motioncontroller) 1000.0)) :`ObjectTypes` (`|MakeArray` "ObjectTypeQuery1" :!type "EObjectTypeQuery Enum") :`DrawDebugType` "ForOneFrame"))
    (if (`GameplayStatics.BreakHitResult` _outhit)
      (bind _output_get (set `self.location` (+ (`.ImpactPoint` (`GameplayStatics.BreakHitResult` _outhit)) (0.0 0.0 14.0))))
      (`/Engine/EditorBlueprintResources/StandardMacros.IsValid` _level
        (:`Is Valid`
          (`self.K2_SetActorLocation` _level (`KismetMathLibrary.VInterpTo` (`self.K2_GetActorLocation` _level) _output_get (`GameplayStatics.GetWorldDeltaSeconds`) 20.0) false false))))))

(event `InputAxisKey|MotionController_Right_TriggerAxis`
  (params (AxisValue :type "Float (single-precision)")))

(event `Key|MotionController_Right_Trigger`
  (params (Key :type "Key Structure"))
  (:`Pressed`
    (set `self.Pressed?` true)
    (bind _returnvalue (`|SpawnActorFromClass` "/Game/Blueprints/BP_Course.BP_Course_C" (`KismetMathLibrary.MakeTransform` (`self.location`) (struct :`Yaw` 190.0) (0.66 0.66 0.66)) "Undefined" "OverrideRootScale" null null))
    (set `self.Level` _returnvalue))
  (:`Released`
    (set `self.Pressed?` false)))

(fn `UserConstructionScript`
  (`parent.UserConstructionScript`))