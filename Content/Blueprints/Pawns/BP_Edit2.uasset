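; VR pawn that serves as a radial selector for switching the player into one of its SubPawns.
; On BeginPlay it spawns a BP_RadialMenuOLD on XRControl, laid out with one evenly spaced icon per sub-pawn.
; Right thumbstick angle, converted to 0–360 degrees, picks the current tool and resizes the icons.
; Releasing the thumbstick button spawns that pawn in place, possesses it and destroys this one; menu cleanup and handover nodes are unconnected.
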(event `self.ReceiveBeginPlay`
  (bind _subpawns (`self.SubPawns`))
  (bind _returnvalue (`SceneComponent.K2_GetComponentToWorld` (`self.XR_Control`)))
  (`parent.ReceiveBeginPlay`)
  (bind _returnvalue_2 (`|SpawnActorFromClass` "/Game/Blueprints/RadialMenu/BP_RadialMenuOLD.BP_RadialMenuOLD_C" (`KismetMathLibrary.MakeTransform` (.location _returnvalue) (`KismetMathLibrary.MakeRotator` (.roll (.rotation _returnvalue)) (- (.pitch (.rotation _returnvalue)) -15.0) (.yaw (.rotation _returnvalue))) (.scale _returnvalue)) "Undefined" "OverrideRootScale" self null))
  (set `self.RadialMenu` _returnvalue_2)
  (bind _output_get (set `self.AngleBetweenIcons` (`self.CalcAngleBetweenIcons` _subpawns)))
  (`/Game/Blueprints/RadialMenu/BP_RadialMenuOLD.ChangeToolLayout` (`self.RadialMenu`) (`KismetArrayLibrary.Array_Length` _subpawns) (`self.SubPawns`) _output_get)
  (`self.K2_AttachToComponent` (`self.RadialMenu`) (`self.XR_Control`) "None" "KeepRelative" "KeepRelative" "KeepRelative" false))

(event `InputAxisKey|MotionController_Right_Thumbstick_X`
  (params (AxisValue :type "Float (single-precision)"))
  (bind _radialmenu (`self.RadialMenu`))
  (bind _returnvalue (`KismetMathLibrary.DegAtan2` AxisValue (`self.GetInputAxisKeyValue`)))
  (bind _returnvalue_2 (`KismetMathLibrary.Round` (/ (+ _returnvalue (* (/ (- (`KismetMathLibrary.SignOfFloat` _returnvalue) 1.0) 2.0) -360.0)) (`self.AngleBetweenIcons`))))
  (if (!= _returnvalue 0.0)
    (if (!= _returnvalue_2 (`self.CurrentTool`))
      (bind _output_get (set `self.CurrentTool` _returnvalue_2))
      (`/Engine/EditorBlueprintResources/StandardMacros.IsValid` _radialmenu
        (:`Is Valid`
          (`/Game/Blueprints/RadialMenu/BP_RadialMenuOLD.Resize Icons` _radialmenu _output_get))))))

(event `Key|MotionController_Right_Thumbstick`
  (params (Key :type "Key Structure")))

(event `Key|MotionController_Right_Thumbstick`
  (params (Key :type "Key Structure"))
  (bind (_returnvalue_location _returnvalue_rotation) (`KismetMathLibrary.BreakTransform` (`self.GetTransform`)))
  (:`Released`
    (bind _returnvalue (`|SpawnActorFromClass` (`|GetArrayItem` (`self.SubPawns`) (`self.CurrentTool`)) (`KismetMathLibrary.MakeTransform` _returnvalue_location _returnvalue_rotation) "Undefined" "OverrideRootScale" null null))
    (`Controller.Possess` (`GameplayStatics.GetPlayerController` 0) _returnvalue)
    (`self.K2_DestroyActor` self)))

(fn `CalcAngleBetweenIcons`
  (params (SubClasses :type "Array of /Game/Blueprints/Pawns/Master_Pawn Class Reference"))
  (returns (Angle :type "Float (double-precision)"))
  (return (/ 360.0 (`KismetMathLibrary.Conv_IntToDouble` (`KismetArrayLibrary.Array_Length` SubClasses)))))

(fn `UserConstructionScript`
  (`parent.UserConstructionScript`))