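; VR editing pawn that spawns and places trees with the right motion controller trigger.
; Pressing the trigger spawns a TreeRoot actor and picks a random height offset; releasing it leaves the tree in place.
; While held, Tick line-traces WorldStatic objects along the XRControl forward vector, eases the tree toward the hit point plus that offset, and rebuilds it.
; Unconnected nodes for rotating the tree remain in the graph.
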(event `self.ReceiveTick`
  (params (DeltaSeconds :type "Float (single-precision)"))
  (bind _tree (`self.Tree`))
  (bind _returnvalue (`SceneComponent.K2_GetComponentLocation` (`self.XR_Control`)))
  (`parent.ReceiveTick` DeltaSeconds)
  (if (`self.Pressed?`)
    (bind _outhit (`KismetSystemLibrary.LineTraceSingleForObjects` _returnvalue (+ _returnvalue (* (`SceneComponent.GetForwardVector` (`self.XR_Control`)) 1000.0)) (`|MakeArray` "ObjectTypeQuery1" :!type "EObjectTypeQuery Enum")))
    (if (`GameplayStatics.BreakHitResult` _outhit)
      (bind _output_get (set `self.location` (+ (`.ImpactPoint` (`GameplayStatics.BreakHitResult` _outhit)) (`KismetMathLibrary.MakeVector` 0.0 0.0 (`self.RandomHeight`)))))
      (`/Engine/EditorBlueprintResources/StandardMacros.IsValid` _tree
        (:`Is Valid`
          (`self.K2_SetActorLocation` _tree (`KismetMathLibrary.VInterpTo` (`self.K2_GetActorLocation` _tree) _output_get (`GameplayStatics.GetWorldDeltaSeconds`) 20.0) false false)
          (`/Game/Blueprints/MenuActors/Build/Tree/TreeRoot.Rebuild Tree` (`self.Tree`)))))))

(event `InputAxisKey|MotionController_Right_TriggerAxis`
  (params (AxisValue :type "Float (single-precision)")))

(event `Key|MotionController_Right_Trigger`
  (params (Key :type "Key Structure"))
  (:`Pressed`
    (set `self.Pressed?` true)
    (set `self.RandomHeight` (`KismetMathLibrary.RandomFloatInRange` 5.0 12.0))
    (bind _returnvalue (`|SpawnActorFromClass` "/Game/Blueprints/MenuActors/Build/Tree/TreeRoot.TreeRoot_C" (`KismetMathLibrary.MakeTransform` (0.0 0.0 0.0)) "Undefined" "OverrideRootScale" null null))
    (set `self.Tree` _returnvalue))
  (:`Released`
    (set `self.Pressed?` false)))

(fn `UserConstructionScript`
  (`parent.UserConstructionScript`))