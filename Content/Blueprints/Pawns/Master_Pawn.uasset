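; Master pawn for motion-controller XR, apparently a base for tool pawns, that handles pawn switching and radial tool selection.
; BeginPlay sets the controller to either hand and removes any leftover old radial menu.
; The Magic Leap home button spawns and possesses BP_Edit2, then destroys this pawn.
; Right thumbstick angle picks a tool index and messages the radial menu to resize, though the menu-spawning logic is disconnected.
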(event `self.ReceiveBeginPlay`
  (set `self.CurrentPawn` self)
  (set `MotionControllerComponent.MotionSource` "AnyHand" (`self.XR_Control`))
  (bind _outactors (`GameplayStatics.GetAllActorsOfClass` "/Game/Blueprints/RadialMenu/BP_RadialMenuOLD.BP_RadialMenuOLD_C"))
  (bind _output (`|GetArrayItem` _outactors))
  (if (`KismetSystemLibrary.IsValid` _output)
    (`self.K2_DestroyActor` _output)))

(event `Key|MagicLeap_Right_HomeButton`
  (params (Key :type "Key Structure"))
  (:`Pressed`
    (bind _returnvalue (`AIBlueprintHelperLibrary.SpawnAIFromClass` "/Game/Blueprints/Pawns/BP_Edit2.BP_Edit2_C"))
    (`Controller.Possess` (`GameplayStatics.GetPlayerController` 0) _returnvalue)
    (`self.K2_DestroyActor` self)))

(event `Key|MagicLeap_Left_HomeButton`
  (params (Key :type "Key Structure")))

(event `InputAxisKey|MotionController_Right_Thumbstick_X`
  (params (AxisValue :type "Float (single-precision)"))
  (bind _returnvalue (`KismetMathLibrary.DegAtan2` AxisValue (stale `InputAxisKey|MotionController_Right_Thumbstick_Y` AxisValue)))
  (if (!= _returnvalue 0.0) :!label _label
    (bind _returnvalue_2 (`KismetMathLibrary.Round` (/ (+ _returnvalue (* (/ (- (`KismetMathLibrary.SignOfFloat` _returnvalue) 1.0) 2.0) -360.0)) (`/Game/Blueprints/RadialMenu/BP_RadialMenuOLD.AngleBetweenTools` (`self.RadialMenu`)))))
    (if (!= (`self.CurrentTool`) _returnvalue_2)
      (bind _output_get (set `self.CurrentTool` _returnvalue_2))
      (message `/Game/Blueprints/Libraries/BPI_RadialMenu.ResizeTools` (`self.RadialMenu`) _output_get (`self.SubPawns`)))))

(event `InputAxisKey|MotionController_Right_Thumbstick_Y`
  (params (AxisValue :type "Float (single-precision)"))
  (goto _label))

(fn `UserConstructionScript`)