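; VR motion-controller pawn for drawing pots in the world.
; A right trigger press spawns a BP_PotActor at the controller and calls BeginPot, then trigger axis input calls its DrawPot until release.
; Spline-stroke code that closes loops and fills them with procedural grass meshes on a triangle grid remains, but is disconnected from the live input path.
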(event `Key|MotionController_Right_Shoulder`
  (params (Key :type "Key Structure")))

(event `self.ReceiveBeginPlay`
  (`parent.ReceiveBeginPlay`)
  (set `MotionControllerComponent.MotionSource` "AnyHand" (`self.MotionController_0`)))

(event `Key|MotionController_Right_Trigger`
  (params (Key :type "Key Structure"))
  (bind _returnvalue (`SceneComponent.K2_GetComponentToWorld` (`self.MotionController`)))
  (:`Pressed`
    (set `self.IsDrawing` true)
    (`/Engine/EditorBlueprintResources/StandardMacros.DoOnce` false :!label _label
      (:`Completed`
        (bind _returnvalue_2 (`|SpawnActorFromClass` "/Game/Blueprints/BP_PotActor.BP_PotActor_C" (`KismetMathLibrary.MakeTransform` (.location _returnvalue) (`KismetMathLibrary.MakeRotator` 0.0 0.0 (.yaw (.rotation _returnvalue)))) "Undefined" "OverrideRootScale" null null))
        (bind _output_get (set `self.PotActor` _returnvalue_2))
        (`/Game/Blueprints/BP_PotActor.BeginPot` _output_get (`self.MotionController`)))))
  (:`Released`
    (set `self.IsDrawing` false)
    (goto _label :!via `Reset`)))

(event `/Game/Blueprints/PotInterface.CustomIsDrawingEvent`
  (params (Drawing :type Boolean))
  (set `self.IsDrawing` Drawing))

(event `InputAxisKey|MotionController_Right_TriggerAxis`
  (params (AxisValue :type "Float (single-precision)"))
  (if (`self.IsDrawing`)
    (`/Game/Blueprints/BP_PotActor.DrawPot` (`self.PotActor`))))

(fn `CheckForLoopAndComplete`
  (returns (Continue :type Boolean))
  (locals (`Continue?` :type Boolean :default true) (GridPoints :type "Array of Integer") (Index :type Integer) (GridXPlus1 :type Integer :default 0))
  (bind _currentsplinewithmesh (`self.CurrentSplineWithMesh`))
  (bind _index (`local.Index`))
  (bind _gridpoints (`local.GridPoints`))
  (bind _index_2 (`local.Index`))
  (bind _gridpoints_2 (`local.GridPoints`))
  (bind _index_3 (`local.Index`))
  (bind _triangles (`self.Triangles`))
  (bind _currentsplinewithmesh_2 (`self.CurrentSplineWithMesh`))
  (bind _currentsplinewithmesh_3 (`self.CurrentSplineWithMesh`))
  (bind _currentsplinewithmesh_4 (`self.CurrentSplineWithMesh`))
  (bind _triangles_2 (`self.Triangles`))
  (bind _returnvalue (`SplineComponent.GetNumberOfSplinePoints` _currentsplinewithmesh_4))
  (bind _returnvalue_2 (- (`local.Index`) (`local.GridXPlus1`)))
  (bind _returnvalue_3 (`SplineComponent.GetNumberOfSplinePoints` _currentsplinewithmesh_3))
  (bind _returnvalue_4 (- _index_3 (`local.GridXPlus1`)))
  (bind _returnvalue_5 (- _returnvalue_3 2))
  (bind _returnvalue_6 (- _returnvalue_3 1))
  (bind _output (`|GetArrayItem` _gridpoints (+ _index 1)))
  (bind _output_2 (`|GetArrayItem` _gridpoints_2 _returnvalue_4))
  (bind _returnvalue_7 (`SplineComponent.GetLocationAtSplinePoint` _currentsplinewithmesh_3 _returnvalue_6 "World"))
  (bind _returnvalue_8 (`SplineComponent.GetLocationAtSplinePoint` _currentsplinewithmesh_3 _returnvalue_5 "World"))
  (bind _output_3 (`|GetArrayItem` _gridpoints_2 (- _returnvalue_4 -1)))
  (bind _returnvalue_9 (- _index (- (`local.GridXPlus1`) (mod (/ (`local.Index`) (`local.GridXPlus1`)) 2))))
  (bind _returnvalue_10 (+ _returnvalue_7 _returnvalue_8))
  (bind _returnvalue_11 (+ (+ (* (mod (/ (`local.Index`) (`local.GridXPlus1`)) 2) -1) 1) _index_3))
  (bind _output_4 (`|GetArrayItem` _gridpoints _returnvalue_9))
  (bind _output_5 (`|GetArrayItem` _gridpoints_2 _returnvalue_11))
  (if (and (> _returnvalue 3) (<= (`KismetMathLibrary.VSize` (- (`SplineComponent.GetLocationAtSplinePoint` _currentsplinewithmesh_4 0 "World") (`SplineComponent.GetLocationAtSplinePoint` _currentsplinewithmesh_4 (- _returnvalue 1) "World"))) 10.0))
    (set `self.IsDrawing` false)
    (set `local.Continue?` false)
    (if (not (> (`KismetMathLibrary.VSize` _returnvalue_10) 5.0))
      (`SplineComponent.SetLocationAtSplinePoint` _currentsplinewithmesh _returnvalue_5 (/ _returnvalue_10 2.0) "World" false)
      (`SplineComponent.SetTangentAtSplinePoint` _currentsplinewithmesh _returnvalue_6 (* (`KismetMathLibrary.Normal` (/ (+ (`SplineComponent.GetTangentAtSplinePoint` _currentsplinewithmesh_3 _returnvalue_6 "World") (`SplineComponent.GetTangentAtSplinePoint` _currentsplinewithmesh_3 _returnvalue_5 "World")) 2.0)) (+ (/ (`KismetMathLibrary.VSize` (- _returnvalue_7 _returnvalue_8)) 2.0) 10.0)) "World" true)
      (`SplineComponent.RemoveSplinePoint` _currentsplinewithmesh _returnvalue_6 true))
    (`SplineComponent.SetClosedLoop` _currentsplinewithmesh_2 true true)
    (`SplineComponent.SetTangentAtSplinePoint` _currentsplinewithmesh_2 0 (* (`KismetMathLibrary.Normal` (- (`SplineComponent.GetLocationAtSplinePoint` _currentsplinewithmesh_3 1 "World") (`SplineComponent.GetLocationAtSplinePoint` _currentsplinewithmesh_3 _returnvalue_6 "World"))) 10.0) "World" true)
    (`SplineWithMesh.AddMesh` (`self.CurrentSplineWithMesh`) self)
    (bind (_points _verts _gridx) (`/Game/Blueprints/BFL_MeshBuilding.MakePointGrid` (`self.CurrentSplineWithMesh`)))
    (bind _output_get (set `local.GridPoints` _points))
    (bind _output_get_2 (set `local.GridXPlus1` (+ _gridx 1)))
    (`self.ClearMeshArrays`)
    (for _index_4 (range _output_get_2 (+ (- (`KismetArrayLibrary.Array_Length` _output_get) 2) 1))
      (set `local.Index` _index_4)
      (`|ExecutionSequence`
        (:`then_0`
          (if (and (!= _output_5 -1) (!= _output_2 -1) (!= _output_3 -1) (!= (+ _output_5 _output_2 _output_3) 3))
            (`KismetArrayLibrary.Array_Add` _triangles_2 _returnvalue_11)
            (`KismetArrayLibrary.Array_Add` _triangles_2 (- _returnvalue_2 -1))
            (`KismetArrayLibrary.Array_Add` _triangles_2 _returnvalue_2)))
        (:`then_1`
          (bind _output_6 (`|GetArrayItem` _gridpoints _index_4))
          (if (and (!= _output_6 -1) (!= _output -1) (!= _output_4 -1) (!= (+ _output_6 _output _output_4) 3))
            (`KismetArrayLibrary.Array_Add` _triangles _index_2)
            (`KismetArrayLibrary.Array_Add` _triangles (+ _index_2 1))
            (`KismetArrayLibrary.Array_Add` _triangles _returnvalue_9)))))
    (bind _returnvalue_12 (`AddComponent|NODE_AddProceduralMeshComponent-1`))
    (`ProceduralMeshComponent.CreateMeshSection_LinearColor` :`self` _returnvalue_12 :`Vertices` _verts :`Triangles` (`self.Triangles`) :`bCreateCollision` true)
    (`PrimitiveComponent.SetMaterial` _returnvalue_12 0 "/Game/Materials/Grass.Grass")
    (else
      (bind _output_get_3 (set `local.Continue?` true))
      (return _output_get_3))))

(fn `GetVertsAndTris`
  (locals (CurrentSplineWithMesh2 :type "SplineWithMesh Object Reference"))
  (bind _triangles (`self.Triangles`))
  (bind _currentsplinewithmesh (`self.CurrentSplineWithMesh`))
  (bind _vertices (`self.Vertices`))
  (bind (_number _length) (`SplineTwistCorrectBPLibrary.CalcRailLength` _currentsplinewithmesh 5.0))
  (for _index (range (+ _number 1))
    (`KismetArrayLibrary.Array_Add` _vertices (`SplineComponent.GetLocationAtDistanceAlongSpline` _currentsplinewithmesh (* _index _length) "World"))
    (`KismetArrayLibrary.Array_Add` _vertices (`SplineComponent.GetLocationAtDistanceAlongSpline` (`self.CurrentSplineWithMesh`) (* (+ _index 1) _length) "World"))
    (`KismetArrayLibrary.Array_Add` _vertices (`self.SplinePointCenter`))
    (bind _returnvalue (* _index 3))
    (`KismetArrayLibrary.Array_Add` _triangles _returnvalue)
    (`KismetArrayLibrary.Array_Add` _triangles (+ _returnvalue 1))
    (`KismetArrayLibrary.Array_Add` _triangles (+ _returnvalue 2))))

(fn `SplinePointsToArray`
  (bind _strokes (`self.Strokes`))
  (bind _output (`|GetArrayItem` _strokes (- (`KismetArrayLibrary.Array_Length` _strokes) 1)))
  (bind (_number _length) (`SplineTwistCorrectBPLibrary.CalcRailLength` _output 5.0))
  (for _index (range (+ _number 1))
    (`KismetArrayLibrary.Array_Set` (`self.Spline Points`) _index (`SplineComponent.GetLocationAtDistanceAlongSpline` _output (* _index _length) "World") true))
  (set `self.SplinePointCenter` (`KismetMathLibrary.GetVectorArrayAverage` (`self.Spline Points`))))

(fn `UserConstructionScript`)