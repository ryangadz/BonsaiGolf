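; VR drawing pawn or tool that lets the player paint log-textured spline strokes, by name bridges, with the right motion controller.
; A trigger press adds a SplineWithMesh stroke with random scale and a hue-shifted M_Log dynamic material.
; While held, the trigger axis event appends points at the controller's position and up vector and calls AddMesh.
; Release detaches the stroke in world space; disconnected tree-spawning and per-section material experiments remain unused.
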(event `Key|MotionController_Right_Shoulder`
  (params (Key :type "Key Structure")))

(event `self.ReceiveBeginPlay`
  (`parent.ReceiveBeginPlay`))

(event `Key|MotionController_Right_Trigger`
  (params (Key :type "Key Structure"))
  (bind _strokes (`self.Strokes`))
  (bind _strokes_2 (`self.Strokes`))
  (bind _returnvalue (`KismetArrayLibrary.Array_Length` _strokes_2))
  (bind _output (`|GetArrayItem` _strokes_2 (- _returnvalue 1)))
  (:`Pressed`
    (set `self.IsDrawing` true)
    (`/Engine/EditorBlueprintResources/StandardMacros.DoOnce` false :!label _label
      (:`Completed`
        (bind _returnvalue_2 (`AddComponent|NODE_AddSplineWithMesh-0` :`self` self :`RelativeTransform` (`KismetMathLibrary.MakeTransform` (`SceneComponent.K2_GetComponentLocation` (`self.XR_Control`)))))
        (`KismetArrayLibrary.Array_Set` _strokes_2 _returnvalue _returnvalue_2 true)
        (`SplineComponent.ClearSplinePoints` _output true)
        (set `SplineWithMesh.Scale` (`KismetMathLibrary.RandomFloatInRange` 0.8 1.4) _output)
        (bind _returnvalue_3 (`KismetMaterialLibrary.CreateDynamicMaterialInstance` "/Game/Materials/M_Log.M_Log"))
        (`MaterialInstanceDynamic.SetScalarParameterValue` _returnvalue_3 "HueShift" (`KismetMathLibrary.RandomFloatInRange` -0.03 0.03))
        (set `SplineWithMesh.MaterialDefault` _returnvalue_3 _output))))
  (:`Released`
    (`SceneComponent.K2_DetachFromComponent` (`|GetArrayItem` _strokes (- (`KismetArrayLibrary.Array_Length` _strokes) 1)) "KeepWorld" "KeepWorld" "KeepWorld" true)
    (set `self.IsDrawing` false)
    (goto _label :!via `Reset`)))

(event `InputAxisKey|MotionController_Right_TriggerAxis`
  (params (AxisValue :type "Float (single-precision)"))
  (bind _strokes (`self.Strokes`))
  (bind _strokes_2 (`self.Strokes`))
  (bind _output (`|GetArrayItem` _strokes (- (`KismetArrayLibrary.Array_Length` _strokes) 1)))
  (bind _returnvalue (`SplineComponent.GetNumberOfSplinePoints` _output))
  (if (`self.IsDrawing`)
    (`SplineComponent.AddSplinePointAtIndex` _output (`SceneComponent.K2_GetComponentLocation` (`self.XR_Control`)) _returnvalue "World" true)
    (`SplineComponent.SetUpVectorAtSplinePoint` _output (- _returnvalue 1) (`SceneComponent.GetUpVector` (`self.XR_Control`)) "World" false)
    (`SplineWithMesh.AddMesh` (`|GetArrayItem` _strokes_2 (- (`KismetArrayLibrary.Array_Length` _strokes_2) 1)) self)))

(fn `UserConstructionScript`)