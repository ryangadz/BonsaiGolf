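; VR drawing pawn that paints colored spline-mesh strokes in the air with a motion controller.
; Right trigger press adds a new spline component at the controller and shifts the hue using a seed from its location; release detaches the stroke.
; While drawing, the trigger axis event appends oriented points, recreates per-segment dynamic materials with color, section and location-seeded variant parameters, then calls AddMesh on the stroke.
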(event `Key|MotionController_Right_Shoulder`
  (params (Key :type "Key Structure")))

(event `self.ReceiveBeginPlay`
  (`parent.ReceiveBeginPlay`)
  (set `MotionControllerComponent.MotionSource` "AnyHand" (`self.MotionController_0`)))

(event `Key|MotionController_Right_Trigger`
  (params (Key :type "Key Structure"))
  (bind _strokes (`self.Strokes`))
  (bind _strokes_2 (`self.Strokes`))
  (bind _strokes_3 (`self.Strokes`))
  (bind _returnvalue (`KismetArrayLibrary.Array_Length` _strokes_3))
  (bind (_h _s _v _a) (`KismetMathLibrary.RGBToHSV` (`self.Color`)))
  (bind (_returnvalue_x _returnvalue_y _returnvalue_z) (`KismetMathLibrary.BreakVector` (`SceneComponent.K2_GetComponentLocation` (`|GetArrayItem` _strokes_2 (- (`KismetArrayLibrary.Array_Length` _strokes_2) 1)))))
  (:`Pressed`
    (set `self.IsDrawing` true)
    (`/Engine/EditorBlueprintResources/StandardMacros.DoOnce` false :!label _label
      (:`Completed`
        (bind _returnvalue_2 (`AddComponent|NODE_AddSplineWithMesh-0` :`self` self :`RelativeTransform` (`KismetMathLibrary.MakeTransform` (`SceneComponent.K2_GetComponentLocation` (`self.MotionController_0`)))))
        (`KismetArrayLibrary.Array_Set` _strokes_3 _returnvalue _returnvalue_2 true)
        (`SplineComponent.ClearSplinePoints` (`|GetArrayItem` _strokes_3 (- _returnvalue 1)) true)
        (set `self.Color` (`KismetMathLibrary.HSVToRGB` (mod (+ _h (`KismetMathLibrary.RandomFloatInRangeFromStream` -180.0 180.0 (`KismetMathLibrary.MakeRandomStream` (`KismetMathLibrary.FTrunc` (+ _returnvalue_x _returnvalue_y _returnvalue_z))))) 359.0) _s _v _a)))))
  (:`Released`
    (`SceneComponent.K2_DetachFromComponent` (`|GetArrayItem` _strokes (- (`KismetArrayLibrary.Array_Length` _strokes) 1)) "KeepWorld" "KeepWorld" "KeepWorld" true)
    (set `self.IsDrawing` false)
    (goto _label :!via `Reset`)))

(event `InputAxisKey|MotionController_Right_TriggerAxis`
  (params (AxisValue :type "Float (single-precision)"))
  (bind _motioncontroller_0 (`self.MotionController_0`))
  (bind _strokes (`self.Strokes`))
  (bind _strokes_2 (`self.Strokes`))
  (bind _strokes_3 (`self.Strokes`))
  (bind _strokes_4 (`self.Strokes`))
  (bind _strokes_5 (`self.Strokes`))
  (bind _output (`|GetArrayItem` _strokes (- (`KismetArrayLibrary.Array_Length` _strokes) 1)))
  (bind _returnvalue (`SplineComponent.GetNumberOfSplinePoints` _output))
  (bind (_returnvalue_x _returnvalue_y _returnvalue_z) (`KismetMathLibrary.BreakVector` (`SceneComponent.K2_GetComponentLocation` (`|GetArrayItem` _strokes_2 (- (`KismetArrayLibrary.Array_Length` _strokes_2) 1)))))
  (bind _number (`SplineTwistCorrectBPLibrary.CalcRailLength` (`|GetArrayItem` _strokes_3 (- (`KismetArrayLibrary.Array_Length` _strokes_3) 1)) 1.0))
  (if (`self.IsDrawing`)
    (`SplineComponent.AddSplinePointAtIndex` _output (`SceneComponent.K2_GetComponentLocation` _motioncontroller_0) _returnvalue "World" true)
    (`SplineComponent.SetUpVectorAtSplinePoint` _output (- _returnvalue 1) (`SceneComponent.GetUpVector` _motioncontroller_0) "World" true)
    (set `self.Random` (`KismetMathLibrary.RandomIntegerInRangeFromStream` 0 19 (`KismetMathLibrary.MakeRandomStream` (`KismetMathLibrary.FTrunc` (+ _returnvalue_x _returnvalue_y _returnvalue_z)))))
    (for _index (range _number)
      (bind _returnvalue_2 (`KismetMaterialLibrary.CreateDynamicMaterialInstance` (`self.Material`)))
      (`MaterialInstanceDynamic.SetScalarParameterValue` _returnvalue_2 "Num" (`KismetMathLibrary.Conv_IntToDouble` (`self.Random`)))
      (`MaterialInstanceDynamic.SetScalarParameterValue` _returnvalue_2 "TotalSec" (`KismetMathLibrary.Conv_IntToDouble` _number))
      (`MaterialInstanceDynamic.SetScalarParameterValue` _returnvalue_2 "CurrentSec" (`KismetMathLibrary.Conv_IntToDouble` _index))
      (`MaterialInstanceDynamic.SetVectorParameterValue` _returnvalue_2 "Color" (`self.Color`))
      (`KismetArrayLibrary.Array_Set` (`SplineWithMesh.MaterialArray` (`|GetArrayItem` _strokes_5 (- (`KismetArrayLibrary.Array_Length` _strokes_5) 1))) _index _returnvalue_2 true))
    (`SplineWithMesh.AddMesh` (`|GetArrayItem` _strokes_4 (- (`KismetArrayLibrary.Array_Length` _strokes_4) 1)) self)))

(fn `UserConstructionScript`)