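; VR edit-mode pawn that lets the player pick a sub-pawn from a radial menu on the motion controller.
; On BeginPlay it spawns BP_RadialMenuOLD, attaches it to the controller and passes it the SubPawns list for icons.
; Right thumbstick angle selects and resizes the highlighted tool; releasing the thumbstick button spawns that sub-pawn, possesses it, and destroys menu and pawn.
; Older menu-building code in the construction script is disconnected.
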(event `self.ReceiveBeginPlay`
  (bind _output_get (set `self.CurrentPawn` self))
  (bind _returnvalue (`|SpawnActorFromClass` "/Game/Blueprints/RadialMenu/BP_RadialMenuOLD.BP_RadialMenuOLD_C" (`SceneComponent.K2_GetComponentToWorld` (`self.MotionController`)) "Undefined" "OverrideRootScale" _output_get null))
  (bind _output_get_2 (set `self.RadialMenu` _returnvalue))
  (message `/Game/Blueprints/Libraries/BPI_RadialMenu.ChangeToolIcons` _output_get_2 (`self.SubPawns`))
  (`self.K2_AttachToComponent` _output_get_2 (`self.MotionController`) "None" "KeepRelative" "KeepRelative" "KeepRelative" false))

(event `InputAxisKey|MotionController_Right_Thumbstick_X`
  (params (AxisValue :type "Float (single-precision)"))
  (bind _returnvalue (`KismetMathLibrary.DegAtan2` AxisValue (`self.GetInputAxisKeyValue`)))
  (bind _returnvalue_2 (`KismetMathLibrary.Round` (/ (+ _returnvalue (* (/ (- (`KismetMathLibrary.SignOfFloat` _returnvalue) 1.0) 2.0) -360.0)) (`/Game/Blueprints/RadialMenu/BP_RadialMenuOLD.AngleBetweenTools` (`self.RadialMenu`)))))
  (if (!= _returnvalue 0.0)
    (if (!= _returnvalue_2 (`self.CurrentTool`))
      (bind _output_get (set `self.CurrentTool` _returnvalue_2))
      (message `/Game/Blueprints/Libraries/BPI_RadialMenu.ResizeTools` (`self.RadialMenu`) _output_get (`self.SubPawns`)))))

(event `Key|MotionController_Right_Thumbstick`
  (params (Key :type "Key Structure"))
  (:`Released`
    (bind _returnvalue (`AIBlueprintHelperLibrary.SpawnAIFromClass` (`|GetArrayItem` (`self.SubPawns`) (`self.CurrentTool`))))
    (`Controller.Possess` (`GameplayStatics.GetPlayerController` 0) _returnvalue)
    (`self.K2_DestroyActor` (`self.RadialMenu`))
    (`self.K2_DestroyActor` self)))

(fn `UserConstructionScript`
  (set `self.CurrentPawn` self)
  (set `MotionControllerComponent.MotionSource` "AnyHand" (`self.MotionController`)))