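; BP_RadialMenu is a radial tool menu that shows one icon per tool class.
; ChangeToolIcons passes the classes to ChangeToolLayout, which spaces static mesh components evenly around a circle of ToolRadius, offset slightly on X.
; Each mesh gets a dynamic M_Icon material textured with that class's default Icon and is stored in MeshIcons.
; ResizeTools enlarges the mesh at the given index and resets the rest; the older billboard path is disconnected.
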(event `self.ReceiveBeginPlay`)

(event `/Game/Blueprints/BPI_RadialMenu.ResizeTools`
  (params (ToolToScale :type Integer) (SubClasses :type "Array of /Game/Blueprints/Pawns/BP_Edit Class Reference (by ref)"))
  (for (_array_element _array_index) (`self.MeshIcons`)
    (if (== _array_index ToolToScale)
      (`SceneComponent.SetRelativeScale3D` _array_element (0.045 0.045 0.045))
      (else
        (`SceneComponent.SetRelativeScale3D` _array_element (0.03 0.03 0.03))))))

(event `/Game/Blueprints/BPI_RadialMenu.Change NumTools`
  (params (NumTools :type Integer)))

(event `/Game/Blueprints/BPI_RadialMenu.ChangeToolIcons`
  (params (SubClasses :type "Array of /Game/Blueprints/Pawns/BP_Edit Class Reference (by ref)"))
  (`self.ChangeToolLayout` 0 SubClasses))

(fn `ChangeToolLayout`
  (params (NumTools :type Integer) (SubClasses :type "Array of /Game/Blueprints/Pawns/BP_Edit Class Reference"))
  (bind _returnvalue (`KismetArrayLibrary.Array_Length` SubClasses))
  (bind _toolradius (`self.ToolRadius`))
  (bind _output_get (set `self.AngleBetweenTools` (/ 360.0 (`KismetMathLibrary.Conv_IntToDouble` _returnvalue))))
  (`KismetArrayLibrary.Array_Resize` (`self.IconBillboards`) _returnvalue)
  (for (_array_element _array_index) SubClasses
    (bind _returnvalue_2 (* _array_index _output_get))
    (bind _returnvalue_3 (`AddComponent|NODE_AddStaticMeshComponent-0` :`RelativeTransform` (`KismetMathLibrary.MakeTransform` (`KismetMathLibrary.MakeVector` (+ (* (`KismetMathLibrary.DegCos` _returnvalue_2) _toolradius) -2.0) (* (`KismetMathLibrary.DegSin` _returnvalue_2) _toolradius) 1.0) (struct :`Yaw` 90.0) (0.03 0.03 0.03))))
    (bind _returnvalue_4 (`KismetMaterialLibrary.CreateDynamicMaterialInstance` "/Game/Materials/IconMaterials/M_Icon.M_Icon"))
    (`PrimitiveComponent.SetMaterial` _returnvalue_3 0 _returnvalue_4)
    (`MaterialInstanceDynamic.SetTextureParameterValue` _returnvalue_4 "Texture" (`/Game/Blueprints/BFL_Menu.Convert Texture` (`.Icon` (defaults `/Game/Blueprints/BP_RadialMenu` _array_element))))
    (`KismetArrayLibrary.Array_Set` (`self.MeshIcons`) _array_index _returnvalue_3 true))
  (`KismetSystemLibrary.PrintString` (`KismetStringLibrary.Conv_IntToString` _array_index) true false)
  (return))

(fn `UserConstructionScript`)