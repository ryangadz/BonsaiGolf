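; Test actor that checks line-trace collision against a procedural mesh.
; MakeMesh adds a Procedural Mesh Component with one collision-enabled, upward-facing triangle.
; The construction script builds it unless BulidMeshAtRuntime is set, while BeginPlay always builds it.
; Tick fires a short vertical WorldStatic trace that oscillates along Y through the actor, drawn each frame without ignoring self.
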(event `self.ReceiveBeginPlay`
  (`self.MakeMesh`))

(event `self.ReceiveTick`
  (params (DeltaSeconds :type "Float (single-precision)"))
  (bind (_returnvalue_x _returnvalue_y _returnvalue_z) (`KismetMathLibrary.BreakVector` (`self.K2_GetActorLocation`)))
  (bind _returnvalue (+ (* (`KismetMathLibrary.DegSin` (* (`KismetSystemLibrary.GetGameTimeInSeconds`) 60.0)) 12.0) _returnvalue_y))
  (`KismetSystemLibrary.LineTraceSingleForObjects` :`Start` (`KismetMathLibrary.MakeVector` _returnvalue_x _returnvalue (+ _returnvalue_z 10.0)) :`End` (`KismetMathLibrary.MakeVector` _returnvalue_x _returnvalue (- _returnvalue_z 10.0)) :`ObjectTypes` (`|MakeArray` "ObjectTypeQuery1" :!type "EObjectTypeQuery Enum") :`DrawDebugType` "ForOneFrame" :`bIgnoreSelf` false))

(fn `MakeMesh`
  (bind _returnvalue (`AddComponent|NODE_AddProceduralMeshComponent-0` :`RelativeTransform` (`KismetMathLibrary.MakeTransform` (0.0 0.0 0.0) (struct))))
  (`ProceduralMeshComponent.CreateMeshSection_LinearColor` :`self` _returnvalue :`Vertices` (`|MakeArray` (15.0 0.0 0.0) (`KismetMathLibrary.RotateAngleAxis` (15.0 0.0 0.0) 240.0 (0.0 0.0 1.0)) (`KismetMathLibrary.RotateAngleAxis` (15.0 0.0 0.0) 120.0 (0.0 0.0 1.0))) :`Triangles` (`|MakeArray` 0 1 2) :`Normals` (`|MakeArray` (0.0 0.0 1.0) (0.0 0.0 1.0) (0.0 0.0 1.0) :!type "Vector Structure") :`bCreateCollision` true))

(fn `UserConstructionScript`
  (if (not (`self.BulidMeshAtRuntime`))
    (`self.MakeMesh`)))