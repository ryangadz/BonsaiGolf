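; XR pawn for a ball-putting game, played with the right motion controller and a spawned laser pointer.
; Each tick it requests a raycast and scales the laser by hit distance, while the shoulder button line-traces to place the ball.
; Once the ball stops, thumbstick input turns and stretches a camera-relative direction arrow, and the trigger applies a matching impulse.
; Physics sleep and wake events toggle the arrow's visibility.
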(event `RequestRaycast`)

(event `self.ReceiveBeginPlay`
  (bind _motioncontroller (`self.MotionController`))
  (set `MotionControllerComponent.MotionSource` "Right" (`self.MotionController`))
  (bind _returnvalue (`AddComponent|NODE_AddStaticMeshComponent-0`))
  (set `self.Platform` _returnvalue)
  (set `self.Ball` (`self.BallS`))
  (bind _returnvalue_2 (`AddComponent|NODE_AddStaticMeshComponent-2`))
  (bind _output_get (set `self.Direction Arrow` _returnvalue_2))
  (bind _returnvalue_3 (`KismetMaterialLibrary.CreateDynamicMaterialInstance` (`PrimitiveComponent.GetMaterial` _output_get 0)))
  (set `self.Arrow Material` _returnvalue_3)
  (bind _returnvalue_4 (`|SpawnActorFromClass` "/Game/Blueprints/BP_Laserpointer.BP_Laserpointer_C" (`SceneComponent.K2_GetComponentToWorld` _motioncontroller) "Undefined" "OverrideRootScale" null null))
  (`self.K2_AttachToComponent` _returnvalue_4 _motioncontroller "None" "KeepRelative" "KeepRelative" "KeepRelative" false)
  (set `self.Laser` _returnvalue_4))

(event `Key|MotionController_Right_FaceButton1`
  (params (Key :type "Key Structure"))
  (bind _motioncontroller (`self.MotionController`))
  (:`Pressed`
    (`RaycastComponent.RequestRaycast` (`self.Raycast`) (make `RaycastQueryParams` (`SceneComponent.K2_GetComponentLocation` _motioncontroller) (`SceneComponent.GetForwardVector` _motioncontroller) (0.0 0.0 0.0) 1 1 1.0) (delegate `RaycastResults`) :!label _label)
    (`SceneComponent.SetWorldScale3D` (`Actor.RootComponent` (`self.Laser`)) (`KismetMathLibrary.MakeVector` (`KismetMathLibrary.VSize` (- (`.HitPoint` (break `RaycastHitResult` (stale `RaycastResults` HitResult))) (`SceneComponent.K2_GetComponentLocation` (`self.MotionController`)))) 1.0 1.0))))

(event `ScaleLaser`
  (goto _label))

(event `Key|MotionController_Right_Thumbstick_Down`
  (params (Key :type "Key Structure")))

(event `Key|MotionController_Right_Thumbstick`
  (params (Key :type "Key Structure")))

(event `RaycastResults`
  (params (HitResult :type "RaycastHitResult Structure")))

(event `AddLights`
  (params (HitResult :type "RaycastHitResult Structure")))

(event `Key|MotionController_Right_Shoulder`
  (params (Key :type "Key Structure"))
  (bind _motioncontroller (`self.MotionController`))
  (bind _ball (`self.Ball`))
  (bind _returnvalue (`SceneComponent.K2_GetComponentLocation` _motioncontroller))
  (:`Pressed`
    (bind _outhit (`KismetSystemLibrary.LineTraceSingleForObjects` :`Start` _returnvalue :`End` (+ _returnvalue (* (`SceneComponent.GetForwardVector` _motioncontroller) 1000.0)) :`ObjectTypes` (`|MakeArray` "ObjectTypeQuery1" :!type "EObjectTypeQuery Enum") :`DrawDebugType` "ForDuration" :`bIgnoreSelf` false :`DrawTime` 2.0))
    (`SceneComponent.K2_SetWorldTransform` _ball (`KismetMathLibrary.MakeTransform` (+ (`.ImpactPoint` (`GameplayStatics.BreakHitResult` _outhit)) (0.0 0.0 10.0)) (struct) (0.66 0.66 0.66)) false true)
    (`PrimitiveComponent.SetPhysicsLinearVelocity` _ball (0.0 0.0 0.0) false "None")))

(event `self.ReceiveTick`
  (params (DeltaSeconds :type "Float (single-precision)"))
  (bind _direction_arrow (`self.Direction Arrow`))
  (bind _thumbx (`self.ThumbX`))
  (bind _thumby (`self.ThumbY`))
  (bind _returnvalue (`SceneComponent.K2_GetComponentLocation` (`self.Ball`)))
  (bind (_returnvalue_roll _returnvalue_pitch _returnvalue_yaw) (`KismetMathLibrary.BreakRotator` (`KismetMathLibrary.MakeRotFromY` (- _returnvalue (`SceneComponent.K2_GetComponentLocation` (`self.XR_Camera`))))))
  (`self.ScaleLaser`)
  (if (> (`KismetMathLibrary.VSizeSquared` (`SceneComponent.GetComponentVelocity` (`self.BallS`))) 0.01)
    (set `self.ReadyToPutt?` false)
    (set `self.ThumbX` 0.0)
    (set `self.ThumbY` 0.0)
    (else
      (set `self.ReadyToPutt?` true)
      (`SceneComponent.K2_SetWorldLocationAndRotation` _direction_arrow _returnvalue (`KismetMathLibrary.MakeRotator` 90.0 0.0 (- (+ _returnvalue_yaw (`KismetMathLibrary.DegAtan2` _thumbx _thumby)) 90.0)) false false)
      (`SceneComponent.SetWorldScale3D` _direction_arrow (`KismetMathLibrary.MakeVector` 1.0 1.0 (* (`KismetMathLibrary.Sqrt` (+ (`KismetMathLibrary.MultiplyMultiply_FloatFloat` _thumbx 2.0) (`KismetMathLibrary.MultiplyMultiply_FloatFloat` _thumby 2.0))) 10.0))))))

(event `InputAxisKey|MotionController_Right_Thumbstick_X`
  (params (AxisValue :type "Float (single-precision)"))
  (set `self.ThumbX` AxisValue :!label _label_2)
  (set `self.ThumbY` (stale `InputAxisKey|MotionController_Right_Thumbstick_Y` AxisValue)))

(event `InputAxisKey|MotionController_Right_Thumbstick_Y`
  (params (AxisValue :type "Float (single-precision)"))
  (goto _label_2))

(event `Key|MotionController_Right_Trigger`
  (params (Key :type "Key Structure"))
  (bind _thumbx (`self.ThumbX`))
  (bind _thumby (`self.ThumbY`))
  (bind (_returnvalue_roll _returnvalue_pitch _returnvalue_yaw) (`KismetMathLibrary.BreakRotator` (`KismetMathLibrary.MakeRotFromY` (- (`SceneComponent.K2_GetComponentLocation` (`self.Ball`)) (`SceneComponent.K2_GetComponentLocation` (`self.XR_Camera`))))))
  (:`Pressed`
    (if (`self.ReadyToPutt?`)
      (`PrimitiveComponent.WakeAllRigidBodies` (`self.BallS`) :!label _label_3)
      (while (not (`PrimitiveComponent.IsAnyRigidBodyAwake` (`self.BallS`)))
        (goto _label_3))
      (`PrimitiveComponent.AddImpulse` (`self.Ball`) (* (`KismetMathLibrary.GreaterGreater_VectorRotator` (1.0 0.0 0.0) (`KismetMathLibrary.MakeRotator` 0.0 0.0 (+ _returnvalue_yaw (`KismetMathLibrary.DegAtan2` _thumbx _thumby)))) (* (`KismetMathLibrary.Sqrt` (+ (`KismetMathLibrary.MultiplyMultiply_FloatFloat` _thumbx 2.0) (`KismetMathLibrary.MultiplyMultiply_FloatFloat` _thumby 2.0))) 10.0)) "None" false)
      (`SceneComponent.SetVisibility` (`self.Direction Arrow`) false false)
      (set `self.ReadyToPutt?` false))))

(event `self.BallS.OnComponentDeactivated`
  (params (Component :type "ActorComponent Object Reference")))

(event `self.BallS.OnComponentSleep`
  (params (SleepingComponent :type "PrimitiveComponent Object Reference") (BoneName :type Name))
  (`SceneComponent.SetVisibility` (`self.Direction Arrow`) true false))

(event `self.BallS.OnComponentWake`
  (params (WakingComponent :type "PrimitiveComponent Object Reference") (BoneName :type Name))
  (if (not (`self.ReadyToPutt?`))
    (`SceneComponent.SetVisibility` (`self.Direction Arrow`) false false)))

(fn `UserConstructionScript`
  (bind _returnvalue (`KismetMaterialLibrary.CreateDynamicMaterialInstance` "/Game/Materials/M_HueShift.M_HueShift"))
  (bind _output_get (set `self.Material` _returnvalue))
  (`PrimitiveComponent.SetMaterial` (`StaticMeshActor.StaticMeshComponent` (`self.StaticMesh`)) 0 _output_get))