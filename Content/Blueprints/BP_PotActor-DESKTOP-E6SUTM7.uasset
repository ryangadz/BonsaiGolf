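; Pot actor whose outline is drawn with a motion controller, then filled with a ground-material mesh.
; DrawPot grows a spline at the starting height from controller position, forward offset or line-trace hit, adding points at spacing intervals.
; When the end nears the start, it stops the BP_Edit_Pot pawn's drawing, closes the loop and builds a procedural mesh with collision from the outline.
; PotComplete, AddHole and EditPot are empty stubs.
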(event `BeginPot`
  (params (MotionController :type "MotionControllerComponent Object Reference"))
  (bind _returnvalue (`self.PointFromMotionController` (`self.LocationType`)))
  (set `self.MotionController` MotionController)
  (bind _returnvalue_2 (`AddComponent|NODE_AddSplineWithMesh-0` :`self` self))
  (bind _output_get (set `self.SplineWithMesh` _returnvalue_2))
  (`SplineComponent.ClearSplinePoints` _output_get true)
  (`SplineComponent.AddSplinePointAtIndex` _output_get _returnvalue 0 "World" true)
  (`SplineComponent.AddSplinePointAtIndex` _output_get _returnvalue 1 "World" true)
  (set `self.NumSplinePoints` 2)
  (set `self.Zvalue` (.z _returnvalue)))

(event `DrawPot`
  (bind _numsplinepoints (`self.NumSplinePoints`))
  (bind _splinewithmesh (`self.SplineWithMesh`))
  (bind _returnvalue (- (`self.NumSplinePoints`) 1))
  (bind _out (`self.FlattenVector` (`self.PointFromMotionController` (`self.LocationType`))))
  (bind _out_2 (`self.FlattenVector` (`self.PointFromMotionController` (`self.LocationType`))))
  (bind _continue_ (`self.CheckForLoopAndComplete`))
  (if (and _continue_ (>= (`self.Last 2 Points`) 10.0))
    (`SplineComponent.AddSplinePointAtIndex` (`self.SplineWithMesh`) _out_2 _numsplinepoints "World" true)
    (set `self.LastPosition` _out_2)
    (`/Engine/EditorBlueprintResources/StandardMacros.IncrementInt` _numsplinepoints)
    (else
      (`SplineComponent.SetLocationAtSplinePoint` _splinewithmesh _returnvalue _out "World" true)
      (`SplineComponent.SetTangentAtSplinePoint` _splinewithmesh _returnvalue (* (`KismetMathLibrary.Normal` (- _out (`self.LastPosition`))) (`self.Last 2 Points`)) "World" true)
      (set `self.LastPosition` _out)
      (`SplineWithMesh.AddMesh` (`self.SplineWithMesh`) self))))

(event `PotComplete`)

(event `AddHole`)

(event `EditPot`)

(fn `CheckForLoopAndComplete`
  (returns (`Continue?` :type Boolean))
  (locals (Continue :type Boolean) (GridPoints :type "Array of Integer") (GridX :type Integer :default 0) (Index :type Integer) (Triangles_ :type "Array of Integer") (Normals :type "Array of Vector Structure"))
  (bind _splinewithmesh (`self.SplineWithMesh`))
  (bind _splinewithmesh_2 (`self.SplineWithMesh`))
  (bind _splinewithmesh_3 (`self.SplineWithMesh`))
  (bind _numsplinepoints (`self.NumSplinePoints`))
  (bind _splinewithmesh_4 (`self.SplineWithMesh`))
  (bind _returnvalue (- (`self.NumSplinePoints`) 1))
  (bind _returnvalue_2 (`SplineComponent.GetLocationAtSplinePoint` _splinewithmesh_4 (- _numsplinepoints 1) "World"))
  (bind _returnvalue_3 (`SplineComponent.GetLocationAtSplinePoint` _splinewithmesh_4 (- _numsplinepoints 2) "World"))
  (bind _returnvalue_4 (+ _returnvalue_2 _returnvalue_3))
  (if (and (> (`self.NumSplinePoints`) 3) (<= (`KismetMathLibrary.VSize` (- (`SplineComponent.GetLocationAtSplinePoint` _splinewithmesh 0 "World") (`SplineComponent.GetLocationAtSplinePoint` _splinewithmesh (- (`self.NumSplinePoints`) 1) "World"))) 10.0))
    (set `local.Continue` false)
    (bind _asbp_edit_pot (cast `/Game/Blueprints/Pawns/BP_Edit_Pot` (`Controller.K2_GetPawn` (`GameplayStatics.GetPlayerController` 0))))
    (`self.CustomIsDrawingEvent` _asbp_edit_pot false)
    (if (not (> (`KismetMathLibrary.VSize` _returnvalue_4) 5.0))
      (`SplineComponent.SetLocationAtSplinePoint` _splinewithmesh_3 (- (`self.NumSplinePoints`) 2) (/ _returnvalue_4 2.0) "World" false)
      (`SplineComponent.SetTangentAtSplinePoint` _splinewithmesh_3 _returnvalue (* (`KismetMathLibrary.Normal` (/ (+ (`SplineComponent.GetTangentAtSplinePoint` (`self.SplineWithMesh`) (- (`self.NumSplinePoints`) 2) "World") (`SplineComponent.GetTangentAtSplinePoint` (`self.SplineWithMesh`) (- (`self.NumSplinePoints`) 1) "World")) 2.0)) (+ (/ (`KismetMathLibrary.VSize` (- _returnvalue_2 _returnvalue_3)) 2.0) 10.0)) "World" true)
      (`SplineComponent.RemoveSplinePoint` _splinewithmesh_3 _returnvalue true))
    (`SplineComponent.SetClosedLoop` _splinewithmesh_3 true true)
    (`SplineComponent.SetTangentAtSplinePoint` (`self.SplineWithMesh`) 0 (`KismetMathLibrary.GetVectorArrayAverage` (`|MakeArray` (`SplineComponent.GetTangentAtSplinePoint` _splinewithmesh_2 0 "World") (`SplineComponent.GetTangentAtSplinePoint` _splinewithmesh_2 (- (`self.NumSplinePoints`) 1) "World"))) "World" true)
    (`SplineWithMesh.AddMesh` (`self.SplineWithMesh`) self)
    (bind (_verts _triangles) (`/Game/Blueprints/Libraries/BFL_MeshBuilding.BuildMeshFromOutline(OLD)` (`self.SplineWithMesh`) (`self.TriangleSize`)))
    (bind _output_get (set `self.Verts` _verts))
    (bind _output_get_2 (set `self.Triangles` _triangles))
    (for (_ _array_index) _output_get
      (`KismetArrayLibrary.Array_Set` (`local.Normals`) _array_index (0.0 0.0 1.0) true))
    (bind _returnvalue_5 (`AddComponent|NODE_AddProceduralMeshComponent-0` :`bManualAttachment` true))
    (`ProceduralMeshComponent.CreateMeshSection_LinearColor` :`self` _returnvalue_5 :`Vertices` _output_get :`Triangles` _output_get_2 :`Normals` (`local.Normals`) :`bCreateCollision` true)
    (`PrimitiveComponent.SetMaterial` _returnvalue_5 0 (`self.GroundMaterial`))
    (`PrimitiveComponent.SetCollisionEnabled` _returnvalue_5 "QueryAndPhysics")
    (`self.PotComplete`)
    (else
      (bind _output_get_3 (set `local.Continue` true))
      (return _output_get_3))))

(fn `FlattenVector`
  (params (In :type "Vector Structure"))
  (returns (Out :type "Vector Structure"))
  (return (`KismetMathLibrary.MakeVector` (.x In) (.y In) (`self.Zvalue`))))

(fn `Last 2 Points`
  (returns (Distance :type "Float (double-precision)"))
  (bind _splinewithmesh (`self.SplineWithMesh`))
  (bind _numsplinepoints (`self.NumSplinePoints`))
  (return (- (`SplineComponent.GetDistanceAlongSplineAtSplinePoint` _splinewithmesh (- _numsplinepoints 1)) (`SplineComponent.GetDistanceAlongSplineAtSplinePoint` _splinewithmesh (- _numsplinepoints 2)))))

(fn `PointFromMotionController`
  (params (Type :type "/Game/Blueprints/Enum_MotionControllerData Enum" :default "NewEnumerator0"))
  (returns (ReturnValue :type "Vector Structure") (ValidLocation :type Boolean))
  (locals (Location :type "Vector Structure" :default (0.0 0.0 0.0)) (`Valid?` :type Boolean :default false))
  (bind _motioncontroller (`self.MotionController`))
  (bind _returnvalue (`SceneComponent.K2_GetComponentLocation` _motioncontroller))
  (bind _returnvalue_2 (`SceneComponent.GetForwardVector` _motioncontroller))
  (switch `/Game/Blueprints/Enum_MotionControllerData` Type
    (:`NewEnumerator0`
      (set `local.Location` (`SceneComponent.K2_GetComponentLocation` (`self.MotionController`)))
      (set `local.Valid?` true))
    (:`NewEnumerator1`
      (set `local.Location` (+ _returnvalue (* _returnvalue_2 30.0)))
      (set `local.Valid?` true))
    (:`NewEnumerator2`
      (bind _outhit (`KismetSystemLibrary.LineTraceSingleForObjects` :`Start` _returnvalue :`End` (+ _returnvalue (* _returnvalue_2 500.0)) :`ObjectTypes` (`|MakeArray` "ObjectTypeQuery1" :!type "EObjectTypeQuery Enum") :`DrawDebugType` "ForOneFrame" :`DrawTime` 1.0))
      (bind _output_get (set `local.Valid?` (`GameplayStatics.BreakHitResult` _outhit)))
      (if _output_get
        (set `local.Location` (+ (`.Location` (`GameplayStatics.BreakHitResult` _outhit)) (0.0 0.0 1.5))))))
  (return (`local.Location`) (`local.Valid?`)))

(fn `UserConstructionScript`)